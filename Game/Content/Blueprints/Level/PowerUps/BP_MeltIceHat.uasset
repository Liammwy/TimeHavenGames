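; BP_MeltIceHat is a destructible object, by its name meltable ice, that releases a hat collectible once destroyed.
; Tick runs the parent logic, then polls IsDestroyed and uses the SpawnedHat flag to call SpawnHat only once.
; SpawnHat spawns a BP_HatCollectible at the actor's transform, passes it CollectibleType and a rotation speed, then calls HatGrow on it.
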(event EventBeginPlay
  (|CallParentFunction) ; This node is disabled and will not be called.\nDrag off pins to build functionality.
)

(event EventTick
  (params (DeltaSeconds :type Float%20%28single-precision%29))
  ;[1 1 1] Spawn Once Destroyed
  (|CallParentFunction DeltaSeconds)
  (if (and (Variables|Default|GetisDestroyed) (not (Variables|Default|GetSpawnedHat)))
    (Variables|Default|SetSpawnedHat true)
    (CallFunction|SpawnHat)))

(fn ConstructionScript
  (|CallParentFunction))

(fn SpawnHat
  ;[1 0.1218 0] SPAWN THE HAT
  (bind _returnvalue (Game|SpawnActorfromClass "/Game/Blueprints/HatShop/BP_HatCollectible.BP_HatCollectible_C" (Transformation|GetActorTransform self) "Undefined" "MultiplyWithRoot" 0 true 2.0 1.0 (Variables|Default|GetCollectibleType) 0))
  (Default|HatGrow _returnvalue))