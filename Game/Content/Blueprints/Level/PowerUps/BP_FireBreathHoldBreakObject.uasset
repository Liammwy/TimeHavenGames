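; Ice block obstacle that the player's fire breath melts away.
; Overlap with any of three player fire colliders starts Tick shrinking the visuals and solid collision over FireHoldTime; melting never pauses, as end-overlap and refreeze logic are disconnected.
; Fully melted, it hides, disables collision and plays a melting event.
; The player's respawn-delay event restores visibility and collision, but not timer, flame count or scale.
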(event OnComponentBeginOverlap(BreakCollisionTrigger)
  (params (OverlappedComponent :type Primitive%20Component%20Object%20Reference) (OtherActor :type Actor%20Object%20Reference) (OtherComp :type Primitive%20Component%20Object%20Reference) (OtherBodyIndex :type Integer) (bFromSweep :type Boolean) (SweepResult :type Hit%20Result%20Structure%20%28by%20ref%29))
  ;[1 1 1 1 42] TOGGLE MELTING ON
  (if (Math|Boolean|ORBoolean (== OtherComp (Variables|Default|GetFireBreathRef0)) (== OtherComp (Variables|Default|GetFireBreathRef1)) (== OtherComp (Variables|Default|GetFireBreathRef2)))
    (Variables|Default|SetactiveFlames (+ (Variables|Default|GetactiveFlames) 1))))

(event OnComponentEndOverlap(BreakCollisionTrigger)
  (params (OverlappedComponent :type Primitive%20Component%20Object%20Reference) (OtherActor :type Actor%20Object%20Reference) (OtherComp :type Primitive%20Component%20Object%20Reference) (OtherBodyIndex :type Integer))
  ;[1 1 1 1 50] TOGGLE MELTING OFF
)

(event Custom|OnRespawnDelayStarted
  (if (Variables|Default|GetisDestroyed)
    (CallFunction|ToggleDestroyed false)))

(event EventBeginPlay
  (bind _returnvalue (Actor|GetActorOfClass "/Game/Blueprints/Player/BP_ThirdPersonCharacter.BP_ThirdPersonCharacter_C"))
  ;[1 1 1] Ensure found object != null
  (if (not (== _returnvalue 0))
    ;[1 1 1] Grab ref to fire collision from player
    (Variables|Default|SetFireBreathRef0 (Variables|/Game/Blueprints/Player/BP_ThirdPersonCharacter.BP_ThirdPersonCharacter_C|GetFireBreathCollision _returnvalue))
    (Variables|Default|SetFireBreathRef1 (Variables|/Game/Blueprints/Player/BP_ThirdPersonCharacter.BP_ThirdPersonCharacter_C|GetFireBreathCollision1 _returnvalue))
    (Variables|Default|SetFireBreathRef2 (Variables|/Game/Blueprints/Player/BP_ThirdPersonCharacter.BP_ThirdPersonCharacter_C|GetFireBreathCollision2 _returnvalue))
    (EventDispatchers|BindEventtoOnRespawnDelayStarted _returnvalue (delegate Custom|OnRespawnDelayStarted))))

(event EventTick
  (params (DeltaSeconds :type Float%20%28single-precision%29))
  (if (not (Variables|Default|GetisDestroyed))
    (if (>= (Variables|Default|GetactiveFlames) 1)
      ;[0.08256 0.8095 1] MELT/SHRINK ICE
      (Transformation|SetRelativeScale3D (Variables|Default|GetVisual%20Pivot) (Math|Conversions|ToVector(Float) (- 1.0 (/ (Variables|Default|GetcurrentTimeTouchingFire) (Variables|Default|GetfireHoldTime)))))
      (Transformation|SetRelativeScale3D (Variables|Default|GetSolidCollision) (Math|Conversions|ToVector(Float) (- 1.0 (/ (Variables|Default|GetcurrentTimeTouchingFire) (Variables|Default|GetfireHoldTime)))))
      (Development|PrintString "Hello")
      (bind _output_get (Variables|Default|SetcurrentTimeTouchingFire (+ (Variables|Default|GetcurrentTimeTouchingFire) DeltaSeconds)))
      (if (>= _output_get (Variables|Default|GetfireHoldTime))
        (CallFunction|ToggleDestroyed true)))))

(fn ConstructionScript)

(fn ToggleDestroyed
  (params (IsDestroyed :type Boolean))
  (bind _solidcollision (Variables|Default|GetSolidCollision))
  (bind _visualsmesh (Variables|Default|GetVisualsMesh))
  (bind _breakcollisiontrigger (Variables|Default|GetBreakCollisionTrigger))
  (bind _output_get (Variables|Default|SetisDestroyed IsDestroyed))
  (if _output_get
    ;[1 1 1] Turn everything off when destroyed
    (Collision|SetCollisionEnabled _solidcollision "NoCollision")
    (Rendering|SetVisibility _visualsmesh false false)
    (Collision|SetCollisionEnabled _breakcollisiontrigger "NoCollision")
    (Class|FMODBlueprintStatics|PlayEventatLocation "/Game/FMOD/Events/melting_Block.melting_Block" (Math|Conversions|ToTransform(Vector) (Transformation|GetActorLocation)))
    (else
      ;[1 1 1] Turn everything on when re-enabled
      (Collision|SetCollisionEnabled _solidcollision "QueryAndPhysics")
      (Rendering|SetVisibility _visualsmesh true false)
      (Collision|SetCollisionEnabled _breakcollisiontrigger "QueryOnly"))))