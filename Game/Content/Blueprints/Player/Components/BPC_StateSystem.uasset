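; Player component that tracks the character's movement state, such as grounded, slipped, jumping, flipping, climbing, ledge climbing and midair without jump.
; Each state event sets CurrentState, copies it to the snowman or standard player anim Blueprint via an accessor, then fires a state-changed call.
; Tick switches grounded states to midair-no-jump when the character falls, preventing a double jump off ledges; that transition skips the anim update.
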(event Custom|OnPlayerJump
  (Variables|Default|SetCurrentState "NewEnumerator2")
  (bind (_asnew_player_anim_bp _assnowman_anim_bp _snowman) (Utilities|AccessAnimationClass))
  (if _snowman
    (Variables|/Game/Blueprints/Player/Animation/Snowman_AnimBp.Snowman_AnimBp_C|SetCurrentPlayerState _assnowman_anim_bp "NewEnumerator2")
    (else
      (Variables|/Game/Blueprints/Player/Animation/NewPlayerAnim_BP.NewPlayerAnim_BP_C|SetCurrentPlayerState _asnew_player_anim_bp "NewEnumerator2")))
  (Default|CallOnStateChanged))

(event Custom|OnPlayerLand
  (Variables|Default|SetCurrentState "NewEnumerator0")
  (bind (_asnew_player_anim_bp _assnowman_anim_bp _snowman) (Utilities|AccessAnimationClass))
  (if _snowman
    (Variables|/Game/Blueprints/Player/Animation/Snowman_AnimBp.Snowman_AnimBp_C|SetCurrentPlayerState _assnowman_anim_bp "NewEnumerator0")
    (else
      (Variables|/Game/Blueprints/Player/Animation/NewPlayerAnim_BP.NewPlayerAnim_BP_C|SetCurrentPlayerState _asnew_player_anim_bp "NewEnumerator0")))
  (Default|CallOnStateChanged))

(event Custom|OnPlayerClimb
  (Variables|Default|SetCurrentState "NewEnumerator1")
  (bind (_asnew_player_anim_bp _assnowman_anim_bp _snowman) (Utilities|AccessAnimationClass))
  (if _snowman
    (Variables|/Game/Blueprints/Player/Animation/Snowman_AnimBp.Snowman_AnimBp_C|SetCurrentPlayerState _assnowman_anim_bp "NewEnumerator1")
    (else
      (Variables|/Game/Blueprints/Player/Animation/NewPlayerAnim_BP.NewPlayerAnim_BP_C|SetCurrentPlayerState _asnew_player_anim_bp "NewEnumerator1")))
  (Default|CallOnStateChanged))

(event Custom|OnPlayerLedgeClimb
  (Variables|Default|SetCurrentState "NewEnumerator3")
  (bind (_asnew_player_anim_bp _assnowman_anim_bp _snowman) (Utilities|AccessAnimationClass))
  (if _snowman
    (Variables|/Game/Blueprints/Player/Animation/Snowman_AnimBp.Snowman_AnimBp_C|SetCurrentPlayerState _assnowman_anim_bp "NewEnumerator3")
    (else
      (Variables|/Game/Blueprints/Player/Animation/NewPlayerAnim_BP.NewPlayerAnim_BP_C|SetCurrentPlayerState _asnew_player_anim_bp "NewEnumerator3")))
  (Default|CallOnStateChanged))

(event Custom|OnMidairNoJump
  (Variables|Default|SetCurrentState "NewEnumerator4")
  (Default|CallOnStateChanged))

(event Custom|OnPlayerFlip
  (Variables|Default|SetCurrentState "NewEnumerator5")
  (bind (_asnew_player_anim_bp _assnowman_anim_bp _snowman) (Utilities|AccessAnimationClass))
  (if _snowman
    (Variables|/Game/Blueprints/Player/Animation/Snowman_AnimBp.Snowman_AnimBp_C|SetCurrentPlayerState _assnowman_anim_bp "NewEnumerator5")
    (else
      (Variables|/Game/Blueprints/Player/Animation/NewPlayerAnim_BP.NewPlayerAnim_BP_C|SetCurrentPlayerState _asnew_player_anim_bp "NewEnumerator5")))
  (Default|CallOnStateChanged))

(event Custom|OnPlayerSlipped
  (Variables|Default|SetCurrentState "NewEnumerator7")
  (bind (_asnew_player_anim_bp _assnowman_anim_bp _snowman) (Utilities|AccessAnimationClass))
  (if _snowman
    (Variables|/Game/Blueprints/Player/Animation/Snowman_AnimBp.Snowman_AnimBp_C|SetCurrentPlayerState _assnowman_anim_bp "NewEnumerator7")
    (else
      (Variables|/Game/Blueprints/Player/Animation/NewPlayerAnim_BP.NewPlayerAnim_BP_C|SetCurrentPlayerState _asnew_player_anim_bp "NewEnumerator7")))
  (Default|CallOnStateChanged))

(event EventTick
  (params (DeltaSeconds :type Float%20%28single-precision%29))
  ;[1 1 1] Check player's fall state to update to MidairNoJump if need be (fix for walking off ledge and getting double jump)
  (bind _isgrounded (CallFunction|IsCurrentStateGrounded))
  (if _isgrounded
    (bind _asbp_third_person_character (Utilities|Casting|CastToBP_ThirdPersonCharacter (Components|GetOwner)))
    (if (AI|Components|NavMovement|IsFalling (Variables|/Script/Engine.Character|GetCharacterMovement _asbp_third_person_character))
      (CallFunction|OnMidairNoJump))))

(fn AccessAnimClass
  (bind (_asnew_player_anim_bp _assnowman_anim_bp) (Utilities|AccessAnimationClass))
  (return _asnew_player_anim_bp _assnowman_anim_bp))

(fn IsCurrentStateGrounded
  (bind _currentstate (Variables|Default|GetCurrentState))
  (return (or (Utilities|Enum|Equal(Enum) _currentstate "NewEnumerator0") (Utilities|Enum|Equal(Enum) _currentstate "NewEnumerator7"))))