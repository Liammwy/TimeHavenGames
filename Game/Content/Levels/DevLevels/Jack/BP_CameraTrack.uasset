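; Camera rail actor that follows an assigned character along a spline track while looking at them; setting the owner toggles its tick.
; The character's nearest point on the Path spline, shifted back by a lag distance, gives a time that positions the camera on the separate CamerTrack spline.
; Each tick eases camera location and rotation toward their targets.
; The lag offset also eases, growing when the character moves quickly against the path direction.
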(event EventTick
  (params (DeltaSeconds :type Float%20%28single-precision%29))
  (bind _camowner (Variables|Default|GetCamOwner)
    (:then
      (CallFunction|UpdateCamera (Transformation|GetSocketLocation (Variables|/Script/Engine.Character|GetMesh _camowner) "Spine2"))
      (CallFunction|InterpLocation)
      (CallFunction|InterpRotation)
      (CallFunction|UpdateMovementLagOffset))
    (:else)))

(fn ConstructionScript)

(fn SetCamOwner
  (params (Character :type BP%20Third%20Person%20Character%20Object%20Reference))
  (bind _output_get (Variables|Default|SetCamOwner Character))
  (Utilities|IsValid _output_get
    (:Is%20Valid
      (Actor|Tick|SetActorTickEnabled true)
      (CallFunction|UpdateCamera (Transformation|GetSocketLocation (Variables|/Script/Engine.Character|GetMesh (Variables|Default|GetCamOwner)) "Spine2")))
    (:Is%20Not%20Valid
      (Actor|Tick|SetActorTickEnabled false))))

(fn UpdateCamera
  (params (World%20Location :type Vector))
  (Variables|Default|SetDesiredLocation (Spline|GetLocationatTime (Variables|Default|GetCamer%20Track) (CallFunction|GetTimeAlongSplineatNearbyLocation World%20Location (Variables|Default|GetMovementLagOffset)) "World" false))
  (Variables|Default|SetDesiredRotation (Math|Rotator|FindLookatRotation (Transformation|GetWorldLocation (Variables|Default|GetTrackCamera)) (Transformation|GetActorLocation (Variables|Default|GetCamOwner)))))

(fn GetTimeAlongSplineatNearbyLocation
  (params (World%20Location :type Vector) (DistanceLag :type Float%20%28double-precision%29))
  (bind _path (Variables|Default|GetPath))
  (bind _camowner (Variables|Default|GetCamOwner))
  (bind _returnvalue (Class|SplineComponent|FindInputKeyClosesttoWorldLocation _path World%20Location))
  (bind _returnvalue_2 (Transformation|GetVelocity _camowner))
  (bind (_x _y) (Math|Vector|BreakVector _returnvalue_2))
  (Variables|Default|SetLagDirection (Math|Integer|SelectInt (Math|Integer|SelectInt 1 2 (Utilities|Operators|EqualEqual (Math|Rotator|GetRotationXVector (Class|SplineComponent|GetRotationatSplineInputKey (Variables|Default|GetPath) _returnvalue "World")) (Math|Vector|Normalize _returnvalue_2) 1.0)) 0 (> (Math|Vector|VectorLength (Math|Vector|MakeVector _x _y 0.0)) 3e+02)))
  (return (Class|SplineComponent|GetTimeatDistanceAlongSpline _path (- (Class|SplineComponent|GetDistanceAlongSplineatSplineInputKey _path _returnvalue) DistanceLag))))

(fn InterpLocation
  (bind _trackcamera (Variables|Default|GetTrackCamera))
  (bind _returnvalue (Transformation|GetWorldLocation _trackcamera))
  (if (not (Utilities|Operators|EqualEqual (Variables|Default|GetDesiredLocation) _returnvalue 1.0))
    (Transformation|SetWorldLocation (Variables|Default|GetTrackCamera) (Math|Interpolation|VInterpTo _returnvalue (Variables|Default|GetDesiredLocation) (Utilities|Time|GetWorldDeltaSeconds) (Variables|Default|GetMovementLagSpeed)) false false)))

(fn InterpRotation
  (bind _trackcamera (Variables|Default|GetTrackCamera))
  (bind _returnvalue (Transformation|GetWorldRotation _trackcamera))
  (if (not (Utilities|Operators|EqualEqual (Variables|Default|GetDesiredRotation) _returnvalue 0.01))
    (Transformation|SetWorldRotation (Variables|Default|GetTrackCamera) (Math|Interpolation|RInterpTo _returnvalue (Variables|Default|GetDesiredRotation) (Utilities|Time|GetWorldDeltaSeconds) (Variables|Default|GetRotationLagSpeed)) false false)))

(fn UpdateMovementLagOffset
  (bind _maxmovementlagoffset (Variables|Default|GetMaxMovementLagOffset))
  (Variables|Default|SetMovementLagOffset (Math|Interpolation|FInterpTo (Variables|Default|GetMovementLagOffset) (Utilities|Select :Index (Variables|Default|GetLagDirection) :Option%200 _maxmovementlagoffset :Option%201 _maxmovementlagoffset :Option%202 (* _maxmovementlagoffset 1.5)) (Utilities|Time|GetWorldDeltaSeconds) (Variables|Default|GetMovementLagOffsetSpeed))))