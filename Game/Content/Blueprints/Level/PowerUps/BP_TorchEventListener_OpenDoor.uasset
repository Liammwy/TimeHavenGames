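; Torch event listener that opens a door, represented by a Cube component, when all torches are ignited.
; It overrides RespondToAllTorchesIgnited to call OpenDoor, which plays a timeline that lerps the cube from its original relative location by an XPos, YPos, ZPos offset.
; The construction script caches that original location, and both response steps print debug strings.
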(event Custom|OpenDoor
  (bind _originallocation (Variables|Default|GetOriginalLocation))
  (Development|PrintString "Hello")
  (bind _alpha (Timeline|Timeline Play)
    (:Update
      (Transformation|SetRelativeLocation (Variables|Default|GetCube) (Math|Vector|Lerp(Vector) _originallocation (+ _originallocation (Math|Vector|MakeVector (+ (Variables|Default|GetXPos) 0.0) (+ (Variables|Default|GetYPos) 0.0) (+ (Variables|Default|GetZPos) 0.0))) _alpha) false false))))

(event EventBeginPlay
  (|CallParentFunction) ; This node is disabled and will not be called.\nDrag off pins to build functionality.
)

(event Collision|EventActorBeginOverlap
  (params (OtherActor :type Actor%20Object%20Reference))
  (|CallParentFunction OtherActor) ; This node is disabled and will not be called.\nDrag off pins to build functionality.
)

(event EventTick
  (params (DeltaSeconds :type Float%20%28single-precision%29))
  (|CallParentFunction DeltaSeconds) ; This node is disabled and will not be called.\nDrag off pins to build functionality.
)

(fn ConstructionScript
  (|CallParentFunction)
  (Variables|Default|SetOriginalLocation (.location (Transformation|GetRelativeTransform (Variables|Default|GetCube)))))

(fn RespondtoAllTorchesIgnited
  (|CallParentFunction)
  (Development|PrintString "Should Open Doors")
  (CallFunction|OpenDoor))