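; Cutscene variant of a breakable block that shatters by itself after a configurable delay from BeginPlay.
; Breaking hides the cube and decal, disables collision, enables physics on ten fragments and plays a sound, pitched down under altered time dilation.
; Tick shrinks the fragments over their lifetime, then hides and deactivates them.
; The construction script traces downward to place the decal on the surface below.
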(event Custom|triggerBreak
  (CallFunction|BlockHitFunction true))

(event EventBeginPlay
  ;[1 1 1] Add all fragment meshes to array on BeginPlay
  (Utilities|Array|Add (Variables|Default|GetFragments) (Variables|Default|GetFragment_1))
  (Utilities|Array|Add (Variables|Default|GetFragments) (Variables|Default|GetFragment_2))
  (Utilities|Array|Add (Variables|Default|GetFragments) (Variables|Default|GetFragment_3))
  (Utilities|Array|Add (Variables|Default|GetFragments) (Variables|Default|GetFragment_4))
  (Utilities|Array|Add (Variables|Default|GetFragments) (Variables|Default|GetFragment_5))
  (Utilities|Array|Add (Variables|Default|GetFragments) (Variables|Default|GetFragment_6))
  (Utilities|Array|Add (Variables|Default|GetFragments) (Variables|Default|GetFragment_7))
  (Utilities|Array|Add (Variables|Default|GetFragments) (Variables|Default|GetFragment_8))
  (Utilities|Array|Add (Variables|Default|GetFragments) (Variables|Default|GetFragment_9))
  (Utilities|Array|Add (Variables|Default|GetFragments) (Variables|Default|GetFragment_10))
  (Utilities|FlowControl|Delay (Variables|Default|GetdelayTimer))
  (CallFunction|TriggerBreak))

(event EventTick
  (params (DeltaSeconds :type Float%20%28single-precision%29))
  (if (Variables|Default|GetisBroken)
    (if (not (Variables|Default|GetfragmentsDestroyed))
      (bind _output_get (Variables|Default|SettimeSinceBroken (+ (Variables|Default|GettimeSinceBroken) DeltaSeconds)))
      (if (>= _output_get (Variables|Default|GetbrokenFragmentLifetime))
        ;[1 1 1] Deactivate fragments when lifetime ended
        (for _array_element (Variables|Default|GetFragments)
          (Physics|SetSimulatePhysics _array_element false)
          (Rendering|SetVisibility _array_element false false)
          (Collision|SetCollisionEnabled _array_element "NoCollision")
          (Variables|Default|SetfragmentsDestroyed true))
        (else
          ;[1 1 1] Update shrinking mesh visuals
          (for _array_element_2 (Variables|Default|GetFragments)
            (Transformation|SetRelativeScale3D _array_element_2 (Math|Vector|MakeVector (- 1.0 (/ (Variables|Default|GettimeSinceBroken) (Variables|Default|GetbrokenFragmentLifetime))) (- 1.0 (/ (Variables|Default|GettimeSinceBroken) (Variables|Default|GetbrokenFragmentLifetime))) (- 1.0 (/ (Variables|Default|GettimeSinceBroken) (Variables|Default|GetbrokenFragmentLifetime)))))))))))

(fn ConstructionScript
  (bind _defaultsceneroot (Variables|Default|GetDefaultSceneRoot))
  (bind _returnvalue (Transformation|GetWorldLocation _defaultsceneroot))
  (bind (_outhit _returnvalue_2) (Collision|LineTraceByChannel _returnvalue (- _returnvalue "0.000000,0.000000,1000.000000") "TraceTypeQuery1" false 0 "None"))
  (if _returnvalue_2
    (Transformation|SetWorldLocation (Variables|Default|GetDecal) (.Location (Collision|BreakHitResult _outhit)) false false)))

(fn BlockHitFunction
  (params (HitBottomColl :type Boolean))
  (bind _returnvalue (Class|FMODBlueprintStatics|PlayEventatLocation "/Game/FMOD/Events/BlockBreaking.BlockBreaking" (Transformation|GetActorTransform)))
  (if (== (Class|GameplayStatics|GetGlobalTimeDilation) 1.0)
    _
    (else
      (Class|FMODBlueprintStatics|EventInstanceSetPitch _returnvalue 0.5)))
  (Rendering|SetVisibility (Variables|Default|GetCube) false false)
  (Rendering|SetVisibility (Variables|Default|GetDecal) false false)
  (Collision|SetCollisionEnabled (Variables|Default|GetCube) "NoCollision")
  (Collision|SetCollisionEnabled (Variables|Default|GetBottomCollider) "NoCollision")
  (if HitBottomColl
    ;[1 1 1] Trigger fragment physics
    (for _array_element (Variables|Default|GetFragments)
      (Physics|SetEnableGravity _array_element true)
      (Physics|SetSimulatePhysics _array_element true))
    (Variables|Default|SetisBroken true)
    (Variables|Default|SettimeSinceBroken 0.0)))