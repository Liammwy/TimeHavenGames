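; BP_CameraDirector is a trigger volume that steers the player's camera in a direction taken from a referenced camera track actor.
; BeginPlay offsets LookAtPoint along the normalized vector between the first points of that actor's CameraTrack and Path splines, scaled by AngleSharpness.
; While the third-person character overlaps the box, Tick interpolates control rotation toward LookAtPoint.
; Both overlap events set HasCameraControl to the inverse of LockUserCameraControl, so exiting never restores locked control.
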(event OnComponentBeginOverlap(Box)
  (params (OverlappedComponent :type Primitive%20Component%20Object%20Reference) (OtherActor :type Actor%20Object%20Reference) (OtherComp :type Primitive%20Component%20Object%20Reference) (OtherBodyIndex :type Integer) (bFromSweep :type Boolean) (SweepResult :type Hit%20Result%20Structure%20%28by%20ref%29))
  ;[1 1 1] Get Player Reference and Activate Camera Movement
  (bind _asbp_third_person_character (Utilities|Casting|CastToBP_ThirdPersonCharacter OtherActor))
  (bind _output_get (Variables|Default|SetPlayerRef _asbp_third_person_character))
  (Variables|/Game/Blueprints/Player/BP_ThirdPersonCharacter.BP_ThirdPersonCharacter_C|SetHasCameraControl _output_get (not (Variables|Default|GetLockUserCameraControl)))
  (Variables|Default|SetInVolume true))

(event OnComponentEndOverlap(Box)
  (params (OverlappedComponent :type Primitive%20Component%20Object%20Reference) (OtherActor :type Actor%20Object%20Reference) (OtherComp :type Primitive%20Component%20Object%20Reference) (OtherBodyIndex :type Integer))
  ;[1 1 1] Stops Camera Movement
  (Variables|/Game/Blueprints/Player/BP_ThirdPersonCharacter.BP_ThirdPersonCharacter_C|SetHasCameraControl (Variables|Default|GetPlayerRef) (not (Variables|Default|GetLockUserCameraControl)))
  (Variables|Default|SetInVolume false))

(event EventTick
  (params (DeltaSeconds :type Float%20%28single-precision%29))
  (bind _playerref (Variables|Default|GetPlayerRef))
  ;[1 1 1] Make Player Look To Designated Point
  (if (Variables|Default|GetInVolume)
    (Pawn|SetControlRotation (Game|GetPlayerController 0) (Math|Interpolation|RInterpTo (Pawn|GetControlRotation _playerref :!class /Script/Engine.Pawn) (Math|Rotator|FindLookatRotation (Transformation|GetActorLocation _playerref) (Transformation|GetWorldLocation (Variables|Default|GetLook%20At%20Point))) DeltaSeconds (Variables|Default|GetCameraPushSpeed)))))

(event EventBeginPlay
  (bind _actorfordirection (Variables|Default|GetActorForDirection))
  ;[1 1 1] Aquire Look To Direction From Selected Camera Track
  (Variables|Default|SetLookDirection (Math|Vector|Normalize (- (Spline|GetLocationatSplinePoint (Variables|/Game/Levels/DevLevels/Jack/Level_Mechanics/Camera/CameraTrack/BP_CameraTrack.BP_CameraTrack_C|GetPath _actorfordirection) 0 "World") (Spline|GetLocationatSplinePoint (Variables|/Game/Levels/DevLevels/Jack/Level_Mechanics/Camera/CameraTrack/BP_CameraTrack.BP_CameraTrack_C|GetCameraTrack _actorfordirection) 0 "World"))))
  (Transformation|SetRelativeLocation (Variables|Default|GetLook%20At%20Point) (* (Variables|Default|GetLookDirection) (Variables|Default|GetAngleSharpness)) false false))

(fn ConstructionScript)