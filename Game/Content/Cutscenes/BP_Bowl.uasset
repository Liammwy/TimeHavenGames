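; Cutscene bowl actor that sets off an explosion effect once it is raised above a height threshold.
; From BeginPlay it polls the root's world Z on a short Delay loop instead of Tick.
; Crossing the threshold ends the loop and, after a further delay, spawns P_EndBowlBoom at the static mesh's location.
; Disconnected leftovers hold an alternative game-mode BowlExplode trigger and an attached spawn.
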(event Custom|ParticleBoom
  (Utilities|FlowControl|Delay 3.0)
  (Niagara|SpawnSystematLocation "/Game/Cutscenes/P_EndBowlBoom.P_EndBowlBoom" (Transformation|GetWorldLocation (Variables|Default|GetStaticMesh))))

(event Custom|Check
  (if (> (.z (Transformation|GetWorldLocation (Variables|Default|GetDefaultSceneRoot))) 1e+01)
    (CallFunction|ParticleBoom)
    (else
      (Utilities|FlowControl|Delay 0.2)
      (CallFunction|Check))))

(event EventBeginPlay
  (if (> (.z (Transformation|GetWorldLocation (Variables|Default|GetDefaultSceneRoot))) 1e+01)
    (CallFunction|ParticleBoom)
    (else
      (Utilities|FlowControl|Delay 0.2)
      (CallFunction|Check))))

(event Collision|EventActorBeginOverlap
  (params (OtherActor :type Actor%20Object%20Reference)))

(event EventTick
  (params (DeltaSeconds :type Float%20%28single-precision%29)))

(fn ConstructionScript)