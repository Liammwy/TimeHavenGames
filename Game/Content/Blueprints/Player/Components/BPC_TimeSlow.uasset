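; Player component for a toggleable time-slow ability that runs on a limited power meter.
; Slowing lowers global time dilation, raises the player's custom dilation to compensate, and drops music pitch.
; A throttled Tick drains or regenerates power, updating the meter and screen tint widgets.
; Depletion only clears the active flag, leaving the regen step to restore speed and pitch; respawning blocks input and cancels active slow.
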(event Custom|OnPlayerRespawn
  ;[1 1 1] If time slow is active when respawning, deactivate it
  (if (Variables|Default|GettimeSlowActive)
    (Variables|/Script/Engine.Actor|SetCustomTimeDilation (Variables|Default|GetplayerRef) 1.0)
    (Utilities|Time|SetGlobalTimeDilation 1.0)
    (Variables|Default|SettimeSlowActive false)
    (Class|FMODBlueprintStatics|EventInstanceSetPitch :Pitch 1.0)))

(event Input|EnhancedActionEvents|EnhancedInputActionIA_SlowDown
  (params (ActionValue :type Boolean) (ElapsedSeconds :type Float%20%28double-precision%29) (TriggeredSeconds :type Float%20%28double-precision%29) (InputAction :type Input%20Action%20Object%20Reference :default "/Game/Data/Input/Actions/IA_SlowDown.IA_SlowDown"))
  (bind _playerref (Variables|Default|GetplayerRef))
  (bind _playerref_2 (Variables|Default|GetplayerRef))
  (bind _bg_audio (Variables|/Game/Blueprints/Player/BP_ThirdPersonCharacter.BP_ThirdPersonCharacter_C|GetBG_Audio _playerref_2))
  (:Started
    ;[1 1 1] Don't allow input response if currently respawning
    (if (not (Variables|/Game/Blueprints/Player/BP_ThirdPersonCharacter.BP_ThirdPersonCharacter_C|GetIsRespawning (Variables|Default|GetplayerRef)))
      (Class|FMODBlueprintStatics|PlayEvent2D "/Game/FMOD/Events/SlowDownTime.SlowDownTime")
      ;[1 1 1] Alter time dilation and BGM pitch
      (if (Variables|Default|GettimeSlowActive)
        (Variables|/Script/Engine.Actor|SetCustomTimeDilation _playerref 1.0 :!label _label)
        (Utilities|Time|SetGlobalTimeDilation 1.0)
        (Variables|Default|SettimeSlowActive false)
        (Class|FMODBlueprintStatics|EventInstanceSetPitch _bg_audio 1.0)
        (elif (> (Variables|BPC_TimeSlow_C|GetcurrentPower (Actor|GetComponentbyClass (Variables|Default|GetplayerRef) "BPC_TimeSlow_C")) 0.0)
          (Variables|/Script/Engine.Actor|SetCustomTimeDilation _playerref 5.0)
          (Utilities|Time|SetGlobalTimeDilation 0.2)
          (Variables|Default|SettimeSlowActive true)
          (Class|FMODBlueprintStatics|EventInstanceSetPitch _bg_audio 0.5)
          (else
            (goto _label)))))))

(event EventTick
  (params (DeltaSeconds :type Float%20%28single-precision%29))
  (bind _output_get (Variables|Default|SetcurrentDelay (- (Variables|Default|GetcurrentDelay) DeltaSeconds)))
  (if (<= _output_get 0.0)
    (Variables|Default|SetcurrentDelay 0.2)
    (if (Variables|Default|GettimeSlowActive)
      (CallFunction|DrainingPower)
      (Variables|/Script/UMG.Widget|SetVisibility (Variables|Default|GettimeSlowTint) "Visible")
      (elif (not (== (Variables|Default|GetcurrentPower) (Variables|Default|GetmaxPower)))
        (CallFunction|RegainingPower)
        (Variables|/Script/UMG.Widget|SetVisibility (Variables|Default|GettimeSlowTint) "Hidden")))))

(event EventBeginPlay
  (Variables|Default|SetcurrentPower (Variables|Default|GetmaxPower))
  (bind _returnvalue (UserInterface|CreateWidget "/Game/Blueprints/UI/WBP_TimeSlow.WBP_TimeSlow_C" (Game|GetPlayerController 0)))
  (bind _output_get (Variables|Default|SettimeSlowWidget _returnvalue))
  (UserInterface|Viewport|AddtoViewport _output_get 0)
  (bind _returnvalue_2 (UserInterface|CreateWidget "/Game/Blueprints/UI/WBP_TimeSlowTint.WBP_TimeSlowTint_C" (Game|GetPlayerController 0)))
  (bind _output_get_2 (Variables|Default|SettimeSlowTint _returnvalue_2))
  (UserInterface|Viewport|AddtoViewport _output_get_2 0)
  (bind _asbp_third_person_character (Utilities|Casting|CastToBP_ThirdPersonCharacter (Components|GetOwner)))
  (Variables|Default|SetplayerRef _asbp_third_person_character))

(fn DrainingPower
  ;[1 1 1 1 30] Logic for draining power
  (if (<= (Variables|Default|GetcurrentPower) 0.0)
    (Variables|Default|SettimeSlowActive false)
    (else
      (Variables|Default|SetcurrentPower (Math|Float|Clamp(Float) (- (Variables|Default|GetcurrentPower) 1.0) 0.0 (Variables|Default|GetmaxPower)))
      (Default|SetPercent (Variables|Default|GettimeSlowWidget) (Variables|Default|GetcurrentPower) (Variables|Default|GetmaxPower)))))

(fn RegainingPower
  (bind _playerref (Variables|Default|GetplayerRef))
  (Variables|Default|SetcurrentPower (Math|Float|Clamp(Float) (+ (Variables|Default|GetcurrentPower) 1.0) 0.0 (Variables|Default|GetmaxPower)))
  (Default|SetPercent (Variables|Default|GettimeSlowWidget) (Variables|Default|GetcurrentPower) (Variables|Default|GetmaxPower))
  (Utilities|Time|SetGlobalTimeDilation 1.0)
  (Variables|/Script/Engine.Actor|SetCustomTimeDilation _playerref 1.0)
  (Class|FMODBlueprintStatics|EventInstanceSetPitch (Variables|/Game/Blueprints/Player/BP_ThirdPersonCharacter.BP_ThirdPersonCharacter_C|GetBG_Audio _playerref) 1.0))