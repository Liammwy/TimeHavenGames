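; Unfinished level-unlock Blueprint meant to record level access in BP_Global_GameInstance's LevelAccessible struct and return the player to the Hub.
; Its LevelAccessChecker event is empty, and the logic behind it is disconnected, so it never runs.
; That logic switches on a constant 0, which only prints an error.
; Only the Level 1 case rebuilds the struct with its flag set; cases 2–4 assign None, leaving their struct builders unused.
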(event Custom|LevelAccessChecker)