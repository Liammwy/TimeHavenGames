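; BP_Cannon is a level decoration cannon that automatically fires BP_Snowball actors at a timed interval.
; Tick accumulates time up to Timer, then resets, spawns a snowball above the Cannon component with yaw flipped around, triggers Recoil and activates a Niagara effect.
; Recoil plays a timeline that offsets the Cannon along world X only, regardless of the cannon's facing.
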(event Custom|Recoil
  (bind _cannon (Variables|Default|GetCannon))
  (bind _returnvalue (Transformation|GetWorldLocation _cannon))
  (bind _output_get (Variables|Default|SetReturn%20Value%20X (.x _returnvalue)))
  (bind _recoil_amount (Timeline|Timeline PlayFromStart)
    (:Update
      (Transformation|SetWorldLocation (Variables|Default|GetCannon) (Math|Vector|MakeVector (+ _output_get _recoil_amount) (.y _returnvalue) (.z _returnvalue)) false false))))

(event EventBeginPlay)

(event Collision|EventActorBeginOverlap
  (params (OtherActor :type Actor%20Object%20Reference)))

(event EventTick
  (params (DeltaSeconds :type Float%20%28single-precision%29))
  (bind _cannon (Variables|Default|GetCannon))
  (bind _returnvalue (Transformation|GetWorldTransform _cannon))
  (Variables|Default|SetCurrentTime (+ DeltaSeconds (Variables|Default|GetCurrentTime)))
  (if (>= (Variables|Default|GetCurrentTime) (Variables|Default|GetTimer))
    (Variables|Default|SetCurrentTime 0.0)
    (Game|SpawnActorfromClass "/Game/Blueprints/Level/Decoration/BP_Snowball.BP_Snowball_C" (Math|Transform|MakeTransform (Math|Vector|MakeVector (.x (.location _returnvalue)) (.y (.location _returnvalue)) (+ (.z (.location _returnvalue)) 1.5e+02)) (Math|Rotator|MakeRotator (.roll (.rotation _returnvalue)) (.pitch (.rotation _returnvalue)) (+ (.yaw (.rotation _returnvalue)) 1.8e+02)) (.scale _returnvalue)) "Undefined" "MultiplyWithRoot" 0 0)
    (CallFunction|Recoil)
    (Components|Activation|Activate (Variables|Default|GetNiagara) true)))

(fn ConstructionScript)