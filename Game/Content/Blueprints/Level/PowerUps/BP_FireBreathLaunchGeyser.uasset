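; Geyser that the player charges with fire breath, then uses as a launch pad.
; Overlap with the player's fire breath colliders builds a timer on Tick; reaching the hold time activates the geyser's visuals and launch collision.
; The timer then drains at a rate scaled by CooldownRate, deactivating the geyser at zero.
; While active, player contact resets vertical velocity, launches along the actor's up vector and plays the Geyser event.
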(event OnComponentBeginOverlap(LaunchPlayerColl)
  (params (OverlappedComponent :type Primitive%20Component%20Object%20Reference) (OtherActor :type Actor%20Object%20Reference) (OtherComp :type Primitive%20Component%20Object%20Reference) (OtherBodyIndex :type Integer) (bFromSweep :type Boolean) (SweepResult :type Hit%20Result%20Structure%20%28by%20ref%29))
  (bind _playerref (Variables|Default|GetPlayerRef))
  (bind _charactermovement (Variables|/Script/Engine.Character|GetCharacterMovement _playerref))
  ;[1 1 1] If active, launch player on contact
  (if (== OtherComp (Variables|Default|GetPlayerCollRef))
    (if (Variables|Default|GetGeyserActive)
      (Variables|/Script/Engine.MovementComponent|SetVelocity _charactermovement (Math|Vector|MakeVector (.x (Variables|/Script/Engine.MovementComponent|GetVelocity _charactermovement)) (.y (Variables|/Script/Engine.MovementComponent|GetVelocity _charactermovement)) 0.0))
      (Character|LaunchCharacter _playerref (* (Math|Vector|GetUpVector (Transformation|GetActorRotation)) (Variables|Default|GetLaunchPower)) false false)
      (Class|FMODBlueprintStatics|PlayEventatLocation "/Game/FMOD/Events/Geyser.Geyser" (Transformation|GetActorTransform)))))

(event OnComponentBeginOverlap(FireBreathTriggerColl)
  (params (OverlappedComponent :type Primitive%20Component%20Object%20Reference) (OtherActor :type Actor%20Object%20Reference) (OtherComp :type Primitive%20Component%20Object%20Reference) (OtherBodyIndex :type Integer) (bFromSweep :type Boolean) (SweepResult :type Hit%20Result%20Structure%20%28by%20ref%29))
  (if (Math|Boolean|ORBoolean (== OtherComp (Variables|Components|GetFireBreathRef0)) (== OtherComp (Variables|Components|GetFireBreathRef1)) (== OtherComp (Variables|Components|GetFireBreathRef2)))
    (Variables|Components|SettouchingFire true)))

(event OnComponentEndOverlap(FireBreathTriggerColl)
  (params (OverlappedComponent :type Primitive%20Component%20Object%20Reference) (OtherActor :type Actor%20Object%20Reference) (OtherComp :type Primitive%20Component%20Object%20Reference) (OtherBodyIndex :type Integer))
  (if (Math|Boolean|ORBoolean (== OtherComp (Variables|Components|GetFireBreathRef0)) (== OtherComp (Variables|Components|GetFireBreathRef1)) (== OtherComp (Variables|Components|GetFireBreathRef2)))
    (Variables|Components|SettouchingFire false)))

(event EventBeginPlay
  (CallFunction|ToggleGeyserActive false)
  (bind _returnvalue (Actor|GetActorOfClass "/Game/Blueprints/Player/BP_ThirdPersonCharacter.BP_ThirdPersonCharacter_C"))
  ;[1 1 1] Ensure found object != null
  (if (not (== _returnvalue 0))
    ;[1 1 1] Grab ref to fire collision from player
    (Variables|Components|SetFireBreathRef0 (Variables|/Game/Blueprints/Player/BP_ThirdPersonCharacter.BP_ThirdPersonCharacter_C|GetFireBreathCollision _returnvalue))
    (Variables|Components|SetFireBreathRef1 (Variables|/Game/Blueprints/Player/BP_ThirdPersonCharacter.BP_ThirdPersonCharacter_C|GetFireBreathCollision1 _returnvalue))
    (Variables|Components|SetFireBreathRef2 (Variables|/Game/Blueprints/Player/BP_ThirdPersonCharacter.BP_ThirdPersonCharacter_C|GetFireBreathCollision2 _returnvalue))
    (Variables|Default|SetPlayerRef _returnvalue)
    (Variables|Default|SetPlayerCollRef (Variables|/Script/Engine.Character|GetCapsuleComponent _returnvalue))))

(event EventTick
  (params (DeltaSeconds :type Float%20%28single-precision%29))
  (if (Variables|Components|GettouchingFire)
    (bind _output_get (Variables|Default|SetcurrentTimeTouchingFire (+ (Variables|Default|GetcurrentTimeTouchingFire) DeltaSeconds)))
    (if (>= _output_get (Variables|Default|GetfireHoldTime))
      (CallFunction|ToggleGeyserActive true)
      (Variables|Components|SettouchingFire false))
    (elif (> (Variables|Default|GetcurrentTimeTouchingFire) 0.0)
      (Variables|Default|SetcurrentTimeTouchingFire (Math|Float|Max(Float) (- (Variables|Default|GetcurrentTimeTouchingFire) (* DeltaSeconds (/ (Variables|Default|GetfireHoldTime) (Variables|Components|GetcooldownRate)))) 0.0))
      (else
        (CallFunction|ToggleGeyserActive false)))))

(fn ConstructionScript)

(fn ToggleGeyserActive
  (params (Active :type Boolean))
  (bind _triggeredvisuals (Variables|Default|GetTriggeredVisuals))
  (bind _launchplayercoll (Variables|Default|GetLaunchPlayerColl))
  (bind _output_get (Variables|Default|SetGeyserActive Active))
  (if _output_get
    (Rendering|SetVisibility _triggeredvisuals true false)
    (Collision|SetCollisionEnabled _launchplayercoll "QueryOnly")
    (else
      (Rendering|SetVisibility _triggeredvisuals false false)
      (Collision|SetCollisionEnabled _launchplayercoll "NoCollision"))))