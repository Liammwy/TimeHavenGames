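; BP_ScarfRemovalZone is a trigger zone that strips the player's active scarf power via a snowman thief.
; Overlapping with a power spawns BP_SnowmanSteal below ground and raises it by timeline, then clears the power, resets scarf materials and plays a witch laugh.
; It also creates and animates a WBP_LostItem widget for the lost power.
; Tick uses that animation's length to time the snowman's timeline descent, which re-arms the zone and destroys the snowman.
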(event OnComponentBeginOverlap(Collider)
  (params (OverlappedComponent :type Primitive%20Component%20Object%20Reference) (OtherActor :type Actor%20Object%20Reference) (OtherComp :type Primitive%20Component%20Object%20Reference) (OtherBodyIndex :type Integer) (bFromSweep :type Boolean) (SweepResult :type Hit%20Result%20Structure%20%28by%20ref%29))
  (bind _snowmansp (Variables|Default|GetSnowmanSP))
  ;[1 1 1] Checks if the player has a power
  (if (not (Variables|Default|GetStartedSteal))
    (if (== OtherComp (Variables|Default|GetPlayerCollisionRef))
      (bind _currentactivepower (Default|GetScarfPower (Variables|/Game/Blueprints/Player/BP_ThirdPersonCharacter.BP_ThirdPersonCharacter_C|GetBPC_ScarfPowerManager (Variables|Default|GetPlayer))))
      (if (not (Utilities|Enum|Equal(Enum) _currentactivepower "NewEnumerator0"))
        ;[1 1 1] If the player has a power, activate snowman steal
        (Variables|Default|SetStartedSteal true)
        (bind _returnvalue (Game|SpawnActorfromClass "/Game/Blueprints/Level/PowerUps/General/BP_SnowmanSteal.BP_SnowmanSteal_C" (Math|Transform|MakeTransform (- (Transformation|GetWorldLocation _snowmansp) (Math|Vector|MakeVector 0.0 0.0 (Variables|Default|GetSpawnHeight))) (Transformation|GetWorldRotation _snowmansp) "1.000000,1.000000,1.000000") "Undefined" "MultiplyWithRoot" 0 0))
        (Variables|Default|SetSnowman _returnvalue)
        (CallFunction|SnowmanAppear)
        (bind _returnvalue_2 (UserInterface|CreateWidget "/Game/Blueprints/UI/WBP_LostItem.WBP_LostItem_C" (Game|GetPlayerController 0) self))
        (Default|ScarfCollectible _returnvalue_2 (Variables|/Game/Blueprints/Player/Components/BPC_ScarfPowerManager.BPC_ScarfPowerManager_C|GetCurrentActivePower (Variables|/Game/Blueprints/Player/BP_ThirdPersonCharacter.BP_ThirdPersonCharacter_C|GetBPC_ScarfPowerManager (Variables|Default|GetPlayer))))
        (UserInterface|Animation|PlayAnimation _returnvalue_2 (Variables|/Game/Blueprints/UI/WBP_LostItem.WBP_LostItem_C|GetgotCollection _returnvalue_2) 0.0 1 "Forward" (Variables|Default|GetUIAnimationSpeed) false)
        (Variables|Default|SetAnimationTime (Class|WidgetAnimation|GetEndTime (Variables|/Game/Blueprints/UI/WBP_LostItem.WBP_LostItem_C|GetgotCollection _returnvalue_2)))
        (Utilities|FlowControl|Delay (* (Class|WidgetAnimation|GetEndTime (Variables|/Game/Blueprints/UI/WBP_LostItem.WBP_LostItem_C|GetgotCollection _returnvalue_2)) 2.0))
        (Widget|RemovefromParent _returnvalue_2)))))

(event Custom|SnowmanSteal
  ;[1 0.2791 0 1 34] Steal Scarf (Widget is placeholder, thats why it is created)
  (Default|SetScarfPower (Variables|/Game/Blueprints/Player/BP_ThirdPersonCharacter.BP_ThirdPersonCharacter_C|GetBPC_ScarfPowerManager (Variables|Default|GetPlayer)) "NewEnumerator0")
  (CallFunction|RemoveVisual)
  (Class|FMODBlueprintStatics|PlayEventatLocation "/Game/FMOD/Events/WitchLaugh.WitchLaugh" (Transformation|GetActorTransform)))

(event Custom|SnowmanAppear
  (bind _snowman (Variables|Default|GetSnowman))
  (bind _snowmansp (Variables|Default|GetSnowmanSP))
  (bind _returnvalue (Transformation|GetWorldLocation _snowmansp))
  (bind _returnvalue_2 (Transformation|GetActorLocation _snowman))
  ;[1 0 0] Make Snowman Rise
  (bind _timerising (Timeline|Timeline PlayFromStart)
    (:Update
      (Transformation|SetActorLocation _snowman (Math|Vector|MakeVector (.x _returnvalue_2) (.y _returnvalue_2) (Math|Float|Lerp (- (.z _returnvalue) (Variables|Default|GetSpawnHeight)) (.z _returnvalue) _timerising)) false false))
    (:Finished
      (CallFunction|SnowmanSteal))))

(event Custom|SnowmanDisappear
  (bind _snowman (Variables|Default|GetSnowman))
  (bind _snowman_2 (Variables|Default|GetSnowman))
  (bind _snowmansp (Variables|Default|GetSnowmanSP))
  (bind _returnvalue (Transformation|GetWorldLocation _snowmansp))
  (bind _returnvalue_2 (Transformation|GetActorLocation _snowman_2))
  ;[0 1 0.02836] Make Snowman Disappear
  (bind _timerising (Timeline|Timeline_0 PlayFromStart)
    (:Update
      (Transformation|SetActorLocation _snowman_2 (Math|Vector|MakeVector (.x _returnvalue_2) (.y _returnvalue_2) (Math|Float|Lerp (.z _returnvalue) (- (.z _returnvalue) (Variables|Default|GetSpawnHeight)) _timerising)) false false)
      (Variables|Default|SetStartedSteal false))
    (:Finished
      ;[1 1 1] Delete old snowman first
      (Utilities|IsValid _snowman
        (:Is%20Valid
          (Actor|DestroyActor _snowman))))))

(event EventBeginPlay
  (bind _returnvalue (Actor|GetActorOfClass "/Game/Blueprints/Player/BP_ThirdPersonCharacter.BP_ThirdPersonCharacter_C"))
  (Variables|Default|SetPlayer _returnvalue)
  (Variables|Default|SetPlayerCollisionRef (Variables|/Script/Engine.Character|GetCapsuleComponent _returnvalue)))

(event EventTick
  (params (DeltaSeconds :type Float%20%28single-precision%29))
  ;[0.3 0.06262 1 1 42] HANDLES SNOWMAN DISAPPEARANCE WITH NEW UI
  (Utilities|IsValid (Variables|Default|GetSnowman)
    (:Is%20Valid
      (bind _output_get (Variables|Default|SetElapsedTime (+ DeltaSeconds (Variables|Default|GetElapsedTime))))
      (if (> _output_get (* (Variables|Default|GetUIAnimationSpeed) (Variables|Default|GetAnimationTime)))
        (CallFunction|SnowmanDisappear)
        (Variables|Default|SetElapsedTime 0.0)))))

(fn ConstructionScript)

(fn RemoveVisual
  (bind _player (Variables|Default|GetPlayer))
  (bind _mesh (Variables|/Script/Engine.Character|GetMesh _player))
  (Rendering|Material|SetMaterial _mesh 0 "/Game/Models/Map/Objects/Hat/M_Hat.M_Hat")
  (Rendering|Material|SetMaterial _mesh 10 "/Game/Meshes/Player/M_Button3.M_Button3")
  (Rendering|Material|SetMaterial _mesh 6 "/Game/Meshes/Player/Material_001.Material_001")
  (Rendering|Material|SetMaterial _mesh 9 "/Game/Meshes/Player/Materials/M_Hat.M_Hat"))