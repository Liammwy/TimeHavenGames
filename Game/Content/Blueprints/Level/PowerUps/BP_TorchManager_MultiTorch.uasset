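; Level manager Blueprint that tracks an array of torches and fires an event once all of them are lit.
; On BeginPlay it binds to each torch's ignition-state change and recounts the lit torches whenever one changes.
; When all are lit, it prints a message, notifies its EventListener, calls its OnAllTorchesIgnited dispatcher and marks every torch as permanently ignited.
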(event Custom|OnTorchIgnitionStateChanged
  (Variables|Default|SetnumTorchesIgnited 0)
  ;[1 1 1] Count how many torches are lit
  (for _array_element (Variables|Default|GetTorchRef_Array)
    (if (Variables|/Game/Blueprints/Level/PowerUps/BP_FireBreathTorch.BP_FireBreathTorch_C|GetIsIgnited _array_element)
      (Variables|Default|SetnumTorchesIgnited (+ (Variables|Default|GetnumTorchesIgnited) 1))))
  ;[1 1 1] Fire event if all torches lit
  (if (== (Variables|Default|GetnumTorchesIgnited) (Utilities|Array|Length (Variables|Default|GetTorchRef_Array)))
    (CallFunction|AllTochesIgnited)))

(event Custom|AllTochesIgnited
  (Development|PrintString "ALL IGNITED")
  (Default|RespondtoAllTorchesIgnited (Variables|Default|GetEventListener))
  (Default|CallOnAllTorchesIgnited)
  ;[1 1 1] Set all torches to stay lit once event fired
  (for _array_element (Variables|Default|GetTorchRef_Array)
    (Variables|/Game/Blueprints/Level/PowerUps/BP_FireBreathTorch.BP_FireBreathTorch_C|SetStayPermanentlyIgnited _array_element true)))

(event EventBeginPlay
  (for _array_element (Variables|Default|GetTorchRef_Array)
    (EventDispatchers|BindEventtoOnIgnitionStateChanged _array_element (delegate Custom|OnTorchIgnitionStateChanged))))

(fn ConstructionScript)