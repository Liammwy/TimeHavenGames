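; Level component that holds back a set of collectibles until SpawnCollectibles is called.
; On BeginPlay it turns off timeline updates and box collision on each entry in the Collectibles array.
; SpawnCollectibles re-enables both, using query-only collision, so the existing collectibles are toggled instead of created.
; FreezeAllCollectibles only prints the array length and freezes nothing.
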(event Custom|SpawnCollectibles
  ;[1 1 1] Call SpawnCollectibles to turn on visibility/collision for all collectibles
  (for _array_element (Variables|Default|GetCollectibles)
    (Collision|SetCollisionEnabled (Variables|/Game/Blueprints/Collectibles/BP_Collectible.BP_Collectible_C|GetBox _array_element) "QueryOnly")
    (Variables|/Game/Blueprints/Collectibles/BP_Collectible.BP_Collectible_C|SetUpdateWithTimelines _array_element true)))

(event EventBeginPlay
  ;[1 1 1] Hide all collectibles on BeginPlay
  (for _array_element (Variables|Default|GetCollectibles)
    (Variables|/Game/Blueprints/Collectibles/BP_Collectible.BP_Collectible_C|SetUpdateWithTimelines _array_element false)
    (Collision|SetCollisionEnabled (Variables|/Game/Blueprints/Collectibles/BP_Collectible.BP_Collectible_C|GetBox _array_element) "NoCollision")))

(fn FreezeAllCollectibles
  (Development|PrintString (Utilities|String|ToString(Integer) (Utilities|Array|Length (Variables|Default|GetCollectibles)))))