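; Level trigger volume that disables the player's jetpack hover while they stand inside it.
; On box overlap with BP_ThirdPersonCharacter, it sets the InHoverDisabledZone flag on the character's BPCHover component and activates the JetpackNotWorkingParticles effect.
; Leaving the box clears the flag and deactivates the particles.
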(event OnComponentBeginOverlap(noJetpackZoneBOX)
  (params (OverlappedComponent :type Primitive%20Component%20Object%20Reference) (OtherActor :type Actor%20Object%20Reference) (OtherComp :type Primitive%20Component%20Object%20Reference) (OtherBodyIndex :type Integer) (bFromSweep :type Boolean) (SweepResult :type Hit%20Result%20Structure%20%28by%20ref%29))
  (bind _asbp_third_person_character (Utilities|Casting|CastToBP_ThirdPersonCharacter OtherActor))
  (Variables|/Game/Blueprints/Player/Components/BPC_Hover.BPC_Hover_C|SetinHoverDisabledZone (Variables|/Game/Blueprints/Player/BP_ThirdPersonCharacter.BP_ThirdPersonCharacter_C|GetBPC_Hover _asbp_third_person_character) true)
  (Components|Activation|Activate (Variables|/Game/Blueprints/Player/BP_ThirdPersonCharacter.BP_ThirdPersonCharacter_C|GetjetpackNotWorkingParticles _asbp_third_person_character) true))

(event OnComponentEndOverlap(noJetpackZoneBOX)
  (params (OverlappedComponent :type Primitive%20Component%20Object%20Reference) (OtherActor :type Actor%20Object%20Reference) (OtherComp :type Primitive%20Component%20Object%20Reference) (OtherBodyIndex :type Integer))
  (bind _asbp_third_person_character (Utilities|Casting|CastToBP_ThirdPersonCharacter OtherActor))
  (Variables|/Game/Blueprints/Player/Components/BPC_Hover.BPC_Hover_C|SetinHoverDisabledZone (Variables|/Game/Blueprints/Player/BP_ThirdPersonCharacter.BP_ThirdPersonCharacter_C|GetBPC_Hover _asbp_third_person_character) false)
  (Components|Activation|Deactivate (Variables|/Game/Blueprints/Player/BP_ThirdPersonCharacter.BP_ThirdPersonCharacter_C|GetjetpackNotWorkingParticles _asbp_third_person_character)))

(fn ConstructionScript)