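; Level transition manager that opens the Tutorial level after a cutscene finishes.
; OnCutsceneFinished adds a WBP_FadeOut widget, plays its fade animation, waits for the animation's length, then opens the level.
; The logic to hide and disable the player, bind that event and play the sequence is disconnected, so this graph never starts the cutscene.
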(event Custom|OnCutsceneFinished
  (Development|PrintString "Cutscene Finished !" true true "(R=1.000000,G=0.797369,B=0.000000,A=1.000000)")
  (bind _returnvalue (UserInterface|CreateWidget "/Game/Blueprints/UI/TransitionScreens/WBP_FadeOut.WBP_FadeOut_C" (Game|GetPlayerController 0)))
  (UserInterface|Viewport|AddtoViewport _returnvalue 10)
  (UserInterface|Animation|PlayAnimation _returnvalue (Variables|/Game/Blueprints/UI/TransitionScreens/WBP_FadeOut.WBP_FadeOut_C|GetfadeOut _returnvalue) 0.0 1 "Forward" 1.0 false)
  (Utilities|FlowControl|Delay (Class|WidgetAnimation|GetEndTime (Variables|/Game/Blueprints/UI/TransitionScreens/WBP_FadeOut.WBP_FadeOut_C|GetfadeOut _returnvalue)))
  (Game|OpenLevel(byName) "Tutorial"))

(event EventBeginPlay)

(event Collision|EventActorBeginOverlap
  (params (OtherActor :type Actor%20Object%20Reference)))

(event EventTick
  (params (DeltaSeconds :type Float%20%28single-precision%29)))

(fn ConstructionScript)