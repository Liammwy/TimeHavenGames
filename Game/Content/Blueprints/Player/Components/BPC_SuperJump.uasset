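; Player component for the super jump scarf power, enabled when the scarf power manager reports that power as current.
; On input it cancels hover, uses up the jump count and launches by overriding BPCJump's height and time.
; Tick retunes gravity at 80% of the jump to slow the peak and re-enables hover.
; OnBlockHit applies the same gravity change to start falling, and OnLand restores the original jump values.
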(event Custom|OnLand
  (if (Variables|Default|GetisCurrentPower)
    (CallFunction|ResetBP)))

(event Custom|UpdateActivity
  (params (NewScarfType :type Enum_ScarfPowerType%20Enum :default "NewEnumerator0"))
  ;[1 1 1 1 45] Handle's power activity
  (if (Utilities|Enum|Equal(Enum) NewScarfType "NewEnumerator1")
    (Variables|Default|SetisCurrentPower true)
    (else
      (Variables|Default|SetisCurrentPower false))))

(event Custom|OnBlockHit
  (bind _player (Variables|Default|GetPlayer))
  (bind _bpc_jump (Variables|/Game/Blueprints/Player/BP_ThirdPersonCharacter.BP_ThirdPersonCharacter_C|GetBPC_Jump _player))
  ;[1 1 1] Ensures player starts falling after hitting a block. Not quite sure why this works, but not complaining
  (Variables|/Game/Blueprints/Player/Components/BPC_Jump.BPC_Jump_C|SetJumpHeight _bpc_jump 1e+01)
  (Variables|/Game/Blueprints/Player/Components/BPC_Jump.BPC_Jump_C|SetJumpTime _bpc_jump 0.75)
  (Default|ResetGravityScale _bpc_jump true)
  (Variables|Default|SetSlowedDownPeak true)
  (Variables|Default|SetTime%20since%20jump 0.0))

(event Input|EnhancedActionEvents|EnhancedInputActionIA_SuperJump
  (params (ActionValue :type Boolean) (ElapsedSeconds :type Float%20%28double-precision%29) (TriggeredSeconds :type Float%20%28double-precision%29) (InputAction :type Input%20Action%20Object%20Reference :default "/Game/Data/Input/Actions/IA_SuperJump.IA_SuperJump"))
  (bind _player (Variables|Default|GetPlayer))
  (bind _bpc_jump (Variables|/Game/Blueprints/Player/BP_ThirdPersonCharacter.BP_ThirdPersonCharacter_C|GetBPC_Jump _player))
  ;[1 1 1 1 29] Power used
  (:Started
    (if (and (Variables|Default|GetisCurrentPower) (not (Variables|Default|GetmidSuperJump)))
      (CallFunction|CancelHoverAbility)
      (Variables|Default|SetmidSuperJump true)
      (Class|FMODBlueprintStatics|PlayEvent2D "/Game/FMOD/Events/SuperJump.SuperJump")
      (Variables|/Game/Blueprints/Player/Components/BPC_Jump.BPC_Jump_C|SetJumpHeight _bpc_jump (Variables|Default|GetSuper%20Jump%20Height))
      (Variables|/Game/Blueprints/Player/Components/BPC_Jump.BPC_Jump_C|SetJumpTime _bpc_jump (Variables|Default|GetSuperJumpTime))
      (Default|ResetGravityScale _bpc_jump true)
      (Variables|/Game/Blueprints/Player/Components/BPC_Jump.BPC_Jump_C|SetSuperJumpJustStarted _bpc_jump true)
      (Default|HandleSuperJump _bpc_jump)
      (Variables|/Game/Blueprints/Player/Components/BPC_Jump.BPC_Jump_C|SetcurrentJumpCount _bpc_jump (Variables|/Game/Blueprints/Player/Components/BPC_Jump.BPC_Jump_C|GetmaxJumpCount _bpc_jump)))))

(event EventBeginPlay
  ;[1 1 1 1 45] Handle's power activity
  (bind _asbp_third_person_character (Utilities|Casting|CastToBP_ThirdPersonCharacter (Components|GetOwner)))
  (bind _output_get (Variables|Default|SetPlayer _asbp_third_person_character))
  (EventDispatchers|BindEventtoOnScarfPowerChanged (Variables|/Game/Blueprints/Player/BP_ThirdPersonCharacter.BP_ThirdPersonCharacter_C|GetBPC_ScarfPowerManager _asbp_third_person_character) (delegate Custom|UpdateActivity))
  (Variables|Default|SetOriginal%20Jump%20height (Variables|/Game/Blueprints/Player/Components/BPC_Jump.BPC_Jump_C|GetJumpHeight (Variables|/Game/Blueprints/Player/BP_ThirdPersonCharacter.BP_ThirdPersonCharacter_C|GetBPC_Jump _output_get)))
  (Variables|Default|SetOriginal%20Jump%20Time (Variables|/Game/Blueprints/Player/Components/BPC_Jump.BPC_Jump_C|GetJumpTime (Variables|/Game/Blueprints/Player/BP_ThirdPersonCharacter.BP_ThirdPersonCharacter_C|GetBPC_Jump _output_get))))

(event EventTick
  (params (DeltaSeconds :type Float%20%28single-precision%29))
  (bind _player (Variables|Default|GetPlayer))
  (bind _bpc_jump (Variables|/Game/Blueprints/Player/BP_ThirdPersonCharacter.BP_ThirdPersonCharacter_C|GetBPC_Jump _player))
  ;[1 1 1 1 37] Section of code to modify slow down speed of super jump
  (if (and (Variables|Default|GetmidSuperJump) (not (Variables|Default|GetSlowedDownPeak)))
    (bind _output_get (Variables|Default|SetTime%20since%20jump (+ (Variables|Default|GetTime%20since%20jump) DeltaSeconds)))
    (if (>= _output_get (* (Variables|Default|GetSuperJumpTime) 0.8))
      (Variables|/Game/Blueprints/Player/Components/BPC_Jump.BPC_Jump_C|SetJumpHeight _bpc_jump 1e+01)
      ;;[1 1 1] Increase number to reduce gravity
      (Variables|/Game/Blueprints/Player/Components/BPC_Jump.BPC_Jump_C|SetJumpTime _bpc_jump 0.75)
      (Default|ResetGravityScale _bpc_jump true)
      (Variables|Default|SetSlowedDownPeak true)
      (Variables|Default|SetTime%20since%20jump 0.0)
      ;[0.7699 1 0.4602] RETURN HOVER ON DESCENT
      (CallFunction|ReturnHoverAbility))))

(fn ResetJumpVariables
  (bind _player (Variables|Default|GetPlayer))
  (bind _bpc_jump (Variables|/Game/Blueprints/Player/BP_ThirdPersonCharacter.BP_ThirdPersonCharacter_C|GetBPC_Jump _player))
  (Variables|/Game/Blueprints/Player/Components/BPC_Jump.BPC_Jump_C|SetJumpHeight _bpc_jump (Variables|Default|GetOriginal%20Jump%20height))
  (Variables|/Game/Blueprints/Player/Components/BPC_Jump.BPC_Jump_C|SetJumpTime _bpc_jump (Variables|Default|GetOriginal%20Jump%20Time))
  (Default|ResetGravityScale _bpc_jump true)
  (Variables|/Game/Blueprints/Player/Components/BPC_Jump.BPC_Jump_C|SetSuperJumpJustStarted _bpc_jump false))

(fn ResetBP
  (CallFunction|ResetJumpVariables)
  (Variables|Default|SetmidSuperJump false)
  (Variables|Default|SetSlowedDownPeak false))

(fn CancelHoverAbility
  ;[1 1 1] CANCEL HOVER IF HOVERING (DOES IT BY DRAINING FUEL)
  (bind _asbp_third_person_character (Utilities|Casting|CastToBP_ThirdPersonCharacter (Components|GetOwner)))
  (Default|SJHoverCancel (Variables|/Game/Blueprints/Player/BP_ThirdPersonCharacter.BP_ThirdPersonCharacter_C|GetBPC_Hover _asbp_third_person_character)))

(fn ReturnHoverAbility
  ;[1 1 1] REFUEL HOVER ABILITY
  (bind _asbp_third_person_character (Utilities|Casting|CastToBP_ThirdPersonCharacter (Components|GetOwner)))
  (Variables|/Game/Blueprints/Player/Components/BPC_Hover.BPC_Hover_C|SethoverDepleted (Variables|/Game/Blueprints/Player/BP_ThirdPersonCharacter.BP_ThirdPersonCharacter_C|GetBPC_Hover _asbp_third_person_character) false))