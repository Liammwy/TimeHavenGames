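; Talkable NPC with snowman, penguin or signpost visuals, chosen in the construction script, that shows multi-line dialogue to the player.
; The first talk-radius overlap opens WBP_TalkingBox automatically; later visits require the interact input.
; Continue input skips typing or advances the Dialogue array, with Tick tracking typing progress.
; A separate hitbox raises a clamped, timeline-driven prompt, showing interact text or a quest popup depending on read state.
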(event OnComponentBeginOverlap(snowmantalkradius)
  (params (OverlappedComponent :type Primitive%20Component%20Object%20Reference) (OtherActor :type Actor%20Object%20Reference) (OtherComp :type Primitive%20Component%20Object%20Reference) (OtherBodyIndex :type Integer) (bFromSweep :type Boolean) (SweepResult :type Hit%20Result%20Structure%20%28by%20ref%29))
  (bind _talkingbox (Variables|Default|GetTalkingBox))
  ;[1 1 1 1 35] On player interact, if there is text within the array, set the text to the first array input
  (if (== OtherComp (Variables|Default|GetplayerCollisionRef))
    (Variables|Default|SetinTalkRadius true)
    (if (Variables|Default|GetfirstInteraction)
      (Variables|Default|SetfirstInteraction false)
      (Variables|/Game/Blueprints/UI/WBP_TalkingBox.WBP_TalkingBox_C|SetstopText (Variables|Default|GetTalkingBox) false)
      (Default|ResetText (Variables|Default|GetTalkingBox))
      (Variables|Default|SethasClosed false)
      (Input|EnableInput (Game|GetPlayerController 0))
      (if (not (== (Utilities|String|Len (Utilities|Array|Get(acopy) (Variables|Default|Getdialogue))) 0))
        (UserInterface|Viewport|AddtoViewport (Variables|Default|GetTalkingBox) 0)
        (Variables|/Game/Blueprints/UI/WBP_TalkingBox.WBP_TalkingBox_C|SetText%20Input _talkingbox (Utilities|Array|Get(acopy) (Variables|Default|Getdialogue)))
        (Default|IncrementDialogueNumber _talkingbox (Variables|Default|GetCurrentText) (Variables|Default|GetmaxDialogue))
        (Transformation|SetWorldLocation (Variables|Default|GetpromptWidget) (Variables|Default|GetdefaultWidgetLoc) false false)
        (Rendering|SetVisibility (Variables|Default|GetpromptWidget) false false)
        (Default|SetSnowmanName (Variables|Default|GetTalkingBox) (Variables|Default|GetsnowmanName)))
      (else
        (CallFunction|ShowManualInputPopup)))))

(event OnComponentEndOverlap(snowmantalkradius)
  (params (OverlappedComponent :type Primitive%20Component%20Object%20Reference) (OtherActor :type Actor%20Object%20Reference) (OtherComp :type Primitive%20Component%20Object%20Reference) (OtherBodyIndex :type Integer))
  (bind _talkingbox (Variables|Default|GetTalkingBox))
  ;[1 1 1 1 30] When leaving talk radius, close the dialogue
  (if (== OtherComp (Variables|Default|GetplayerCollisionRef))
    (Variables|Default|SetinTalkRadius false)
    (CallFunction|CloseDialogue)
    (if (Variables|Default|GethasReadQuest)
      (CallFunction|HideManualInputPopup)
      (else
        (CallFunction|QuestPopup)))
    (Default|ResetText _talkingbox)
    (Default|EndLoop _talkingbox)))

(event OnComponentBeginOverlap(promptHitbox)
  (params (OverlappedComponent :type Primitive%20Component%20Object%20Reference) (OtherActor :type Actor%20Object%20Reference) (OtherComp :type Primitive%20Component%20Object%20Reference) (OtherBodyIndex :type Integer) (bFromSweep :type Boolean) (SweepResult :type Hit%20Result%20Structure%20%28by%20ref%29))
  ;[1 1 1 1 30] Check to see if player overruns with prompt box, if so - check if they've already read the quest in it's entirety (if yes, don't show)
  (if (== OtherComp (Variables|Default|GetplayerCollisionRef))
    (if (Variables|Default|GethasReadQuest)
      (CallFunction|ReadQuestPopup)
      (else
        (CallFunction|QuestPopup)))))

(event OnComponentEndOverlap(promptHitbox)
  (params (OverlappedComponent :type Primitive%20Component%20Object%20Reference) (OtherActor :type Actor%20Object%20Reference) (OtherComp :type Primitive%20Component%20Object%20Reference) (OtherBodyIndex :type Integer))
  ;[1 1 1 1 30] Check if player overruns with prompt box
  (if (== OtherComp (Variables|Default|GetplayerCollisionRef))
    (Transformation|SetWorldLocation (Variables|Default|GetpromptWidget) (Variables|Default|GetdefaultWidgetLoc) false false)
    (Rendering|SetVisibility (Variables|Default|GetpromptWidget) false false)))

(event Custom|readQuestPopup
  (bind _defaultwidgetloc (Variables|Default|GetdefaultWidgetLoc))
  (CallFunction|HideManualInputPopup)
  (Rendering|SetVisibility (Variables|Default|GetpromptWidget) true false)
  (Variables|Default|SetwidgetLocation (Transformation|GetWorldLocation (Variables|Default|GetpromptWidget)))
  (bind _widgetrise (Timeline|Timeline_0 PlayFromStart)
    (:Update
      (Transformation|SetWorldLocation (Variables|Default|GetpromptWidget) (Math|Vector|MakeVector (.x (Variables|Default|GetwidgetLocation)) (.y (Variables|Default|GetwidgetLocation)) (Math|Float|Clamp(Float) (+ (.z (Variables|Default|GetwidgetLocation)) _widgetrise) (.z _defaultwidgetloc) (+ (.z _defaultwidgetloc) 5e+01))) false false))))

(event Custom|shouldSkipDialogue
  (bind _talkingbox (Variables|Default|GetTalkingBox))
  ;[1 1 1] Skipping dialogue
  (Default|SkipDialogue _talkingbox (Utilities|Array|Get(acopy) (Variables|Default|Getdialogue) (Variables|Default|GetCurrentText)))
  (Variables|/Game/Blueprints/UI/WBP_TalkingBox.WBP_TalkingBox_C|SetstopText _talkingbox true)
  (Variables|Default|SetisTalking false))

(event Custom|shouldContinueDialogue
  (bind _talkingbox (Variables|Default|GetTalkingBox))
  (Variables|Default|SetisTalking true)
  (bind _output_get (Variables|Default|SetCurrentText (+ (Variables|Default|GetCurrentText) 1)))
  (if (== _output_get (Variables|Default|GetmaxDialogue))
    (CallFunction|Close)
    (elif (== (Utilities|String|Len (Utilities|Array|Get(acopy) (Variables|Default|Getdialogue) (Variables|Default|GetCurrentText))) 0)
      (CallFunction|Close)
      (else
        (Variables|/Game/Blueprints/UI/WBP_TalkingBox.WBP_TalkingBox_C|SetstopText (Variables|Default|GetTalkingBox) false)
        (Default|IncrementDialogueNumber _talkingbox (Variables|Default|GetCurrentText) (Variables|Default|GetmaxDialogue))
        (Default|StartLoop _talkingbox)
        (Default|ResetText _talkingbox)
        (Variables|/Game/Blueprints/UI/WBP_TalkingBox.WBP_TalkingBox_C|SetText%20Input (Variables|Default|GetTalkingBox) (Utilities|Array|Get(acopy) (Variables|Default|Getdialogue) (Variables|Default|GetCurrentText)))))))

(event Custom|close
  ;[1 1 1] If the talking box has stopped talking, then we set the read quest to true and close dialogue
  (Variables|Default|SethasReadQuest true)
  (CallFunction|CloseDialogue)
  (Variables|Default|SetisTalking false)
  (Variables|Default|SethasClosed true)
  (if (not (Variables|Default|GetnotDefaultAnim))
    (Components|Animation|PlayAnimation (Variables|Default|GetPenguinVisuals) "/Game/Models/Map/Live/Penguin/PenguinV1_Anim.PenguinV1_Anim" false)
    (Rendering|SetVisibility (Variables|Default|GetpromptWidget) false false)))

(event Custom|playAnimation
  (if (Audio|Components|Audio|IsPlaying (Variables|Default|GetPenguinVisuals))
    (Variables|Default|SetnotDefaultAnim true)
    (else
      (Utilities|FlowControl|Delay (Math|Random|RandomFloatinRange 0.0 2.0))
      (Components|Animation|PlayAnimation (Variables|Default|GetPenguinVisuals) "/Game/Models/Map/Live/Penguin/PenguinAnimations/penguinWave.penguinWave" true))))

(event Custom|questPopup
  (bind _defaultwidgetloc (Variables|Default|GetdefaultWidgetLoc))
  ;[1 1 1 1 30] Logic for bobbing of the question mark - when it raises up to begin with (clamps to 100 above the default location, so it can never go higher)
  (Rendering|SetVisibility (Variables|Default|GetpromptWidget) true false)
  (Variables|Default|SetwidgetLocation (Transformation|GetWorldLocation (Variables|Default|GetpromptWidget)))
  (bind _widgetrise (Timeline|Timeline PlayFromStart)
    (:Update
      (Transformation|SetWorldLocation (Variables|Default|GetpromptWidget) (Math|Vector|MakeVector (.x (Variables|Default|GetwidgetLocation)) (.y (Variables|Default|GetwidgetLocation)) (Math|Float|Clamp(Float) (+ (.z (Variables|Default|GetwidgetLocation)) _widgetrise) (.z _defaultwidgetloc) (+ (.z _defaultwidgetloc) 5e+01))) false false))))

(event Custom|showManualInputPopup
  ;[1 1 1] Shows 'Press X - Interact' text
  (bind _aswbp_prompt (Utilities|Casting|CastToWBP_Prompt (UserInterface|GetWidget (Variables|Default|GetpromptWidget))))
  (Variables|/Script/UMG.Widget|SetVisibility (Variables|/Game/Blueprints/UI/WBP_Prompt.WBP_Prompt_C|GetRichTextBlock _aswbp_prompt) "Visible")
  (Variables|/Script/UMG.Widget|SetVisibility (Variables|/Game/Blueprints/UI/WBP_Prompt.WBP_Prompt_C|GetRichTextBlock_535 _aswbp_prompt) "Visible"))

(event Custom|hideManualInputPopup
  ;[1 1 1] Hides 'Press X - Interact' text
  (bind _aswbp_prompt (Utilities|Casting|CastToWBP_Prompt (UserInterface|GetWidget (Variables|Default|GetpromptWidget))))
  (Variables|/Script/UMG.Widget|SetVisibility (Variables|/Game/Blueprints/UI/WBP_Prompt.WBP_Prompt_C|GetRichTextBlock _aswbp_prompt) "Hidden")
  (Variables|/Script/UMG.Widget|SetVisibility (Variables|/Game/Blueprints/UI/WBP_Prompt.WBP_Prompt_C|GetRichTextBlock_535 _aswbp_prompt) "Hidden"))

(event Input|EnhancedActionEvents|EnhancedInputActionIA_ContinueDialogue
  (params (ActionValue :type Boolean) (ElapsedSeconds :type Float%20%28double-precision%29) (TriggeredSeconds :type Float%20%28double-precision%29) (InputAction :type Input%20Action%20Object%20Reference :default "/Game/Data/Input/Actions/IA_ContinueDialogue.IA_ContinueDialogue"))
  ;[1 1 1 1 45] Continue dialogue logic
  (if (not (Variables|Default|GethasClosed))
    (if (Variables|Default|GetisTalking)
      (CallFunction|ShouldSkipDialogue)
      (else
        (CallFunction|ShouldContinueDialogue)))))

(event Input|EnhancedActionEvents|EnhancedInputActionIA_Quest
  (params (ActionValue :type Boolean) (ElapsedSeconds :type Float%20%28double-precision%29) (TriggeredSeconds :type Float%20%28double-precision%29) (InputAction :type Input%20Action%20Object%20Reference :default "/Game/Data/Input/Actions/IA_Quest.IA_Quest"))
  (bind _talkingbox (Variables|Default|GetTalkingBox))
  ;[1 1 1 1 35] On player interact, if there is text within the array, set the text to the first array input
  (:Started
    (if (Variables|Default|GetinTalkRadius)
      (if (not (Widget|IsVisible (Variables|Default|GetTalkingBox)))
        (Variables|/Game/Blueprints/UI/WBP_TalkingBox.WBP_TalkingBox_C|SetstopText (Variables|Default|GetTalkingBox) false)
        (Default|ResetText (Variables|Default|GetTalkingBox))
        (Variables|Default|SethasClosed false)
        (Input|EnableInput (Game|GetPlayerController 0))
        (if (not (== (Utilities|String|Len (Utilities|Array|Get(acopy) (Variables|Default|Getdialogue))) 0))
          (UserInterface|Viewport|AddtoViewport (Variables|Default|GetTalkingBox) 0)
          (Variables|/Game/Blueprints/UI/WBP_TalkingBox.WBP_TalkingBox_C|SetText%20Input _talkingbox (Utilities|Array|Get(acopy) (Variables|Default|Getdialogue)))
          (Default|IncrementDialogueNumber _talkingbox (Variables|Default|GetCurrentText) (Variables|Default|GetmaxDialogue))
          (Transformation|SetWorldLocation (Variables|Default|GetpromptWidget) (Variables|Default|GetdefaultWidgetLoc) false false)
          (Rendering|SetVisibility (Variables|Default|GetpromptWidget) false false)
          (Default|SetSnowmanName (Variables|Default|GetTalkingBox) (Variables|Default|GetsnowmanName)))))))

(event EventTick
  (params (DeltaSeconds :type Float%20%28single-precision%29))
  (if (== (Variables|/Game/Blueprints/UI/WBP_TalkingBox.WBP_TalkingBox_C|GetnumOfCharCounter (Variables|Default|GetTalkingBox)) (Utilities|String|Len (Utilities|Array|Get(acopy) (Variables|Default|Getdialogue) (Variables|Default|GetCurrentText))))
    (Variables|Default|SetisTalking false)
    (else
      (Variables|Default|SetisTalking true))))

(event EventBeginPlay
  ;[1 1 1 1 30] Create snowman talking text
  (CallFunction|HideManualInputPopup)
  (CallFunction|PlayAnimation)
  (bind _returnvalue (Actor|GetActorOfClass "/Game/Blueprints/Player/BP_ThirdPersonCharacter.BP_ThirdPersonCharacter_C"))
  (Variables|Default|SetplayerRef _returnvalue)
  (Variables|Default|SetplayerCollisionRef (Variables|/Script/Engine.Character|GetCapsuleComponent _returnvalue))
  (bind _returnvalue_2 (UserInterface|CreateWidget "/Game/Blueprints/UI/WBP_TalkingBox.WBP_TalkingBox_C"))
  (Variables|Default|SetTalkingBox _returnvalue_2)
  (Variables|Default|SetdefaultWidgetLoc (Transformation|GetWorldLocation (Variables|Default|GetpromptWidget)))
  (for _array_element (Variables|Default|Getdialogue)
    (if (not (== (Utilities|String|Len _array_element) 0))
      (Math|Integer|IncrementInt (Variables|Default|GetmaxDialogue)))))

(fn ConstructionScript
  (CallFunction|SetVisuals) ; Set model visuals snowman/penguin/signpost
  (Components|Box|SetBoxExtent (Variables|Default|GetpromptHitbox) (Variables|Default|GetwidgetShowDistance) true)
  (if (Utilities|Enum|Equal(Enum) (Variables|Default|GetvisualsType) "NewEnumerator1")
    (Transformation|AddWorldOffset (Variables|Default|GetpromptWidget) "0.000000,0.000000,-125.000000" false false)))

(fn CloseDialogue
  (Widget|RemovefromParent (Variables|Default|GetTalkingBox))
  (Variables|Default|SetCurrentText 0)
  (if (Variables|Default|GethasClosed)
    _
    (else
      ;[1 1 1] update state system so jump button works
      (Default|OnTalkStop (Variables|/Game/Blueprints/Player/BP_ThirdPersonCharacter.BP_ThirdPersonCharacter_C|GetBPC_StateSystem (Variables|Default|GetplayerRef)))))
  (Variables|Default|SethasClosed true))

(fn SetVisuals
  (bind _visualstype (Variables|Default|GetvisualsType))
  (bind _returnvalue (Utilities|Enum|Equal(Enum) _visualstype "NewEnumerator2"))
  ;[1 1 1] snowman visuals
  (Rendering|SetVisibility (Variables|Default|GetSphere3) (Utilities|Enum|Equal(Enum) (Variables|Default|GetvisualsType) "NewEnumerator0") false)
  ;[1 1 1] penguin visuals
  (Rendering|SetVisibility (Variables|Default|GetPenguinVisuals) (Utilities|Enum|Equal(Enum) (Variables|Default|GetvisualsType) "NewEnumerator1") false)
  (Rendering|SetVisibility (Variables|Default|GetSignpostVisuals) _returnvalue false)
  (Rendering|SetVisibility (Variables|Default|GetWidget) _returnvalue false))