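; Fire-breath tutorial actor that ignites when the player's fire breath hits it, making linked sad penguins play a looping celebration.
; FireHitbox overlaps with the player's three breath colliders trigger SetIsIgnited, which toggles the fire particle and broadcasts state changes, alongside a point light.
; Tick handles an optional burn time limit, and player respawn extinguishes the fire unless permanently ignited.
; UpdateFlameSize scales flame by remaining time but is not called here.
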(event OnComponentBeginOverlap(FireHitbox)
  (params (OverlappedComponent :type Primitive%20Component%20Object%20Reference) (OtherActor :type Actor%20Object%20Reference) (OtherComp :type Primitive%20Component%20Object%20Reference) (OtherBodyIndex :type Integer) (bFromSweep :type Boolean) (SweepResult :type Hit%20Result%20Structure%20%28by%20ref%29))
  (if (not (Variables|Default|GetIsIgnited))
    (if (Math|Boolean|ORBoolean (== OtherComp (Variables|Default|GetFireColl_0)) (== OtherComp (Variables|Default|GetFireColl_1)) (== OtherComp (Variables|Default|GetFireColl_2)))
      (Rendering|SetVisibility (Variables|Default|GetPointLight) true false)
      (CallFunction|SetIsIgnited true)
      (for _array_element (Variables|Default|GetsadPenguins)
        (Components|Animation|PlayAnimation (Variables|/Game/Blueprints/LevelAnimations/BP_PenguinSad.BP_PenguinSad_C|GetSkeletalMesh _array_element) "/Game/Models/Map/Live/Penguin/penguin_celebrate.penguin_celebrate" true)))))

(event Custom|OnPlayerRespawn
  (CallFunction|SetIsIgnited false))

(event EventBeginPlay
  (CallFunction|SetIsIgnited false)
  (bind _returnvalue (Actor|GetActorOfClass "/Game/Blueprints/Player/BP_ThirdPersonCharacter.BP_ThirdPersonCharacter_C"))
  (Variables|Default|SetPlayerRef _returnvalue)
  (Variables|Default|SetFireColl_0 (Variables|/Game/Blueprints/Player/BP_ThirdPersonCharacter.BP_ThirdPersonCharacter_C|GetFireBreathCollision _returnvalue))
  (Variables|Default|SetFireColl_1 (Variables|/Game/Blueprints/Player/BP_ThirdPersonCharacter.BP_ThirdPersonCharacter_C|GetFireBreathCollision1 _returnvalue))
  (Variables|Default|SetFireColl_2 (Variables|/Game/Blueprints/Player/BP_ThirdPersonCharacter.BP_ThirdPersonCharacter_C|GetFireBreathCollision2 _returnvalue))
  (EventDispatchers|BindEventtoOnRespawnDelayStarted _returnvalue (delegate Custom|OnPlayerRespawn)))

(event EventTick
  (params (DeltaSeconds :type Float%20%28single-precision%29))
  (CallFunction|UpdateIgnition DeltaSeconds))

(fn ConstructionScript)

(fn SetIsIgnited
  (params (Ignited :type Boolean))
  (if Ignited
    _
    (else
      ;[1 1 1] If trying to extinguish, check if fire should stay lit and cancel
      (if (Variables|Default|GetStayPermanentlyIgnited)
        (return)
        (else
          _))))
  (bind _output_get (Variables|Default|SetIsIgnited Ignited))
  (if _output_get
    (Rendering|SetVisibility (Variables|Default|GetFireParticle) true false)
    (Variables|Default|SetCurrentTimeIgnited 0.0)
    (else
      (Rendering|SetVisibility (Variables|Default|GetFireParticle) false false)))
  (Default|CallOnIgnitionStateChanged))

(fn UpdateIgnition
  (params (deltaTime :type Float%20%28double-precision%29))
  (if (Variables|Default|GetIsIgnited)
    (bind _output_get (Variables|Default|SetCurrentTimeIgnited (+ (Variables|Default|GetCurrentTimeIgnited) deltaTime)))
    (if (Variables|Default|GetHasTimeLimit)
      (if (>= _output_get (Variables|Default|GetIgniteTimeLimit))
        (CallFunction|SetIsIgnited false)
        (Rendering|SetVisibility (Variables|Default|GetPointLight) false false)))
    (else
      (return))))

(fn UpdateFlameSize
  (bind _currenttimeignited (Variables|Default|GetCurrentTimeIgnited))
  (bind _ignitetimelimit (Variables|Default|GetIgniteTimeLimit))
  (bind _returnvalue (/ _currenttimeignited _ignitetimelimit))
  (bind _returnvalue_2 (- 1.0 _returnvalue))
  (bind _returnvalue_3 (Math|Float|Clamp(Float) _returnvalue_2))
  (if (Variables|Default|GetIsIgnited)
    (if (Variables|Default|GetHasTimeLimit)
      (Development|PrintString (Utilities|String|ToString(Float) _returnvalue_3))
      (Transformation|SetWorldScale3D (Variables|Default|GetFireParticle) (Math|Vector|MakeVector _returnvalue_3 _returnvalue_3 _returnvalue_3))
      (else
        (Transformation|SetRelativeScale3D (Variables|Default|GetFireParticle) "1.000000,1.000000,1.000000")
        (return)))
    (else
      (return))))