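; Level path actor that moves a referenced Snowball actor along its spline in an endless loop.
; The construction script snaps the snowball to the first spline point.
; From BeginPlay, a timeline with play rate scaled by TimeToComplete drives distance along the spline, updating position and rotation, then restarts when finished.
; Rotation takes the raw spline tangent components as roll, pitch and yaw, rather than converting the direction to a rotator.
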(event Custom|PlayTimeline
  (bind _spline (Variables|Default|GetSpline))
  (bind _spline_2 (Variables|Default|GetSpline))
  (bind _snowball (Variables|Default|GetSnowball))
  (bind _timeline (Timeline|Timeline PlayFromStart)
    (:Update
      (Transformation|SetActorLocation _snowball (Spline|GetLocationatDistanceAlongSpline _spline_2 (Math|Float|Lerp 0.0 (Spline|GetDistanceAlongSplineatSplinePoint _spline (- (Spline|GetNumberOfSplinePoints _spline) 1)) _timeline) "World") false false)
      (Transformation|SetActorRotation _snowball (Math|Rotator|MakeRotator (.x (Spline|GetTangentatDistanceAlongSpline _spline_2 (Math|Float|Lerp 0.0 (Spline|GetDistanceAlongSplineatSplinePoint _spline (- (Spline|GetNumberOfSplinePoints _spline) 1)) _timeline) "World")) (.y (Spline|GetTangentatDistanceAlongSpline _spline_2 (Math|Float|Lerp 0.0 (Spline|GetDistanceAlongSplineatSplinePoint _spline (- (Spline|GetNumberOfSplinePoints _spline) 1)) _timeline) "World")) (.z (Spline|GetTangentatDistanceAlongSpline _spline_2 (Math|Float|Lerp 0.0 (Spline|GetDistanceAlongSplineatSplinePoint _spline (- (Spline|GetNumberOfSplinePoints _spline) 1)) _timeline) "World")))))
    (:Finished
      (CallFunction|PlayTimeline))))

(event EventBeginPlay
  (Components|Timeline|SetPlayRate (Variables|Default|GetTimeline) (/ 1.0 (Variables|Default|GetTimeToComplete)))
  (CallFunction|PlayTimeline))

(fn ConstructionScript
  (Transformation|SetActorLocation (Variables|Default|GetSnowball) (Spline|GetLocationatSplinePoint (Variables|Default|GetSpline) 0 "World") false false))