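; Moving platform actor that travels between its placed position and a relative target offset, Movtopos.
; The construction script adds both control points to an InterpToMovement component and uses Speed as its Duration, so larger values move it slower.
; BeginPlay enables player input and applies Scale to the cube's X and Y, keeping Z.
; Tick toggles the movement component's tick from CanMove every frame to run or pause motion.
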(event EventBeginPlay
  (bind _cube (Variables|Default|GetCube))
  (bind _scale (Variables|Default|GetScale))
  (Input|EnableInput (Game|GetPlayerController 0))
  ;[1 1 1] Takes inspector parameter 'Scale' and changes the size of the moving platform
  (Transformation|SetRelativeScale3D _cube (Math|Vector|MakeVector _scale _scale (.z (Variables|/Script/Engine.SceneComponent|GetRelativeScale3D _cube)))))

(event Collision|EventActorBeginOverlap
  (params (OtherActor :type Actor%20Object%20Reference)))

(event EventTick
  (params (DeltaSeconds :type Float%20%28single-precision%29))
  (Components|Tick|SetComponentTickEnabled (Variables|Default|GetInterpToMovement) (Variables|Default|GetCanMove)))

(fn ConstructionScript
  (bind _interptomovement (Variables|Default|GetInterpToMovement))
  (Class|InterptoMovementComponent|AddControlPointPosition _interptomovement "0, 0, 0" true)
  (Class|InterptoMovementComponent|AddControlPointPosition (Variables|Default|GetInterpToMovement) (Variables|Default|Getmovtopos) true)
  (Variables|/Script/Engine.InterpToMovementComponent|SetDuration _interptomovement (Variables|Default|GetSpeed)))