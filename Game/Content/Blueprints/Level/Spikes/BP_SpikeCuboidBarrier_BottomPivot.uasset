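; A bottom-pivot spike cuboid barrier that forces the player to respawn on contact.
; On BeginPlay it caches the BP_ThirdPersonCharacter and its capsule, and the DeathTrigger overlap calls ForceRespawn only when that capsule enters.
; MoveFloorCrack is empty, with an unconnected debug line trace that would trace downward from Visuals to place a component on the surface hit.
; The construction script does nothing.
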(event OnComponentBeginOverlap(DeathTrigger)
  (params (OverlappedComponent :type Primitive%20Component%20Object%20Reference) (OtherActor :type Actor%20Object%20Reference) (OtherComp :type Primitive%20Component%20Object%20Reference) (OtherBodyIndex :type Integer) (bFromSweep :type Boolean) (SweepResult :type Hit%20Result%20Structure%20%28by%20ref%29))
  (if (== OtherComp (Variables|Default|GetplayerHitboxRef))
    (Default|ForceRespawn (Variables|Default|GetplayerRef))))

(event EventBeginPlay
  (bind _returnvalue (Actor|GetActorOfClass "/Game/Blueprints/Player/BP_ThirdPersonCharacter.BP_ThirdPersonCharacter_C"))
  (Variables|Default|SetplayerRef _returnvalue)
  (Variables|Default|SetplayerHitboxRef (Variables|/Script/Engine.Character|GetCapsuleComponent _returnvalue)))

(fn ConstructionScript)

(fn MoveFloorCrack)