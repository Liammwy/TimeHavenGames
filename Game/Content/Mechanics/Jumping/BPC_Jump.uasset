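; BPC_Jump is a player component that handles multi-jump with variable height through the IA_Jump input.
; On press, it launches the third-person character upward, overriding vertical velocity, while the jump count is below its maximum.
; On release, it zeroes any upward velocity to cut the jump short, and a landing event resets the count.
; While triggered, it also calls JumpFromWall on the owner's climbing component.
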(event Custom|OnPlayerLandedEvent
  (Variables|Default|SetcurrentJumpCount 0))

(event Input|EnhancedActionEvents|EnhancedInputActionIA_Jump
  (params (ActionValue :type Boolean) (ElapsedSeconds :type Float%20%28double-precision%29) (TriggeredSeconds :type Float%20%28double-precision%29) (InputAction :type Input%20Action%20Object%20Reference :default "/Game/ThirdPerson/Input/Actions/IA_Jump.IA_Jump"))
  (:Triggered
    (Default|JumpfromWall (Actor|GetComponentbyClass (Components|GetOwner) "/Game/Mechanics/WallClimbing/BPC_Climbing.BPC_Climbing_C")))
  (:Started
    (if (< (Variables|Default|GetcurrentJumpCount) (Variables|Default|GetmaxJumpCount))
      (bind _asbp_third_person_character (Utilities|Casting|CastToBP_ThirdPersonCharacter (Components|GetOwner)))
      (Character|LaunchCharacter _asbp_third_person_character (Math|Vector|MakeVector 0.0 0.0 (Variables|Default|GetjumpVelocity)) false true)
      (Variables|Default|SetcurrentJumpCount (+ (Variables|Default|GetcurrentJumpCount) 1))))
  (:Completed
    (bind _asbp_third_person_character_2 (Utilities|Casting|CastToBP_ThirdPersonCharacter (Components|GetOwner)))
    (if (> (.z (Variables|/Script/Engine.MovementComponent|GetVelocity (Variables|/Script/Engine.Character|GetCharacterMovement _asbp_third_person_character_2))) 0.0)
      (Variables|/Script/Engine.MovementComponent|SetVelocity (Variables|/Script/Engine.Character|GetCharacterMovement _asbp_third_person_character_2) (Math|Vector|MakeVector (.x (Variables|/Script/Engine.MovementComponent|GetVelocity (Variables|/Script/Engine.Character|GetCharacterMovement _asbp_third_person_character_2))) (.y (Variables|/Script/Engine.MovementComponent|GetVelocity (Variables|/Script/Engine.Character|GetCharacterMovement _asbp_third_person_character_2))) 0.0)))))