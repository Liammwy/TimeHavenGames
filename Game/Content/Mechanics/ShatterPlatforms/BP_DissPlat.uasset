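; BP_DissPlat is a disappearing platform that vanishes shortly after the player steps on it, then respawns.
; On BeginPlay it caches the third-person character's capsule, and the trigger Box reacts only to that component.
; An overlap turns the Cube red as a warning, waits, then hides it and disables its collision.
; After a second delay it restores the material, visibility and collision.
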(event OnComponentBeginOverlap(Box)
  (params (OverlappedComponent :type Primitive%20Component%20Object%20Reference) (OtherActor :type Actor%20Object%20Reference) (OtherComp :type Primitive%20Component%20Object%20Reference) (OtherBodyIndex :type Integer) (bFromSweep :type Boolean) (SweepResult :type Hit%20Result%20Structure%20%28by%20ref%29))
  (if (== OtherComp (Variables|Default|GetPlayerHitboxRef))
    (Rendering|Material|SetMaterial (Variables|Default|GetCube) 0 "/Game/Materials/Level/MAT_Red.MAT_Red")
    (Utilities|FlowControl|Delay (Variables|Default|GetTimeToDisappear))
    (Rendering|SetVisibility (Variables|Default|GetCube) false false)
    (Collision|SetCollisionEnabled (Variables|Default|GetCube) "NoCollision")
    (Utilities|FlowControl|Delay (Variables|Default|GetTimeToRespawn))
    (Rendering|Material|SetMaterial (Variables|Default|GetCube) 0 "/Game/StarterContent/Materials/M_AssetPlatform.M_AssetPlatform")
    (Rendering|SetVisibility (Variables|Default|GetCube) true false)
    (Collision|SetCollisionEnabled (Variables|Default|GetCube) "QueryAndPhysics")))

(event EventBeginPlay
  (bind _returnvalue (Actor|GetActorOfClass "/Game/Blueprints/Player/BP_ThirdPersonCharacter.BP_ThirdPersonCharacter_C"))
  (Variables|Default|SetPlayerHitboxRef (Variables|/Script/Engine.Character|GetCapsuleComponent _returnvalue)))

(fn ConstructionScript)