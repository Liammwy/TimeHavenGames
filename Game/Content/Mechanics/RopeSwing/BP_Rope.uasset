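; Rope swing actor that attaches the player to a cable when they touch its capsule trigger.
; On overlap it sets movement to Flying, attaches the cable end, binds the player's capsule to a physics constraint, simulates physics and enables input.
; Q releases the rope, stopping simulation, resetting capsule yaw and setting movement mode to None.
; Move input currently adds zero force, as the forward-push calculation is unconnected.
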(event OnComponentBeginOverlap(Capsule)
  (params (OverlappedComponent :type Primitive%20Component%20Object%20Reference) (OtherActor :type Actor%20Object%20Reference) (OtherComp :type Primitive%20Component%20Object%20Reference) (OtherBodyIndex :type Integer) (bFromSweep :type Boolean) (SweepResult :type Hit%20Result%20Structure%20%28by%20ref%29))
  (bind _returnvalue (Game|GetPlayerCharacter 0))
  (bind _returnvalue_2 (Game|GetPlayerCharacter 0))
  (bind _cable (Variables|Default|GetCable))
  (bind _capsulecomponent (Variables|/Script/Engine.Character|GetCapsuleComponent _returnvalue_2))
  (if (== OtherActor _returnvalue)
    (Pawn|Components|CharacterMovement|SetMovementMode (Variables|/Script/Engine.Character|GetCharacterMovement _returnvalue) "MOVE_Flying" 0)
    (Class|CableComponent|SetAttachEndto _cable _returnvalue_2 "None" "None")
    (Variables|/Script/CableComponent.CableComponent|SetbAttachEnd _cable true)
    (Class|PhysicsConstraintComponent|SetConstrainedComponents (Variables|Default|GetPhysicsConstraint) _capsulecomponent "None" 0 "None")
    (Physics|SetSimulatePhysics _capsulecomponent true)
    (Input|EnableInput (Game|GetPlayerController 0) 0)))

(event Input|EnhancedActionEvents|EnhancedInputActionIA_Move
  (params (ActionValue :type Vector%202D%20Structure) (ElapsedSeconds :type Float%20%28double-precision%29) (TriggeredSeconds :type Float%20%28double-precision%29) (InputAction :type Input%20Action%20Object%20Reference :default "/Game/Data/Input/Actions/IA_Move.IA_Move"))
  (:Triggered
    (Physics|AddForce (Variables|/Script/Engine.Character|GetCapsuleComponent (Game|GetPlayerCharacter 0)) "0, 0, 0" "None" false)))

(event EventBeginPlay)

(event Collision|EventActorBeginOverlap
  (params (OtherActor :type Actor%20Object%20Reference)))

(event EventTick
  (params (DeltaSeconds :type Float%20%28single-precision%29)))

(event Input|KeyboardEvents|Q
  (params (Key :type Key%20Structure :default "None"))
  (bind _returnvalue (Game|GetPlayerCharacter 0))
  (bind _cable (Variables|Default|GetCable))
  (bind _capsulecomponent (Variables|/Script/Engine.Character|GetCapsuleComponent _returnvalue))
  (:Pressed
    (Pawn|Components|CharacterMovement|SetMovementMode (Variables|/Script/Engine.Character|GetCharacterMovement _returnvalue) "MOVE_None" 0)
    (Physics|SetSimulatePhysics _capsulecomponent false)
    (Transformation|SetWorldRotation _capsulecomponent (Math|Rotator|MakeRotator 0.0 0.0 (.yaw (Pawn|GetControlRotation _returnvalue :!class /Script/Engine.Pawn))) false false)
    (Class|PhysicsConstraintComponent|SetConstrainedComponents (Variables|Default|GetPhysicsConstraint) 0 "None" 0 "None")
    (Class|CableComponent|SetAttachEndto _cable 0 "None" "None")
    (Variables|/Script/CableComponent.CableComponent|SetbAttachEnd _cable false)))

(fn ConstructionScript)