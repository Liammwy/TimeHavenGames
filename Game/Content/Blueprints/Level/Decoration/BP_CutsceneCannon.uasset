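; Cutscene cannon that automatically fires a single snowball after a configurable delay from BeginPlay.
; Firing spawns a BP_SnowballCutscene above the cannon with yaw flipped, activates the cannon's Niagara effect and starts a timeline recoil along world X.
; Fixed delays then hide the snowball, trigger its own Niagara effect and destroy it, with no collision check involved.
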(event Custom|Recoil
  (bind _cannon (Variables|Default|GetCannon))
  (bind _returnvalue (Transformation|GetWorldLocation _cannon))
  (bind _output_get (Variables|Default|SetReturn%20Value%20X (.x _returnvalue)))
  (bind _recoil_amount (Timeline|Timeline PlayFromStart)
    (:Update
      (Transformation|SetWorldLocation (Variables|Default|GetCannon) (Math|Vector|MakeVector (+ _output_get _recoil_amount) (.y _returnvalue) (.z _returnvalue)) false false))))

(event Custom|fireCannon
  (bind _cannon (Variables|Default|GetCannon))
  (bind _returnvalue (Transformation|GetWorldTransform _cannon))
  (bind _returnvalue_2 (Game|SpawnActorfromClass "/Game/Blueprints/Level/Decoration/BP_SnowballCutscene.BP_SnowballCutscene_C" (Math|Transform|MakeTransform (Math|Vector|MakeVector (.x (.location _returnvalue)) (.y (.location _returnvalue)) (+ (.z (.location _returnvalue)) 2e+02)) (Math|Rotator|MakeRotator (.roll (.rotation _returnvalue)) (.pitch (.rotation _returnvalue)) (+ (.yaw (.rotation _returnvalue)) 1.8e+02)) (.scale _returnvalue)) "Undefined" "MultiplyWithRoot" 0 0))
  (Variables|Default|SetsnowBallVAR _returnvalue_2)
  (CallFunction|Recoil)
  (Components|Activation|Activate (Variables|Default|GetNiagara) true))

(event EventBeginPlay
  (bind _snowballvar (Variables|Default|GetsnowBallVAR))
  (Utilities|FlowControl|Delay (Variables|Default|GetdelayTimer))
  (CallFunction|FireCannon)
  (Utilities|FlowControl|Delay 0.275)
  (Rendering|SetVisibility (Variables|/Game/Blueprints/Level/Decoration/BP_SnowballCutscene.BP_SnowballCutscene_C|GetSnowball _snowballvar) false false)
  (Components|Activation|Activate (Variables|/Game/Blueprints/Level/Decoration/BP_SnowballCutscene.BP_SnowballCutscene_C|GetNiagara _snowballvar) true)
  (Utilities|FlowControl|Delay 0.75)
  (Actor|DestroyActor _snowballvar))

(fn ConstructionScript)