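; Player component that tracks which scarf power is currently active and exposes a getter and setter for it.
; Setting a power stores it, plays the scarf equip sound and broadcasts OnScarfPowerChanged.
; It then casts the owner to BP_ThirdPersonCharacter to update the equipped-scarf widget directly, a link marked as temporary.
; ApplyComponent is an empty stub.
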(event EventBeginPlay)

(event EventTick
  (params (DeltaSeconds :type Float%20%28single-precision%29)))

(fn SetScarfPower
  (params (ScarfPowerType :type Enum_ScarfPowerType%20Enum :default "NewEnumerator0"))
  (bind _output_get (Variables|Default|SetCurrentActivePower ScarfPowerType))
  (Class|FMODBlueprintStatics|PlayEvent2D "/Game/FMOD/Events/ScarfEquip.ScarfEquip")
  (Default|CallOnScarfPowerChanged _output_get)
  ;[1 0.375 0.375] PURELY TEMPORARY
  (bind _asbp_third_person_character (Utilities|Casting|CastToBP_ThirdPersonCharacter (Components|GetOwner)))
  (Default|UpdateScarfEquipped (Variables|/Game/Blueprints/Player/BP_ThirdPersonCharacter.BP_ThirdPersonCharacter_C|GetscarfEquippedWidget _asbp_third_person_character) (Variables|Default|GetCurrentActivePower)))

(fn ApplyComponent)

(fn GetScarfPower
  (return (Variables|Default|GetCurrentActivePower)))