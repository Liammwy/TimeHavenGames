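; BP_MeltIceCollectible is a level power-up actor, named as meltable ice, that releases a collectible rune once destroyed.
; Tick watches the IsDestroyed flag and calls SpawnRune only once, guarded by SpawnedRune.
; SpawnRune spawns a BP_Collectible slightly above the root component's transform, then calls GrowIn on it.
; The melting and destruction logic is not in these graphs, which only react to the flag.
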(event EventBeginPlay
  (|CallParentFunction) ; This node is disabled and will not be called.\nDrag off pins to build functionality.
)

(event Collision|EventActorBeginOverlap
  (params (OtherActor :type Actor%20Object%20Reference)))

(event EventTick
  (params (DeltaSeconds :type Float%20%28single-precision%29))
  ;[1 1 1] SPAWN ONCE DESTROYED
  (|CallParentFunction DeltaSeconds)
  (if (and (Variables|Default|GetisDestroyed) (not (Variables|Default|GetSpawnedRune)))
    (Variables|Default|SetSpawnedRune true)
    (CallFunction|SpawnRune)))

(fn ConstructionScript
  (|CallParentFunction))

(fn SpawnRune
  (bind _defaultsceneroot (Variables|Default|GetDefaultSceneRoot))
  (bind _returnvalue (Transformation|GetRelativeTransform _defaultsceneroot))
  ;[1 0.2528 0.1129] SPAWN THE RUNE
  (bind _returnvalue_2 (Game|SpawnActorfromClass "/Game/Blueprints/Collectibles/BP_Collectible.BP_Collectible_C" (Math|Transform|MakeTransform (+ (.location _returnvalue) "0.000000,0.000000,25.000000") (.rotation _returnvalue) (.scale _returnvalue)) "Undefined" "MultiplyWithRoot" 0 0))
  (Default|Growin _returnvalue_2))