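; Player jump component for BP_ThirdPersonCharacter, handling ground, midair and super jumps, plus handoff to wall jumps.
; Derives launch velocity and gravity scale from jump height and time, recalculating gravity on early release for variable height.
; Input passes through jump-count, hover and bounce-pad cooldown checks, with coyote time, trace-based landing buffer and a bigger bounce for presses during pad cooldown.
; Landing resets count and gravity, then fires buffered jumps.
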(event Custom|OnPlayerLandedEvent
  (Variables|Default|SetSuperJumpJustStarted true)
  (bind _asbp_third_person_character (Utilities|Casting|CastToBP_ThirdPersonCharacter (Components|GetOwner)))
  ;[1 1 1] Reset jump count on land
  (Components|Activation|SetActive (Variables|/Game/Blueprints/Player/BP_ThirdPersonCharacter.BP_ThirdPersonCharacter_C|GetdobuleJumpFX _asbp_third_person_character) false true)
  (Variables|Default|SetcurrentJumpCount 0)
  ;[1 1 1] Reset Gravity Scale
  (CallFunction|ResetGravityScale true)
  (if (Utilities|IsValid (Variables|Default|GetRecentBouncePad))
    (Variables|Default|SetRecentBouncePad 0)
    (if (Variables|Default|GethasBufferedJump)
      (Variables|Default|SethasBufferedJump false))
    (else
      ;[1 1 1] If player has stored jump buffer, wipe that value and handle jump
      (if (Variables|Default|GethasBufferedJump)
        (Variables|Default|SethasBufferedJump false)
        (bind _jumpallowed (CallFunction|CanPlayerJump))
        (if _jumpallowed
          (CallFunction|HandleJump true))))))

(event Custom|OnBouncePadLaunch
  (params (BouncePad :type BP%20Bounce%20Pad%20Object%20Reference))
  (Variables|Default|SettimeSinceLastBouncePad 0.0)
  (Variables|Default|SetRecentBouncePad BouncePad))

(event Custom|OnPlayerStateChanged
  ;[1 1 1] Setup state change event binding
  (if (Utilities|Enum|Equal(Enum) (Variables|/Game/Blueprints/Player/Components/BPC_StateSystem.BPC_StateSystem_C|GetCurrentState (Variables|/Game/Blueprints/Player/BP_ThirdPersonCharacter.BP_ThirdPersonCharacter_C|GetBPC_StateSystem (stale EventBeginPlay _asbp_third_person_character))) "NewEnumerator4")
    (Variables|Default|SetCT_TimeSinceMidairNoJump 0.0)))

(event Input|EnhancedActionEvents|EnhancedInputActionIA_Jump
  (params (ActionValue :type Boolean) (ElapsedSeconds :type Float%20%28double-precision%29) (TriggeredSeconds :type Float%20%28double-precision%29) (InputAction :type Input%20Action%20Object%20Reference :default "/Game/Data/Input/Actions/IA_Jump.IA_Jump"))
  (:Started
    (CallFunction|JumpInputStarted))
  (:Completed
    (CallFunction|JumpInputComplete)))

(event Input|EnhancedActionEvents|EnhancedInputActionIA_Move
  (params (ActionValue :type Vector%202D%20Structure) (ElapsedSeconds :type Float%20%28double-precision%29) (TriggeredSeconds :type Float%20%28double-precision%29) (InputAction :type Input%20Action%20Object%20Reference :default "/Game/Data/Input/Actions/IA_Move.IA_Move"))
  ;[1 1 1] trying to cache latest movement input (reading it directly from input action just gave me 0) for rotation snapping in jumps (currently unused)
  (bind _output_get (Variables|Default|SetmoveInputCache (Math|Vector2D|MakeVector2D (.x ActionValue) (.y ActionValue))))
  (if (< (.x _output_get) 0.0)
    (Variables|Default|SetmoveInputCache (* (Variables|Default|GetmoveInputCache) "(X=-1.000000,Y=-1.000000)"))))

(event Input|EnhancedActionEvents|EnhancedInputActionIA_MoveKeyReleased
  (params (ActionValue :type Vector%202D%20Structure) (ElapsedSeconds :type Float%20%28double-precision%29) (TriggeredSeconds :type Float%20%28double-precision%29) (InputAction :type Input%20Action%20Object%20Reference :default "/Game/Data/Input/Actions/IA_MoveKeyReleased.IA_MoveKeyReleased"))
  ;[1 1 1] trying to cache latest movement input (reading it directly from input action just gave me 0) for rotation snapping in jumps (currently unused)
  (Variables|Default|SetmoveInputCache ""))

(event EventTick
  (params (DeltaSeconds :type Float%20%28single-precision%29))
  (if (< (Variables|Default|GettimeSinceLastBouncePad) (Variables|Default|GetbouncePadCooldownTime))
    (Variables|Default|SettimeSinceLastBouncePad (+ (Variables|Default|GettimeSinceLastBouncePad) DeltaSeconds)))
  (if (< (Variables|Default|GetCT_TimeSinceMidairNoJump) (Variables|Default|GetCT_MaxCoyoteTime))
    (Variables|Default|SetCT_TimeSinceMidairNoJump (+ (Variables|Default|GetCT_TimeSinceMidairNoJump) DeltaSeconds))))

(event EventBeginPlay
  ;[1 1 1] Initialise jump gravity
  (CallFunction|ResetGravityScale true)
  ;[1 1 1] Setup state change event binding
  (bind _asbp_third_person_character (Utilities|Casting|CastToBP_ThirdPersonCharacter (Components|GetOwner)))
  (Variables|Default|SetPlayerRef _asbp_third_person_character)
  (EventDispatchers|BindEventtoOnStateChanged (Variables|/Game/Blueprints/Player/BP_ThirdPersonCharacter.BP_ThirdPersonCharacter_C|GetBPC_StateSystem _asbp_third_person_character) (delegate Custom|OnPlayerStateChanged)))

(fn SnapRotationBeforeJumpUNUSED
  (params (Player :type BP%20Third%20Person%20Character%20Object%20Reference))
  (bind _returnvalue (Transformation|GetActorForwardVector Player))
  (Character|LaunchCharacter Player (Math|Vector|MakeVector (* (.x _returnvalue) 1e+02) (* (.y _returnvalue) 1e+02) 0.0) true false))

(fn HandleJump
  (params (fromJumpBuffer :type Boolean))
  (bind _returnvalue (Components|GetOwner))
  (bind _returnvalue_2 (Actor|GetComponentbyClass _returnvalue "/Game/Blueprints/Player/Components/BPC_StateSystem.BPC_StateSystem_C"))
  (bind _jumpfromcoyote (CallFunction|IsJumpingfromCoyoteTime))
  (bind _asbp_third_person_character (Utilities|Casting|CastToBP_ThirdPersonCharacter (Components|GetOwner)))
  (Character|LaunchCharacter _asbp_third_person_character (Math|Vector|MakeVector (.x (* (Transformation|GetActorForwardVector _asbp_third_person_character) "10.000000,10.000000,0.000000")) (.y (* (Transformation|GetActorForwardVector _asbp_third_person_character) "10.000000,10.000000,0.000000")) (Variables|Default|GetjumpVelocity)) false true)
  (bind _isgrounded (Default|IsCurrentStateGrounded (Actor|GetComponentbyClass (Components|GetOwner) "/Game/Blueprints/Player/Components/BPC_StateSystem.BPC_StateSystem_C")))
  (if (== (Variables|Default|GetcurrentJumpCount) 1)
    (bind _returnvalue_3 (Class|FMODBlueprintStatics|PlayEvent2D "/Game/FMOD/Events/DoubleJump.DoubleJump"))
    (if (== (Class|GameplayStatics|GetGlobalTimeDilation) 1.0)
      _
      (else
        (Class|FMODBlueprintStatics|EventInstanceSetPitch _returnvalue_3 0.5))))
  ;[1 1 1] Ensure player only gets midair jumps if they start grounded
  (if (Math|Boolean|ORBoolean _isgrounded fromJumpBuffer _jumpfromcoyote)
    (Variables|Default|SetcurrentJumpCount (+ (Variables|Default|GetcurrentJumpCount) 1))
    (Default|OnPlayerJump _returnvalue_2)
    (else
      (Variables|Default|SetcurrentJumpCount (Variables|Default|GetmaxJumpCount))
      (Default|OnPlayerJump _returnvalue_2)
      (Default|OnPlayerFlip (Variables|/Game/Blueprints/Player/BP_ThirdPersonCharacter.BP_ThirdPersonCharacter_C|GetBPC_StateSystem _asbp_third_person_character))
      (bind _asbp_third_person_character_2 (Utilities|Casting|CastToBP_ThirdPersonCharacter (Game|GetPlayerCharacter 0)))
      (Components|Activation|SetActive (Variables|/Game/Blueprints/Player/BP_ThirdPersonCharacter.BP_ThirdPersonCharacter_C|GetdobuleJumpFX _asbp_third_person_character_2) true false))))

(fn CanPlayerJump
  (bind _bouncepadcooldowntime (Variables|Default|GetbouncePadCooldownTime))
  (bind _timesincelastbouncepad (Variables|Default|GettimeSinceLastBouncePad))
  (bind _returnvalue (>= _timesincelastbouncepad _bouncepadcooldowntime))
  (return (Math|Boolean|ANDBoolean (< (Variables|Default|GetcurrentJumpCount) (Variables|Default|GetmaxJumpCount)) (not (Variables|/Game/Blueprints/Player/Components/BPC_Hover.BPC_Hover_C|GetisHovering (Actor|GetComponentbyClass (Components|GetOwner) "/Game/Blueprints/Player/Components/BPC_Hover.BPC_Hover_C"))) _returnvalue) (not _returnvalue)))

(fn HandleJumpBuffer
  (bind _returnvalue (Components|GetOwner))
  (bind _returnvalue_2 (Transformation|GetActorLocation _returnvalue))
  (if (not (Variables|/Game/Blueprints/Player/Components/BPC_SuperJump.BPC_SuperJump_C|GetmidSuperJump (Variables|/Game/Blueprints/Player/BP_ThirdPersonCharacter.BP_ThirdPersonCharacter_C|GetBPC_SuperJump (Variables|Default|GetPlayerRef))))
    (bind _jumpallowed (CallFunction|CanPlayerJump))
    (if _jumpallowed
      (return)
      (else
        (bind _asbp_third_person_character (Utilities|Casting|CastToBP_ThirdPersonCharacter _returnvalue))
        (if (Math|Boolean|ORBoolean (Utilities|Enum|Equal(Enum) (Variables|/Game/Blueprints/Player/Components/BPC_StateSystem.BPC_StateSystem_C|GetCurrentState (Variables|/Game/Blueprints/Player/BP_ThirdPersonCharacter.BP_ThirdPersonCharacter_C|GetBPC_StateSystem _asbp_third_person_character)) "NewEnumerator6") (Utilities|Enum|Equal(Enum) (Variables|/Game/Blueprints/Player/Components/BPC_StateSystem.BPC_StateSystem_C|GetCurrentState (Variables|/Game/Blueprints/Player/BP_ThirdPersonCharacter.BP_ThirdPersonCharacter_C|GetBPC_StateSystem _asbp_third_person_character)) "NewEnumerator2") (Utilities|Enum|Equal(Enum) (Variables|/Game/Blueprints/Player/Components/BPC_StateSystem.BPC_StateSystem_C|GetCurrentState (Variables|/Game/Blueprints/Player/BP_ThirdPersonCharacter.BP_ThirdPersonCharacter_C|GetBPC_StateSystem _asbp_third_person_character)) "NewEnumerator4") (Utilities|Enum|Equal(Enum) (Variables|/Game/Blueprints/Player/Components/BPC_StateSystem.BPC_StateSystem_C|GetCurrentState (Variables|/Game/Blueprints/Player/BP_ThirdPersonCharacter.BP_ThirdPersonCharacter_C|GetBPC_StateSystem _asbp_third_person_character)) "NewEnumerator5") (Utilities|Enum|Equal(Enum) (Variables|/Game/Blueprints/Player/Components/BPC_StateSystem.BPC_StateSystem_C|GetCurrentState (Variables|/Game/Blueprints/Player/BP_ThirdPersonCharacter.BP_ThirdPersonCharacter_C|GetBPC_StateSystem _asbp_third_person_character)) "NewEnumerator6"))
          (bind _outhit (Collision|LineTraceByChannel _returnvalue_2 (- _returnvalue_2 "0.000000,0.000000,1000.000000") "TraceTypeQuery1" false 0 "None"))
          (Variables|Default|SethasBufferedJump (<= (.distance _outhit) (Variables|Default|GetjumpBufferDistance)))
          (return)
          (else
            (return)))))
    (else
      ;[1 1 1] If In super jump, dont allow jump buffer
      (return))))

(fn ResetGravityScale
  (params (Rise :type Boolean))
  (bind _jumpheight (Variables|Default|GetJumpHeight))
  (bind _jumptime (Variables|Default|GetJumpTime))
  ;[1 1 1 1 45] Uses max height, and the time to get there, to calculate jump velocity and gravity
  (if Rise
    (LocalVariables|SetHeightTime _jumptime)
    (else
      (LocalVariables|SetHeightTime (* _jumptime (LocalVariables|GetFallingTimeReduction)))))
  (bind _asbp_third_person_character (Utilities|Casting|CastToBP_ThirdPersonCharacter (Components|GetOwner)))
  (bind _output_get (Variables|/Script/Engine.CharacterMovementComponent|SetGravityScale (Variables|/Script/Engine.Character|GetCharacterMovement _asbp_third_person_character) (/ (* (/ (* (Math|Float|MakeLiteralFloat 2.0) _jumpheight) (Math|Float|Square (LocalVariables|GetHeightTime))) 1e+02) (Variables|Default|GetGravityStrength))))
  (bind _output_get_2 (Variables|Default|SetjumpVelocity (* (/ (* (Math|Float|MakeLiteralFloat 2.0) _jumpheight) (LocalVariables|GetHeightTime)) 1e+02))))

(fn IsJumpingfromCoyoteTime
  (if (Math|Boolean|ANDBoolean (Utilities|Enum|Equal(Enum) (Variables|/Game/Blueprints/Player/Components/BPC_StateSystem.BPC_StateSystem_C|GetCurrentState (Variables|/Game/Blueprints/Player/BP_ThirdPersonCharacter.BP_ThirdPersonCharacter_C|GetBPC_StateSystem (Variables|Default|GetPlayerRef))) "NewEnumerator4") (< (Variables|Default|GetCT_TimeSinceMidairNoJump) (Variables|Default|GetCT_MaxCoyoteTime)) (<= (.z (Transformation|GetVelocity (Variables|Default|GetPlayerRef))) 0.0))
    (return true)
    (else
      (return false))))

(fn JumpInputComplete
  (if (not (Variables|/Game/Blueprints/Player/BP_ThirdPersonCharacter.BP_ThirdPersonCharacter_C|GetIsRespawning (Variables|Default|GetPlayerRef)))
    (Variables|Default|SetjumpButtonPressed false)
    ;[1 1 1] When jump released, cancel any upward velocity if still moving up from a prev jump (jump cancel)
    (if (Utilities|Enum|Equal(Enum) (Variables|/Game/Blueprints/Player/Components/BPC_StateSystem.BPC_StateSystem_C|GetCurrentState (Actor|GetComponentbyClass (Components|GetOwner) "/Game/Blueprints/Player/Components/BPC_StateSystem.BPC_StateSystem_C")) "NewEnumerator2")
      (bind _asbp_third_person_character (Utilities|Casting|CastToBP_ThirdPersonCharacter (Components|GetOwner)))
      (if (> (.z (Variables|/Script/Engine.MovementComponent|GetVelocity (Variables|/Script/Engine.Character|GetCharacterMovement _asbp_third_person_character))) 0.0)
        (CallFunction|ResetGravityScale false)))))

(fn JumpInputStarted
  (if (not (Variables|/Game/Blueprints/Player/BP_ThirdPersonCharacter.BP_ThirdPersonCharacter_C|GetIsRespawning (Variables|Default|GetPlayerRef)))
    (Variables|Default|SetjumpButtonPressed true)
    (bind _asbp_third_person_character (Utilities|Casting|CastToBP_ThirdPersonCharacter (Components|GetOwner)))
    (if (Variables|/Game/Blueprints/Player/Components/BPC_Burrow.BPC_Burrow_C|GetIsClimbing (Variables|/Game/Blueprints/Player/BP_ThirdPersonCharacter.BP_ThirdPersonCharacter_C|GetBPC_Burrow _asbp_third_person_character))
      (Default|StopClimbing (Variables|/Game/Blueprints/Player/BP_ThirdPersonCharacter.BP_ThirdPersonCharacter_C|GetBPC_Burrow _asbp_third_person_character)))
    (CallFunction|HandleJumpBuffer)
    (if (Utilities|Enum|Equal(Enum) (Variables|/Game/Blueprints/Player/Components/BPC_StateSystem.BPC_StateSystem_C|GetCurrentState (Actor|GetComponentbyClass (Components|GetOwner) "/Game/Blueprints/Player/Components/BPC_StateSystem.BPC_StateSystem_C")) "NewEnumerator1")
      (Default|JumpfromWall (Actor|GetComponentbyClass (Components|GetOwner) "/Game/Blueprints/Player/Components/BPC_Climbing.BPC_Climbing_C"))
      (else
        ;[1 1 1] When jump pressed, if jump permitted, allow jump and increment jump count
        (bind (_jumpallowed _toosoonsincebouncepad) (CallFunction|CanPlayerJump))
        (if _jumpallowed
          (CallFunction|HandleJump false)
          (elif _toosoonsincebouncepad
            (if (Utilities|IsValid (Variables|Default|GetRecentBouncePad))
              (Default|FakeBigBounce (Variables|Default|GetRecentBouncePad))
              (Variables|Default|SetRecentBouncePad 0)
              (Variables|Default|SetcurrentJumpCount 1))))))))

(fn HandleSuperJump
  (bind _asbp_third_person_character (Utilities|Casting|CastToBP_ThirdPersonCharacter (Components|GetOwner)))
  (Character|LaunchCharacter _asbp_third_person_character (Math|Vector|MakeVector (.x (Variables|/Script/Engine.MovementComponent|GetVelocity (Variables|/Script/Engine.Character|GetCharacterMovement _asbp_third_person_character))) (.y (Variables|/Script/Engine.MovementComponent|GetVelocity (Variables|/Script/Engine.Character|GetCharacterMovement _asbp_third_person_character))) (Variables|Default|GetjumpVelocity)) false true)
  (Default|OnPlayerJump (Actor|GetComponentbyClass (Components|GetOwner) "/Game/Blueprints/Player/Components/BPC_StateSystem.BPC_StateSystem_C")))