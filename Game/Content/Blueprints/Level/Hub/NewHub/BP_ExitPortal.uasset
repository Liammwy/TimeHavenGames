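; Exit portal that completes the current area and returns the player to the Hub when the player character overlaps it.
; On overlap it marks the matching GameInstance LevelData entry complete, updates its rune high score, saves and transitions through the GameMode.
; Tick unconditionally sets the portal unlocked and reapplies the unlocked Niagara effect every frame.
; SetupKeyLevelData, uncalled here, disables fire breath and records completed areas, alongside disconnected per-level flag logic.
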(event OnComponentBeginOverlap(PortalCollider)
  (params (OverlappedComponent :type Primitive%20Component%20Object%20Reference) (OtherActor :type Actor%20Object%20Reference) (OtherComp :type Primitive%20Component%20Object%20Reference) (OtherBodyIndex :type Integer) (bFromSweep :type Boolean) (SweepResult :type Hit%20Result%20Structure%20%28by%20ref%29))
  ;[0.08085 1 0.212 1 50] PORTAL ENTERED
  (Utilities|Casting|CastToBP_ThirdPersonCharacter OtherActor)
  (CallFunction|UnlockLevel))

(event Custom|unlockLevel
  (bind _asbp_global_game_instance (Utilities|Casting|CastToBP_Global_GameInstance (Game|GetGameInstance)))
  (for (_array_element _array_index) (Variables|/Game/Blueprints/BP_Global_GameInstance.BP_Global_GameInstance_C|GetlevelData _asbp_global_game_instance)
    (if (Utilities|Enum|Equal(Enum) (.level (Utilities|Struct|Breaks_levels _array_element)) (Variables|Default|GetTheAreaName))
      (if (< (.runeHighScore (Utilities|Struct|Breaks_levels _array_element)) (.runecount (Utilities|Struct|Breaks_levels _array_element)))
        (Variables|Default|Sethighscorerune (.runecount (Utilities|Struct|Breaks_levels _array_element)))
        (else
          (Variables|Default|Sethighscorerune (.runeHighScore (Utilities|Struct|Breaks_levels _array_element)))))
      (Utilities|Array|SetArrayElem (Variables|/Game/Blueprints/BP_Global_GameInstance.BP_Global_GameInstance_C|GetlevelData _asbp_global_game_instance) _array_index (Utilities|Struct|Makes_levels (.level (Utilities|Struct|Breaks_levels _array_element)) (.runecount (Utilities|Struct|Breaks_levels _array_element)) (.hatCount (Utilities|Struct|Breaks_levels _array_element)) true (.isCurrentLevel (Utilities|Struct|Breaks_levels _array_element)) (.isAccessible (Utilities|Struct|Breaks_levels _array_element)) (.cutsceneHasPlayed (Utilities|Struct|Breaks_levels _array_element)) (.maximumRuneCount (Utilities|Struct|Breaks_levels _array_element)) (.maximumHatCount (Utilities|Struct|Breaks_levels _array_element)) (Variables|Default|Gethighscorerune)))))
  (bind _asbp_global_game_instance_2 (Utilities|Casting|CastToBP_Global_GameInstance (Game|GetGameInstance)))
  (Default|SaveGame _asbp_global_game_instance_2 (Variables|/Game/Blueprints/BP_Global_GameInstance.BP_Global_GameInstance_C|GetsaveName _asbp_global_game_instance_2))
  (bind _asbp_third_person_game_mode (Utilities|Casting|CastToBP_ThirdPersonGameMode (Game|GetGameMode)))
  (Default|TransitiontoLevel _asbp_third_person_game_mode "Hub" false))

(event EventBeginPlay
  ;[0.1864 0.7469 1 1 66] SETUP KEY RELATED VARIABELSE
  (if (== (Variables|Default|GetLevel%20Name) "Hub")
    (CallFunction|SetVisiibility)))

(event EventTick
  (params (DeltaSeconds :type Float%20%28single-precision%29))
  ;[1 0 0.2118 1 74] PORTAL UNLOCKED
  (Variables|Default|SetPortalUnlocked true)
  (Class|NiagaraComponent|SetAsset (Variables|Default|GetNS_PortalEffect) "/Game/Blueprints/Level/Hub/NS_PortalUnlocked.NS_PortalUnlocked" true))

(fn ConstructionScript
  (|CallParentFunction)
  (Class|NiagaraComponent|SetAsset (Variables|Default|GetNS_PortalEffect) 0 true))

(fn SetupKeyLevelData
  (params (HitActor :type Actor%20Object%20Reference))
  (bind _theareaname (Variables|Default|GetTheAreaName))
  (bind _returnvalue (Utilities|String|EnumtoString _theareaname))
  ;[1 1 1 1 66] KEY LOGIC DUPLICATED
  (bind _asbp_third_person_character (Utilities|Casting|CastToBP_ThirdPersonCharacter HitActor))
  (Default|ToggleFireBreath (Variables|/Game/Blueprints/Player/BP_ThirdPersonCharacter.BP_ThirdPersonCharacter_C|GetBPC_FireBreath _asbp_third_person_character) false)
  (bind _asbp_global_game_instance (Utilities|Casting|CastToBP_Global_GameInstance (Game|GetGameInstance)))
  (if (< (Utilities|Array|FindItem (Variables|/Game/Blueprints/BP_Global_GameInstance.BP_Global_GameInstance_C|GetlevelsComplete _asbp_global_game_instance) (Utilities|String|StringToName _returnvalue)) 0)
    (Utilities|Array|Add (Variables|/Game/Blueprints/BP_Global_GameInstance.BP_Global_GameInstance_C|GetlevelsComplete _asbp_global_game_instance) (Utilities|String|StringToName _returnvalue))
    (Development|PrintString _returnvalue)))