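; A level object that the player's fire breath can break, and that restores itself when the player respawns.
; On BeginPlay it caches the third-person character's three fire breath collision components and binds to its respawn-delay-started event.
; When one of those components overlaps the break trigger, ToggleDestroyed disables both collisions and hides the mesh instead of destroying the actor, so the respawn event can re-enable it.
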(event OnComponentBeginOverlap(BreakCollisionTrigger)
  (params (OverlappedComponent :type Primitive%20Component%20Object%20Reference) (OtherActor :type Actor%20Object%20Reference) (OtherComp :type Primitive%20Component%20Object%20Reference) (OtherBodyIndex :type Integer) (bFromSweep :type Boolean) (SweepResult :type Hit%20Result%20Structure%20%28by%20ref%29))
  (if (Math|Boolean|ORBoolean (== OtherComp (Variables|Default|GetFireBreathRef0)) (== OtherComp (Variables|Default|GetFireBreathRef1)) (== OtherComp (Variables|Default|GetFireBreathRef2)))
    (CallFunction|ToggleDestroyed true)))

(event Custom|OnRespawnDelayStarted
  (if (Variables|Default|GetisDestroyed)
    (CallFunction|ToggleDestroyed false)))

(event EventBeginPlay
  (bind _returnvalue (Actor|GetActorOfClass "/Game/Blueprints/Player/BP_ThirdPersonCharacter.BP_ThirdPersonCharacter_C"))
  ;[1 1 1] Ensure found object != null
  (if (not (== _returnvalue 0))
    ;[1 1 1] Grab ref to fire collision from player
    (Variables|Default|SetFireBreathRef0 (Variables|/Game/Blueprints/Player/BP_ThirdPersonCharacter.BP_ThirdPersonCharacter_C|GetFireBreathCollision _returnvalue))
    (Variables|Default|SetFireBreathRef1 (Variables|/Game/Blueprints/Player/BP_ThirdPersonCharacter.BP_ThirdPersonCharacter_C|GetFireBreathCollision1 _returnvalue))
    (Variables|Default|SetFireBreathRef2 (Variables|/Game/Blueprints/Player/BP_ThirdPersonCharacter.BP_ThirdPersonCharacter_C|GetFireBreathCollision2 _returnvalue))
    (EventDispatchers|BindEventtoOnRespawnDelayStarted _returnvalue (delegate Custom|OnRespawnDelayStarted))))

(event Collision|EventActorBeginOverlap
  (params (OtherActor :type Actor%20Object%20Reference)))

(event EventTick
  (params (DeltaSeconds :type Float%20%28single-precision%29)))

(fn ConstructionScript)

(fn ToggleDestroyed
  (params (IsDestroyed :type Boolean))
  (bind _solidcollision (Variables|Default|GetSolidCollision))
  (bind _visualsmesh (Variables|Default|GetVisualsMesh))
  (bind _breakcollisiontrigger (Variables|Default|GetBreakCollisionTrigger))
  (bind _output_get (Variables|Default|SetisDestroyed IsDestroyed))
  (if _output_get
    ;[1 1 1] Turn everything off when destroyed
    (Collision|SetCollisionEnabled _solidcollision "NoCollision")
    (Rendering|SetVisibility _visualsmesh false false)
    (Collision|SetCollisionEnabled _breakcollisiontrigger "NoCollision")
    (else
      ;[1 1 1] Turn everything on when re-enabled
      (Collision|SetCollisionEnabled _solidcollision "QueryAndPhysics")
      (Rendering|SetVisibility _visualsmesh true false)
      (Collision|SetCollisionEnabled _breakcollisiontrigger "QueryOnly"))))