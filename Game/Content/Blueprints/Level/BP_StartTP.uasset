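; BP_StartTP is a teleport pad that returns the third-person character to the player start.
; Tick looks up the player start location and yaws the actor to point at it.
; BeginPlay caches the character and its capsule, which the pad's capsule overlap matches against.
; A match triggers a delayed SetActorLocation to the start, with no check that the player is still on the pad.
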(event OnComponentBeginOverlap(Capsule)
  (params (OverlappedComponent :type Primitive%20Component%20Object%20Reference) (OtherActor :type Actor%20Object%20Reference) (OtherComp :type Primitive%20Component%20Object%20Reference) (OtherBodyIndex :type Integer) (bFromSweep :type Boolean) (SweepResult :type Hit%20Result%20Structure%20%28by%20ref%29))
  (if (== OtherComp (Variables|Default|GetPlayerCollisionref))
    (Variables|Default|SetPlayer%20On%20Teleport true)
    (Utilities|FlowControl|Delay 1e+01)
    (Transformation|SetActorLocation (Variables|Default|GetPlayer%20Ref) (Variables|Default|GetStartPos) false false)
    (else
      (Variables|Default|SetPlayer%20On%20Teleport false))))

(event EventBeginPlay
  (bind _returnvalue (Actor|GetActorOfClass "/Game/Blueprints/Player/BP_ThirdPersonCharacter.BP_ThirdPersonCharacter_C"))
  (Variables|Default|SetPlayer%20Ref _returnvalue)
  (Variables|Default|SetPlayerCollisionref (Variables|/Script/Engine.Character|GetCapsuleComponent _returnvalue)))

(event EventTick
  (params (DeltaSeconds :type Float%20%28single-precision%29))
  (bind _returnvalue (Transformation|GetActorRotation))
  ;[1 1 1] Grabs player start location, and aims arrow to it
  (bind _output_get (Variables|Default|SetStartPos (Transformation|GetActorLocation (Class|GameModeBase|FindPlayerStart (Game|GetGameMode)))))
  (Transformation|SetActorRotation (Math|Rotator|MakeRotator (.roll _returnvalue) (.pitch _returnvalue) (.yaw (Math|Rotator|MakeRotfromXZ (- _output_get (Transformation|GetActorLocation)) (Variables|Default|GetZ))))))

(fn ConstructionScript)