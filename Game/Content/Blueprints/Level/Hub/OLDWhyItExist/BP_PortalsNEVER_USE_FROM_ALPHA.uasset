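; A legacy hub-world portal actor that sends the player to the level named in its LevelName variable.
; When the third-person character overlaps its collider, it saves the player's mesh, anim class and snowman flag to the global GameInstance and clears InHubWorld.
; It then asks the game mode to transition to that level.
; The construction script's logic for auto-numbering DoorIndx from the portal count is disconnected and never runs.
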(event OnComponentBeginOverlap(PortalCollider)
  (params (OverlappedComponent :type Primitive%20Component%20Object%20Reference) (OtherActor :type Actor%20Object%20Reference) (OtherComp :type Primitive%20Component%20Object%20Reference) (OtherBodyIndex :type Integer) (bFromSweep :type Boolean) (SweepResult :type Hit%20Result%20Structure%20%28by%20ref%29))
  ;[1 1 1 1 25] On component hit, open level
  (bind _asbp_third_person_character (Utilities|Casting|CastToBP_ThirdPersonCharacter OtherActor))
  (bind _asbp_global_game_instance (Utilities|Casting|CastToBP_Global_GameInstance (Game|GetGameInstance)))
  (Default|SavePlayerModel _asbp_global_game_instance (Variables|/Script/Engine.SkeletalMeshComponent|GetSkeletalMeshAsset (Variables|/Script/Engine.Character|GetMesh _asbp_third_person_character)) (Variables|/Script/Engine.SkeletalMeshComponent|GetAnimClass (Variables|/Script/Engine.Character|GetMesh _asbp_third_person_character)) (Variables|/Game/Blueprints/Player/BP_ThirdPersonCharacter.BP_ThirdPersonCharacter_C|GetSnowMan _asbp_third_person_character))
  (Variables|/Game/Blueprints/BP_Global_GameInstance.BP_Global_GameInstance_C|SetinHubWorld _asbp_global_game_instance false)
  (bind _asbp_third_person_game_mode (Utilities|Casting|CastToBP_ThirdPersonGameMode (Game|GetGameMode)))
  (Default|TransitiontoLevel _asbp_third_person_game_mode (Variables|Default|GetLevel%20Name)))

(fn ConstructionScript
  ;[1 1 1] Logic to auto sort the door index numbers
)