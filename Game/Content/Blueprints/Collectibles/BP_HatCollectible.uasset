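; BP_HatCollectible is a hat pickup, selected by index, that starts locked in a box unless set open for pickup.
; Each tick it scales a progress box by the player's currency over total runes, triggering a snowball burst and revealing the hat when full.
; The visible pivot spins and bobs using a ping-ponged eased timer.
; Overlapping the open hat marks it collected in the player's hat collection component and destroys the actor.
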(event OnComponentBeginOverlap(HatCollision)
  (params (OverlappedComponent :type Primitive%20Component%20Object%20Reference) (OtherActor :type Actor%20Object%20Reference) (OtherComp :type Primitive%20Component%20Object%20Reference) (OtherBodyIndex :type Integer) (bFromSweep :type Boolean) (SweepResult :type Hit%20Result%20Structure%20%28by%20ref%29))
  ;[0 1 0.8981 1 34] PICKUP HAT
  (if (Variables|Default|GetOpenForPickup)
    (bind _asbp_third_person_character (Utilities|Casting|CastToBP_ThirdPersonCharacter OtherActor))
    ;;[1 0.01661 0] FUNCTION TO HANDLE HAT COLLECTION
    (CallFunction|GivePlayerHat _asbp_third_person_character)
    (Development|PrintString "Player Picked Up Hat")
    ;;[1 0 0.06749] Comment
    (CallFunction|HatDisappearAnimation)
    (Actor|DestroyActor)))

(event EventBeginPlay
  ;[1 0.6896 0 1 34] GET TOTAL RUNES
  (bind _asbp_third_person_character (Utilities|Casting|CastToBP_ThirdPersonCharacter (Game|GetPlayerCharacter 0)))
  (bind _output_get (Variables|Default|SetTPC_Player _asbp_third_person_character))
  (bind _runetotal (Default|NumOfRunes _output_get))
  (Variables|Default|SetTotalRunes _runetotal))

(event EventTick
  (params (DeltaSeconds :type Float%20%28single-precision%29))
  ;[0 1 0.1796 1 34] HANDLE HAT MOVEMENT
  (CallFunction|UpdateRuneCount)
  (bind _output_get (Variables|Default|SetElapsedTime (+ (Variables|Default|GetElapsedTime) (* DeltaSeconds (Variables|Default|GetMoveDirection)))))
  (if (Variables|Default|GetOpenForPickup)
    (CallFunction|MoveObject (Variables|Default|GetHatPivot) _output_get DeltaSeconds)
    (else
      (CallFunction|MoveObject (Variables|Default|GetBoxPivot) _output_get DeltaSeconds)))
  (if (or (< (Variables|Default|GetElapsedTime) 0.0) (> (Variables|Default|GetElapsedTime) (Variables|Default|GetBobSpeed)))
    (Variables|Default|SetMoveDirection (* (Variables|Default|GetMoveDirection) -1))))

(fn ConstructionScript
  ;[1 1 1] SETUP HAT USING INDEX
  (bind _returnvalue (Components|StaticMesh|SetStaticMesh (Variables|Default|GetHatMesh) (Utilities|Array|Get(acopy) (Variables|Default|GetHats) (Variables|Default|GetIndex))))
  (if _returnvalue
    ;[1 1 1] TOGGLES MODE
    (if (not (Variables|Default|GetOpenForPickup))
      (Development|SetHiddeninGame (Variables|Default|GetHatPivot) true true)
      (else
        (Development|SetHiddeninGame (Variables|Default|GetBoxPivot) true true)))
    (else
      (Development|PrintString "Invalid Index For Hat"))))

(fn GivePlayerHat
  (params (Player :type BP%20Third%20Person%20Character%20Object%20Reference))
  (bind _bpc_hatcollection (Variables|/Game/Blueprints/Player/BP_ThirdPersonCharacter.BP_ThirdPersonCharacter_C|GetBPC_HatCollection Player))
  (if (Math|Integer|InRange(Integer) (Variables|Default|GetIndex) 0 (- (Utilities|Array|Length (Variables|/Game/Blueprints/Player/Components/BPC_HatCollection.BPC_HatCollection_C|GetHats _bpc_hatcollection)) 1))
    (Utilities|Array|SetArrayElem (Variables|/Game/Blueprints/Player/Components/BPC_HatCollection.BPC_HatCollection_C|GetHatsCollected _bpc_hatcollection) (Variables|Default|GetIndex) true)))

(fn MoveObject
  (params (pivot :type Scene%20Component%20Object%20Reference) (elapsedTime :type Float%20%28double-precision%29) (deltaTime :type Float%20%28double-precision%29))
  (bind _relativelocation (Variables|/Script/Engine.SceneComponent|GetRelativeLocation pivot))
  (Transformation|SetRelativeLocation pivot (Math|Vector|MakeVector (.x _relativelocation) (.y _relativelocation) (Math|Interpolation|Ease "EaseInOut" elapsedTime 3e+01 5e+01 2.0)) false false)
  (Transformation|AddRelativeRotation pivot (Math|Rotator|MakeRotator 0.0 0.0 (* deltaTime (* (Variables|Default|GetRotationSpeed) 1e+01))) false false)
  (return))

(fn UpdateRuneCount
  (bind _totalrunes (Variables|Default|GetTotalRunes))
  (bind _progressboxpivot (Variables|Default|GetProgressBoxPivot))
  (bind _tpc_player (Variables|Default|GetTPC_Player))
  (bind _returnvalue (Math|Conversions|ToFloat(Integer) _totalrunes))
  (bind _bpc_currency (Variables|/Game/Blueprints/Player/BP_ThirdPersonCharacter.BP_ThirdPersonCharacter_C|GetBPC_Currency _tpc_player))
  (bind _relativescale3d (Variables|/Script/Engine.SceneComponent|GetRelativeScale3D _progressboxpivot))
  (bind _currency (Variables|/Game/Blueprints/Player/Components/BPC_Currency.BPC_Currency_C|Getcurrency _bpc_currency))
  (bind _returnvalue_2 (Math|Conversions|ToFloat(Integer) _currency))
  (bind _returnvalue_3 (/ _returnvalue_2 _returnvalue))
  ;[0.2444 1 0.1655] FILL PROGRESS BOX
  (Utilities|IsValid _tpc_player
    (:Is%20Valid
      (Transformation|SetRelativeScale3D _progressboxpivot (Math|Vector|MakeVector (.x _relativescale3d) (.y _relativescale3d) _returnvalue_3))
      ;[0.1458 0.812 1] EXPLODE BOX - HAT UNLOCKED
      (if (and (>= _returnvalue_3 1.0) (not (Variables|Default|GetOpenForPickup)))
        (Components|Activation|Activate (Variables|Default|GetNS_SnowballExplosion) false)
        ;[1 0.4063 0.03844] HAT IS VISIBLE
        (Development|SetHiddeninGame (Variables|Default|GetBoxPivot) true true)
        (Development|SetHiddeninGame (Variables|Default|GetHatPivot) false true)
        (Development|SetHiddeninGame (Variables|Default|GetHatCollision) true true)
        (Variables|Default|SetOpenForPickup true)))))

(fn HatDisappearAnimation)