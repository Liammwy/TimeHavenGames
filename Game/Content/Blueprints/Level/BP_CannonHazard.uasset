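; Cannon hazard that repeatedly fires exploding cannonballs on a fixed delay.
; Tick accumulates time, then plays the fire audio event and spawns a ball at the Arrow, passing it speed, lifetime and the actor's forward direction before launching it.
; An optional start offset holds back the firing timer until it runs out.
; The PawnSensing handler only casts and delays, so seeing the player does not affect firing.
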(event OnSeePawn(PawnSensing)
  (params (Pawn :type Pawn%20Object%20Reference))
  (Utilities|Casting|CastToBP_ThirdPersonCharacter Pawn)
  (Utilities|FlowControl|Delay (Variables|Default|GetCannon%20Fire%20Delay)))

(event EventTick
  (params (DeltaSeconds :type Float%20%28single-precision%29))
  (bind _arrow (Variables|Default|GetArrow))
  (bind _returnvalue (Transformation|GetWorldTransform _arrow))
  (CallFunction|UpdatePreventFiring DeltaSeconds)
  (if (not (Variables|Default|GetPrevent%20Firing))
    (bind _output_get (Variables|Default|SetTimeSinceLastFire (+ DeltaSeconds (Variables|Default|GetTimeSinceLastFire))))
    (if (>= _output_get (Variables|Default|GetCannon%20Fire%20Delay))
      (Variables|Default|SetTimeSinceLastFire 0.0)
      (Class|FMODBlueprintStatics|PlayEventatLocation "/Game/FMOD/Events/Cannon_Fire.Cannon_Fire" _returnvalue)
      (bind _returnvalue_2 (Game|SpawnActorfromClass "/Game/Blueprints/Level/Testing/TESTJOSEPH_ExplodingBall.TESTJOSEPH_ExplodingBall_C" _returnvalue "Undefined" "MultiplyWithRoot" 0 0))
      ;[1 1 1] ensure cannonball gets spawned correctly
      (if (Utilities|IsValid _returnvalue_2)
        (Variables|/Game/Blueprints/Level/Testing/TESTJOSEPH_ExplodingBall.TESTJOSEPH_ExplodingBall_C|SetProjectileSpeed _returnvalue_2 (Variables|Default|GetProjectile%20speed))
        (Variables|/Game/Blueprints/Level/Testing/TESTJOSEPH_ExplodingBall.TESTJOSEPH_ExplodingBall_C|SetProjectileDirection _returnvalue_2 (Transformation|GetActorForwardVector))
        (Variables|/Game/Blueprints/Level/Testing/TESTJOSEPH_ExplodingBall.TESTJOSEPH_ExplodingBall_C|SetMaxLifetime _returnvalue_2 (Variables|Default|GetProjectileLifetime))
        (Default|OnProjectileLaunch _returnvalue_2)))))

(event EventBeginPlay
  ;[1 1 1] If offset is used, prevent firing/timing updates from happening for length of offset
  (if (> (Variables|Default|GetCannon%20Fire%20Offset) 0.0)
    (Variables|Default|SetPrevent%20Firing true)
    (Variables|Default|SetTime%20To%20Prevent%20Firing (Variables|Default|GetCannon%20Fire%20Offset))))

(fn ConstructionScript)

(fn UpdatePreventFiring
  (params (deltaTime :type Float%20%28double-precision%29))
  ;[1 1 1] Deplete Time To Prevent Firing until it's less than 0, then disable Prevent Firing
  (if (Variables|Default|GetPrevent%20Firing)
    (bind _output_get (Variables|Default|SetTime%20To%20Prevent%20Firing (- (Variables|Default|GetTime%20To%20Prevent%20Firing) deltaTime)))
    (if (not (>= _output_get 0.0))
      (Variables|Default|SetPrevent%20Firing false))))