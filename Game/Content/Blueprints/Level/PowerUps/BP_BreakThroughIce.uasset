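; BP_BreakThroughIce is a level block the player breaks through while super jumping.
; Top and bottom colliders detect overlaps from the player's capsule and call BlockHitFunction, whose bottom-hit flag is unused.
; If the player's hover component is inactive and a super jump is underway, it plays a BlockBreaking event at the block.
; It then hides the cube and disables its collision and both colliders rather than destroying the actor.
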(event OnComponentBeginOverlap(BottomCollider)
  (params (OverlappedComponent :type Primitive%20Component%20Object%20Reference) (OtherActor :type Actor%20Object%20Reference) (OtherComp :type Primitive%20Component%20Object%20Reference) (OtherBodyIndex :type Integer) (bFromSweep :type Boolean) (SweepResult :type Hit%20Result%20Structure%20%28by%20ref%29))
  (if (== OtherComp (Variables|Default|GetPlayerHitboxRef))
    (CallFunction|BlockHitFunction true)))

(event OnComponentBeginOverlap(TopCollider)
  (params (OverlappedComponent :type Primitive%20Component%20Object%20Reference) (OtherActor :type Actor%20Object%20Reference) (OtherComp :type Primitive%20Component%20Object%20Reference) (OtherBodyIndex :type Integer) (bFromSweep :type Boolean) (SweepResult :type Hit%20Result%20Structure%20%28by%20ref%29))
  (if (== OtherComp (Variables|Default|GetPlayerHitboxRef))
    (CallFunction|BlockHitFunction false)))

(event EventBeginPlay
  (bind _returnvalue (Actor|GetActorOfClass "/Game/Blueprints/Player/BP_ThirdPersonCharacter.BP_ThirdPersonCharacter_C"))
  (Variables|Default|SetPlayerRef _returnvalue)
  (Variables|Default|SetPlayerHitboxRef (Variables|/Script/Engine.Character|GetCapsuleComponent _returnvalue)))

(event EventTick
  (params (DeltaSeconds :type Float%20%28single-precision%29)))

(fn ConstructionScript)

(fn BlockHitFunction
  (params (HitBottomColl :type Boolean))
  (bind _playerref (Variables|Default|GetPlayerRef))
  (if (not (Variables|/Game/Blueprints/Player/Components/BPC_Hover.BPC_Hover_C|GetisHovering (Variables|/Game/Blueprints/Player/BP_ThirdPersonCharacter.BP_ThirdPersonCharacter_C|GetBPC_Hover _playerref)))
    (if (Variables|/Game/Blueprints/Player/Components/BPC_SuperJump.BPC_SuperJump_C|GetmidSuperJump (Variables|/Game/Blueprints/Player/BP_ThirdPersonCharacter.BP_ThirdPersonCharacter_C|GetBPC_SuperJump _playerref))
      (Class|FMODBlueprintStatics|PlayEventatLocation "/Game/FMOD/Events/BlockBreaking.BlockBreaking" (Transformation|GetActorTransform))
      (Rendering|SetVisibility (Variables|Default|GetCube) false false)
      (Collision|SetCollisionEnabled (Variables|Default|GetCube) "NoCollision")
      (Collision|SetCollisionEnabled (Variables|Default|GetBottomCollider) "NoCollision")
      (Collision|SetCollisionEnabled (Variables|Default|GetTopCollider) "NoCollision"))))