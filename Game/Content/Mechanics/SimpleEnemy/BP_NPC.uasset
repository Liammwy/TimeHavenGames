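; BP_NPC is a simple AI enemy that chases the player, knocks them back on contact and can be jumped on.
; Overlapping SeenPlayerRange sets the Blackboard key playerInRange; hitting Collider clears it and, after a short delay, bounces the player upward.
; DeathCollider pushes the player opposite their facing direction.
; A red-glow fuse timeline ending in explosion and destruction exists but is unconnected, so it never runs.
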(event OnComponentBeginOverlap(SeenPlayerRange)
  (params (OverlappedComponent :type Primitive%20Component%20Object%20Reference) (OtherActor :type Actor%20Object%20Reference) (OtherComp :type Primitive%20Component%20Object%20Reference) (OtherBodyIndex :type Integer) (bFromSweep :type Boolean) (SweepResult :type Hit%20Result%20Structure%20%28by%20ref%29))
  (bind _self self)
  (bind _returnvalue (AI|GetAIController _self))
  (bind _returnvalue_2 (AI|GetBlackboard _returnvalue))
  ;[1 0.03977 0 1 58] Has Seen player, and starts chasing. They glow red over time to show fuse
  (Utilities|Casting|CastToBP_ThirdPersonCharacter OtherActor)
  (if (not (ScalableFloat|GetValueasBool _returnvalue_2 (Utilities|Name|MakeLiteralName "playerInRange")))
    (AI|Components|Blackboard|SetValueasBool _returnvalue_2 (Utilities|Name|MakeLiteralName "playerInRange") true)))

(event OnComponentHit(Collider)
  (params (HitComponent :type Primitive%20Component%20Object%20Reference) (OtherActor :type Actor%20Object%20Reference) (OtherComp :type Primitive%20Component%20Object%20Reference) (NormalImpulse :type Vector :default "0, 0, 0") (Hit :type Hit%20Result%20Structure%20%28by%20ref%29))
  ;[0.849 0.3319 0.09106 1 41] Handle Jumps, enemy returns to path once jumped on once
  (bind _asbp_third_person_character (Utilities|Casting|CastToBP_ThirdPersonCharacter OtherActor))
  (Utilities|FlowControl|Delay 0.2)
  (Physics|AddImpulse (Variables|/Script/Engine.Character|GetCharacterMovement _asbp_third_person_character) "0.000000,0.000000,300.000000" true)
  (AI|Components|Blackboard|SetValueasBool (AI|GetBlackboard (AI|GetAIController self)) (Utilities|Name|MakeLiteralName "playerInRange") false))

(event OnComponentBeginOverlap(DeathCollider)
  (params (OverlappedComponent :type Primitive%20Component%20Object%20Reference) (OtherActor :type Actor%20Object%20Reference) (OtherComp :type Primitive%20Component%20Object%20Reference) (OtherBodyIndex :type Integer) (bFromSweep :type Boolean) (SweepResult :type Hit%20Result%20Structure%20%28by%20ref%29))
  ;[0.08333 0.3366 1 1 42] Handle Player and AI hit collisions, add impulse to player horizontal
  (bind _asbp_third_person_character (Utilities|Casting|CastToBP_ThirdPersonCharacter OtherActor))
  (Physics|AddImpulse (Variables|/Script/Engine.Character|GetCharacterMovement _asbp_third_person_character) (* (Transformation|GetActorForwardVector _asbp_third_person_character) -1.5e+03) true))

(event EventBeginPlay
  ;[1 1 1] Set body material
)

(fn ConstructionScript)