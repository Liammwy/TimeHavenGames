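; Key collectible that completes a level when the third-person character overlaps its Box.
; Its Level variable selects whether Level1Complete or Level2Complete is set on BP_Global_GameInstance, then the Hub level opens; other values do nothing.
; A disconnected "Bin" graph holds an unused, partly wired switch version that writes a LevelAccessible struct instead.
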(event OnComponentBeginOverlap(Box)
  (params (OverlappedComponent :type Primitive%20Component%20Object%20Reference) (OtherActor :type Actor%20Object%20Reference) (OtherComp :type Primitive%20Component%20Object%20Reference) (OtherBodyIndex :type Integer) (bFromSweep :type Boolean) (SweepResult :type Hit%20Result%20Structure%20%28by%20ref%29))
  (Utilities|Casting|CastToBP_ThirdPersonCharacter OtherActor)
  (if (== (Variables|Default|GetLevel) 1)
    (bind _asbp_global_game_instance (Utilities|Casting|CastToBP_Global_GameInstance (Game|GetGameInstance)))
    (Variables|/Game/Blueprints/BP_Global_GameInstance.BP_Global_GameInstance_C|SetLevel1Complete _asbp_global_game_instance true)
    (Game|OpenLevel(byObjectReference) "/Game/Levels/_FinalLevels/Hub.Hub" :!label _label)
    (elif (== (Variables|Default|GetLevel) 2)
      (bind _asbp_global_game_instance_2 (Utilities|Casting|CastToBP_Global_GameInstance (Game|GetGameInstance)))
      (Variables|/Game/Blueprints/BP_Global_GameInstance.BP_Global_GameInstance_C|SetLevel2Complete _asbp_global_game_instance_2 true)
      (goto _label))))

(fn ConstructionScript)