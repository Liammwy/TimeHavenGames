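; Hub island actor that rises into view after Levels 1 and 2 are complete in the game instance, or when the 8 key is pressed.
; It triggers the tagged falling bridge's GrowIn while a timeline animates the island's height.
; Chained timelines then reset penguins and hat to positions cached in the construction script, scale them up, and scale the trees.
; Portal spawning remains as disconnected logic, removed for beta.
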(event EventBeginPlay
  (bind _island (Variables|Default|GetIsland))
  (bind _relativelocation (Variables|/Script/Engine.SceneComponent|GetRelativeLocation _island))
  (Input|EnableInput (Game|GetPlayerController 0))
  (bind _asbp_global_game_instance (Utilities|Casting|CastToBP_Global_GameInstance (Game|GetGameInstance)))
  (if (and (Variables|/Game/Blueprints/BP_Global_GameInstance.BP_Global_GameInstance_C|GetLevel1Complete _asbp_global_game_instance) (Variables|/Game/Blueprints/BP_Global_GameInstance.BP_Global_GameInstance_C|GetLevel2Complete _asbp_global_game_instance))
    (Utilities|FlowControl|Delay 0.5)
    (bind _outactors (Actor|GetAllActorsOfClasswithTag "/Game/Blueprints/Level/Hub/NewHub/BP_FallingBridge.BP_FallingBridge_C" "Bridge1"))
    (Default|Growin (Utilities|Array|Get(acopy) _outactors))
    (bind _movement (Timeline|Timeline Play)
      (:Update
        (Transformation|SetRelativeLocation _island (Math|Vector|MakeVector (.x _relativelocation) (.y _relativelocation) (* _movement 5e+03)) false false))
      (:Finished
        (Transformation|SetRelativeLocation (Variables|Default|GetPenguin) (Variables|Default|GetPenguin%20Pos) false false)
        (Transformation|SetRelativeLocation (Variables|Default|GetHat) (Variables|Default|GetCrown%20Pos) false false)
        (Transformation|SetRelativeLocation (Variables|Default|GetDancingPenguin1) (Variables|Default|GetDancePenguin1) false false)
        (Transformation|SetRelativeLocation (Variables|Default|GetDancingPenguin2) (Variables|Default|GetDancePenguin2) false false)
        (Transformation|SetRelativeLocation (Variables|Default|GetDancingPenguin3) (Variables|Default|GetDancePenguin3) false false)
        (bind _scale (Timeline|Timeline_1 PlayFromStart)
          (:Update
            (Transformation|SetWorldScale3D (Variables|Default|GetPenguin) (Math|Conversions|ToVector(Float) _scale))
            (Transformation|SetWorldScale3D (Variables|Default|GetHat) (Math|Conversions|ToVector(Float) _scale))
            (Transformation|SetWorldScale3D (Variables|Default|GetDancingPenguin1) (/ (Math|Conversions|ToVector(Float) _scale) 8))
            (Transformation|SetWorldScale3D (Variables|Default|GetDancingPenguin2) (/ (Math|Conversions|ToVector(Float) _scale) 8))
            (Transformation|SetWorldScale3D (Variables|Default|GetDancingPenguin3) (/ (Math|Conversions|ToVector(Float) _scale) 8)))
          (:Finished
            (bind _movement_2 (Timeline|Timeline_0 PlayFromStart)
              (:Update
                (Transformation|SetRelativeScale3D (Variables|Default|GetTree1) (Math|Conversions|ToVector(Float) _movement_2))))))))))

(event Input|KeyboardEvents|8
  (params (Key :type Key%20Structure :default "None"))
  (bind _island (Variables|Default|GetIsland))
  (bind _relativelocation (Variables|/Script/Engine.SceneComponent|GetRelativeLocation _island))
  (:Pressed
    (bind _outactors (Actor|GetAllActorsOfClasswithTag "/Game/Blueprints/Level/Hub/NewHub/BP_FallingBridge.BP_FallingBridge_C" "Bridge1"))
    (Default|Growin (Utilities|Array|Get(acopy) _outactors))
    (bind _movement (Timeline|Timeline Play)
      (:Update
        (Transformation|SetRelativeLocation _island (Math|Vector|MakeVector (.x _relativelocation) (.y _relativelocation) (* _movement 5e+03)) false false))
      (:Finished
        (Transformation|SetRelativeLocation (Variables|Default|GetPenguin) (Variables|Default|GetPenguin%20Pos) false false)
        (Transformation|SetRelativeLocation (Variables|Default|GetHat) (Variables|Default|GetCrown%20Pos) false false)
        (Transformation|SetRelativeLocation (Variables|Default|GetDancingPenguin1) (Variables|Default|GetDancePenguin1) false false)
        (Transformation|SetRelativeLocation (Variables|Default|GetDancingPenguin2) (Variables|Default|GetDancePenguin2) false false)
        (Transformation|SetRelativeLocation (Variables|Default|GetDancingPenguin3) (Variables|Default|GetDancePenguin3) false false)
        (bind _scale (Timeline|Timeline_1 PlayFromStart)
          (:Update
            (Transformation|SetWorldScale3D (Variables|Default|GetPenguin) (Math|Conversions|ToVector(Float) _scale))
            (Transformation|SetWorldScale3D (Variables|Default|GetHat) (Math|Conversions|ToVector(Float) _scale))
            (Transformation|SetWorldScale3D (Variables|Default|GetDancingPenguin1) (/ (Math|Conversions|ToVector(Float) _scale) 8))
            (Transformation|SetWorldScale3D (Variables|Default|GetDancingPenguin2) (/ (Math|Conversions|ToVector(Float) _scale) 8))
            (Transformation|SetWorldScale3D (Variables|Default|GetDancingPenguin3) (/ (Math|Conversions|ToVector(Float) _scale) 8)))
          (:Finished
            (bind _movement_2 (Timeline|Timeline_0 PlayFromStart)
              (:Update
                (Transformation|SetRelativeScale3D (Variables|Default|GetTree1) (Math|Conversions|ToVector(Float) _movement_2))))))))))

(fn ConstructionScript
  (Variables|Default|SetPenguin%20Pos (Variables|/Script/Engine.SceneComponent|GetRelativeLocation (Variables|Default|GetPenguin)))
  (Variables|Default|SetCrown%20Pos (Variables|/Script/Engine.SceneComponent|GetRelativeLocation (Variables|Default|GetHat)))
  (Variables|Default|SetDancePenguin1 (Variables|/Script/Engine.SceneComponent|GetRelativeLocation (Variables|Default|GetDancingPenguin1)))
  (Variables|Default|SetDancePenguin2 (Variables|/Script/Engine.SceneComponent|GetRelativeLocation (Variables|Default|GetDancingPenguin2)))
  (Variables|Default|SetDancePenguin3 (Variables|/Script/Engine.SceneComponent|GetRelativeLocation (Variables|Default|GetDancingPenguin3))))