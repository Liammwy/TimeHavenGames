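; Player component that gives the third-person character a timed jetpack hover.
; Holding IA_Hover zeroes vertical velocity while Tick drains the hover timer; release or depletion blocks further hovering until BPC_StateSystem reports grounded.
; CanPlayerHover gates input on disabled zones, depletion and allowed movement states.
; PlayerJetpackBoost toggles both thruster effects and scales them by remaining time, alongside an FMOD jetpack sound stopped on release or landing.
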(event Custom|Reset%20Hover%20Time
  (Variables|Default|SetcurrentHoverTime (Variables|Default|GetmaxHoverTime)))

(event Input|EnhancedActionEvents|EnhancedInputActionIA_Hover
  (params (ActionValue :type Boolean) (ElapsedSeconds :type Float%20%28double-precision%29) (TriggeredSeconds :type Float%20%28double-precision%29) (InputAction :type Input%20Action%20Object%20Reference :default "/Game/Data/Input/Actions/IA_Hover.IA_Hover"))
  (bind _playerref (Variables|Default|GetplayerRef))
  (bind _returnvalue (Actor|GetComponentbyClass _playerref "/Script/Engine.CharacterMovementComponent"))
  (:Triggered
    (bind _hoverallowed (CallFunction|CanPlayerHover))
    (if _hoverallowed
      ;[1 1 1] Freeze vertical velocity for hover effect
      (Variables|/Script/Engine.MovementComponent|SetVelocity _returnvalue (Math|Vector|MakeVector (.x (Variables|/Script/Engine.MovementComponent|GetVelocity _returnvalue)) (.y (Variables|/Script/Engine.MovementComponent|GetVelocity _returnvalue)) 0.0))
      (bind _output_get (Variables|Default|SetisHovering true))
      (CallFunction|PlayerJetpackBoost _output_get)))
  (:Started
    ;[1 1 1] Reset hover time on initial input
    (bind _hoverallowed_2 (CallFunction|CanPlayerHover))
    (if _hoverallowed_2
      (Variables|Default|SetcurrentHoverTime (Variables|Default|GetmaxHoverTime))
      (Variables|Default|SetisHovering true)
      (bind _returnvalue_2 (Class|FMODBlueprintStatics|PlayEvent2D "/Game/FMOD/Events/Jetpack.Jetpack"))
      (Variables|Default|SetAudio _returnvalue_2))))

(event Input|EnhancedActionEvents|EnhancedInputActionIA_HoverReleased
  (params (ActionValue :type Boolean) (ElapsedSeconds :type Float%20%28double-precision%29) (TriggeredSeconds :type Float%20%28double-precision%29) (InputAction :type Input%20Action%20Object%20Reference :default "/Game/Data/Input/Actions/IA_HoverReleased.IA_HoverReleased"))
  ;[1 1 1] Reset hover state when button released
  (if (Variables|Default|GetisHovering)
    (Variables|Default|SethoverDepleted true)
    (bind _output_get (Variables|Default|SetisHovering false))
    (Class|FMODBlueprintStatics|EventInstanceStop (Variables|Default|GetAudio) false)
    (CallFunction|PlayerJetpackBoost _output_get)))

(event EventBeginPlay
  ;[1 1 1] Get ref to player on startup
  (bind _asbp_third_person_character (Utilities|Casting|CastToBP_ThirdPersonCharacter (Components|GetOwner)))
  (bind _output_get (Variables|Default|SetplayerRef _asbp_third_person_character))
  (Variables|Default|SetLeft%20Jetpack%20Boost (Variables|/Game/Blueprints/Player/BP_ThirdPersonCharacter.BP_ThirdPersonCharacter_C|GetleftJetpackBoost _output_get))
  (Variables|Default|SetRight%20Jetpack%20Boost (Variables|/Game/Blueprints/Player/BP_ThirdPersonCharacter.BP_ThirdPersonCharacter_C|GetrightJetpackBoost (Variables|Default|GetplayerRef))))

(event EventTick
  (params (DeltaSeconds :type Float%20%28single-precision%29))
  (if (Variables|Default|GetisHovering)
    ;[1 1 1] Deplete hover time
    (bind _output_get (Variables|Default|SetcurrentHoverTime (- (Variables|Default|GetcurrentHoverTime) DeltaSeconds)))
    (if (<= _output_get 0.0)
      (Variables|Default|SethoverDepleted true)
      (bind _output_get_2 (Variables|Default|SetisHovering false))
      (CallFunction|PlayerJetpackBoost _output_get_2))
    (else
      ;[1 1 1] Reset hover state when grounded
      (bind _isgrounded (Default|IsCurrentStateGrounded (Actor|GetComponentbyClass (Variables|Default|GetplayerRef) "/Game/Blueprints/Player/Components/BPC_StateSystem.BPC_StateSystem_C")))
      (if _isgrounded
        (Variables|Default|SethoverDepleted false)
        (bind _output_get_3 (Variables|Default|SetisHovering false))
        (Class|FMODBlueprintStatics|EventInstanceStop (Variables|Default|GetAudio) false)
        (CallFunction|PlayerJetpackBoost _output_get_3)))))

(fn CanPlayerHover
  (bind _playerref (Variables|Default|GetplayerRef))
  (bind _returnvalue (Actor|GetComponentbyClass _playerref "/Game/Blueprints/Player/Components/BPC_StateSystem.BPC_StateSystem_C"))
  (bind _currentstate (Variables|/Game/Blueprints/Player/Components/BPC_StateSystem.BPC_StateSystem_C|GetCurrentState _returnvalue))
  (if (Variables|Default|GetinHoverDisabledZone)
    _
    (elif (Variables|Default|GethoverDepleted)
      _
      (elif (Math|Boolean|ORBoolean (Utilities|Enum|Equal(Enum) _currentstate "NewEnumerator2") (Utilities|Enum|Equal(Enum) _currentstate "NewEnumerator4") (Utilities|Enum|Equal(Enum) _currentstate "NewEnumerator5") (Utilities|Enum|Equal(Enum) _currentstate "NewEnumerator6"))
        (return true)
        (else
          _))))
  (return false))

(fn PlayerJetpackBoost
  (params (isHover :type Boolean))
  (bind _left_jetpack_boost (Variables|Default|GetLeft%20Jetpack%20Boost))
  (bind _right_jetpack_boost (Variables|Default|GetRight%20Jetpack%20Boost))
  (if isHover
    (Components|Activation|SetActive (Variables|Default|GetLeft%20Jetpack%20Boost) true false)
    (Components|Activation|SetActive (Variables|Default|GetRight%20Jetpack%20Boost) true false)
    (Rendering|SetVisibility (Variables|Default|GetLeft%20Jetpack%20Boost) true false)
    (Transformation|SetWorldScale3D (Variables|Default|GetLeft%20Jetpack%20Boost) (* "0.900000,0.900000,0.900000" (Variables|Default|GetcurrentHoverTime)))
    (Rendering|SetVisibility (Variables|Default|GetRight%20Jetpack%20Boost) true false)
    (Transformation|SetWorldScale3D (Variables|Default|GetRight%20Jetpack%20Boost) (* "0.900000,0.900000,0.900000" (Variables|Default|GetcurrentHoverTime)))
    (else
      (Components|Activation|SetActive _left_jetpack_boost false true)
      (Rendering|SetVisibility _left_jetpack_boost false false)
      (Rendering|SetVisibility _right_jetpack_boost false false)
      (Components|Activation|SetActive _right_jetpack_boost false true))))