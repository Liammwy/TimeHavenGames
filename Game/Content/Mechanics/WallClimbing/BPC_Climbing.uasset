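; Actor component that lets the third-person character latch onto walls, push off them and climb over ledges.
; HitWall latches via a forward trace, snapping the capsule to the surface in Flying mode and notifying BPC_StateSystem.
; While latched, Tick re-traces; losing the wall triggers a downward ledge check, then a climb or fall.
; The climb disables input and lerps position in Tick, since components lack Timelines.
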(event Custom|AttachToWall
  (bind (_outhit _returnvalue) (Utilities|WallTrace))
  (if _returnvalue
    ;[1 1 1] Maybe not the best approach to access owning actor (The Player)
    (bind _asbp_third_person_character (Utilities|Casting|CastToBP_ThirdPersonCharacter (Components|GetOwner)))
    ;[1 1 1 1 42] Change Player Movement Mode to flying and slow them down as they are now attached to the wall, this will lock the player position to the wall.
    (Pawn|Components|CharacterMovement|SetMovementMode (Variables|/Script/Engine.Character|GetCharacterMovement _asbp_third_person_character) "MOVE_Flying" 0)
    (Components|Movement|StopMovementImmediately (Variables|/Script/Engine.Character|GetCharacterMovement _asbp_third_person_character))
    (Variables|/Script/Engine.CharacterMovementComponent|SetbOrientRotationToMovement (Variables|/Script/Engine.Character|GetCharacterMovement _asbp_third_person_character) false)
    (Components|MoveComponentTo (Variables|/Script/Engine.Character|GetCapsuleComponent _asbp_third_person_character) (+ (.Location (Collision|BreakHitResult _outhit)) (* (.Normal (Collision|BreakHitResult _outhit)) (Variables|/Script/Engine.CapsuleComponent|GetCapsuleRadius (Variables|/Script/Engine.Character|GetCapsuleComponent _asbp_third_person_character)))) (Math|Rotator|MakeRotfromX (* (.Normal (Collision|BreakHitResult _outhit)) -1)) false false 0.2 false)
    (Default|OnPlayerClimb (Actor|GetComponentbyClass (Components|GetOwner) "/Game/Mechanics/PlayerState/BPC_StateSystem.BPC_StateSystem_C"))
    (else
      ;[1 0.2601 0.6949] Player Latch Failed So Reset
      (Variables|Default|SetLatched false))))

(event Custom|JumpFromWall
  ;[1 1 1 1 42] Player Pushes Themselves off of a wall
  (if (Variables|Default|GetLatched)
    (CallFunction|ResetPlayerMovement)
    (bind _asbp_third_person_character (Utilities|Casting|CastToBP_ThirdPersonCharacter (Components|GetOwner)))
    (Physics|AddImpulse (Variables|/Script/Engine.Character|GetCharacterMovement _asbp_third_person_character) (* (* (Transformation|GetActorForwardVector _asbp_third_person_character) -1) 400) true)
    (Variables|Default|SetLatched false)))

(event EventBeginPlay
  ;[1 1 1 1 17] Player starts "Unlatched" to the wall
  (Variables|Default|SetLatched false))

(event EventTick
  (params (DeltaSeconds :type Float%20%28single-precision%29))
  ;[1 1 1] Check if player is on wall
  (if (Variables|Default|GetLatched)
    (bind (_outhit _returnvalue) (Utilities|WallTrace))
    (if (not _returnvalue)
      ;[1 1 1] Detect The Ledge When Player Is Near Edge Of Wall
      (bind _returnvalue_2 (Collision|LineTraceByChannel (.TraceEnd (Collision|BreakHitResult _outhit)) (Math|Vector|MakeVector (.X (Math|Vector|BreakVector (.TraceEnd (Collision|BreakHitResult _outhit)))) (.Y (Math|Vector|BreakVector (.TraceEnd (Collision|BreakHitResult _outhit)))) (- (.Z (Math|Vector|BreakVector (.TraceEnd (Collision|BreakHitResult _outhit)))) 1e+01)) "TraceTypeQuery1" false 0 "None"))
      (Variables|Default|SetLatched false)
      (if _returnvalue_2
        ;[1 1 1 1 25] Disables Player Input While They Transition Over The Ledge, Creating A Start And End Position For The Movement Lerp (Using Lerp Because Components Do Not Support Timelines)
        (bind _asbp_third_person_character (Utilities|Casting|CastToBP_ThirdPersonCharacter (Components|GetOwner)))
        (Input|DisableInput _asbp_third_person_character (Game|GetPlayerController 0))
        (Variables|Default|SetelapsedTime 0.0)
        (Variables|Default|SetClimbingLedge true)
        (Variables|Default|SetStartingLedgePos (Transformation|GetActorLocation _asbp_third_person_character))
        (Variables|Default|SetTargetLedgePos (+ (Math|Vector|MakeVector (.x (Transformation|GetActorLocation _asbp_third_person_character)) (.y (Transformation|GetActorLocation _asbp_third_person_character)) (+ (.z (Transformation|GetActorLocation _asbp_third_person_character)) (Variables|/Script/Engine.CapsuleComponent|GetCapsuleHalfHeight (Variables|/Script/Engine.Character|GetCapsuleComponent _asbp_third_person_character)))) (* (Transformation|GetActorForwardVector _asbp_third_person_character) 50)))
        (else
          ;[1 1 1] Player Reaches Edge Of The Wall And Falls
          (CallFunction|ResetPlayerMovement))))
    (elif (Variables|Default|GetClimbingLedge)
      ;[0.4427 1 0.9769 1 34] Handles Lerp Movement For When The Player Is Climbing Over A Ledge
      (bind _output_get (Variables|Default|SetelapsedTime (+ DeltaSeconds (Variables|Default|GetelapsedTime))))
      (bind _asbp_third_person_character_2 (Utilities|Casting|CastToBP_ThirdPersonCharacter (Components|GetOwner)))
      (Transformation|SetActorLocation _asbp_third_person_character_2 (Math|Vector|Lerp(Vector) (Variables|Default|GetStartingLedgePos) (Variables|Default|GetTargetLedgePos) _output_get) false false)
      ;;[1 0.25 0.25] If The Player Has Completed The Climb, Reset Movement Mode And Controls
      (if (>= (.z (Transformation|GetActorLocation _asbp_third_person_character_2)) (.z (Variables|Default|GetTargetLedgePos)))
        (Variables|Default|SetClimbingLedge false)
        (CallFunction|ResetPlayerMovement)
        (Input|EnableInput _asbp_third_person_character_2 (Game|GetPlayerController 0))))))

(fn HitWall
  ;[1 1 1] If Player hits wall and is not "latched" toggle connection to the wall
  (if (not (Variables|Default|GetLatched))
    (Variables|Default|SetLatched true)
    ;[1 1 1] Attach Player To The Wall
    (CallFunction|AttachtoWall)))

(fn ResetPlayerMovement
  (bind _asbp_third_person_character (Utilities|Casting|CastToBP_ThirdPersonCharacter (Components|GetOwner)))
  (Pawn|Components|CharacterMovement|SetMovementMode (Variables|/Script/Engine.Character|GetCharacterMovement _asbp_third_person_character) "MOVE_Falling" 0)
  (Variables|/Script/Engine.CharacterMovementComponent|SetbOrientRotationToMovement (Variables|/Script/Engine.Character|GetCharacterMovement _asbp_third_person_character) true))

(fn ClimbOverLedge
  (params (LedgeHeight :type Vector)))