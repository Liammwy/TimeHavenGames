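; BP_Checkpoint is a checkpoint actor that becomes the player's current respawn point when touched.
; When the player's capsule enters the trigger volume, an inactive checkpoint plays a sound, activates, deactivates the previous checkpoint and stores itself on the character.
; Activation and deactivation swap the base material and penguin flag animations, and in the hub world activation also increments the game instance's checkpoint index.
; GetSpawnPoint returns its location plus a height offset.
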(event OnComponentBeginOverlap(TriggerVolume)
  (params (OverlappedComponent :type Primitive%20Component%20Object%20Reference) (OtherActor :type Actor%20Object%20Reference) (OtherComp :type Primitive%20Component%20Object%20Reference) (OtherBodyIndex :type Integer) (bFromSweep :type Boolean) (SweepResult :type Hit%20Result%20Structure%20%28by%20ref%29))
  (bind _playerref (Variables|Default|GetplayerRef))
  (if (== OtherComp (Variables|Default|GetplayerHitboxRef))
    (if (not (Variables|Default|GetActivated))
      (Class|FMODBlueprintStatics|PlayEvent2D "/Game/FMOD/Events/Waypoint.Waypoint")
      (CallFunction|Activate)
      (bind _asbp_global_game_instance (Utilities|Casting|CastToBP_Global_GameInstance (Game|GetGameInstance)))
      (if (Variables|/Game/Blueprints/BP_Global_GameInstance.BP_Global_GameInstance_C|GetinHubWorld _asbp_global_game_instance)
        (Variables|/Game/Blueprints/BP_Global_GameInstance.BP_Global_GameInstance_C|SetcheckpointIndx _asbp_global_game_instance (+ (Variables|/Game/Blueprints/BP_Global_GameInstance.BP_Global_GameInstance_C|GetcheckpointIndx _asbp_global_game_instance) 1)))
      (Utilities|IsValid (Variables|/Game/Blueprints/Player/BP_ThirdPersonCharacter.BP_ThirdPersonCharacter_C|GetCheckpoint _playerref)
        (:Is%20Valid
          (CallFunction|Deactivate (Variables|/Game/Blueprints/Player/BP_ThirdPersonCharacter.BP_ThirdPersonCharacter_C|GetCheckpoint _playerref)))
        (:Is%20Not%20Valid
          _))
      (Variables|/Game/Blueprints/Player/BP_ThirdPersonCharacter.BP_ThirdPersonCharacter_C|SetCheckpoint _playerref self))))

(event Custom|penguinFlag
  (Components|Animation|PlayAnimation (Variables|Default|GetSkeletalMesh) "/Game/Models/Map/Live/Penguin/PenguinAnimations/ANIM_RaiseFlag.ANIM_RaiseFlag" false)
  (Utilities|FlowControl|Delay 1.0)
  (Components|Animation|PlayAnimation (Variables|Default|GetSkeletalMesh) "/Game/Models/Map/Live/Penguin/PenguinAnimations/waveFlags.waveFlags" true))

(event Custom|penguinUnflag
  (Components|Animation|PlayAnimation (Variables|Default|GetSkeletalMesh) "/Game/Models/Map/Live/Penguin/PenguinV1_Anim.PenguinV1_Anim" true))

(event Collision|EventActorBeginOverlap
  (params (OtherActor :type Actor%20Object%20Reference))
  ;[1 1 1] Toggle's Checkpoint: Deactivating Previous Checkpoint and Establishing this as the new one
)

(event EventBeginPlay
  (bind _returnvalue (Actor|GetActorOfClass "/Game/Blueprints/Player/BP_ThirdPersonCharacter.BP_ThirdPersonCharacter_C"))
  (Variables|Default|SetplayerRef _returnvalue)
  (Variables|Default|SetplayerHitboxRef (Variables|/Script/Engine.Character|GetCapsuleComponent _returnvalue)))

(fn ConstructionScript)

(fn GetSpawnPoint
  (bind _self self)
  (bind _returnvalue (Transformation|GetActorLocation _self))
  (return (Math|Vector|MakeVector (.x _returnvalue) (.y _returnvalue) (+ (.z _returnvalue) (Variables|Default|GetSpawnHeightOffset)))))

(fn Activate
  (Rendering|Material|SetMaterial (Variables|Default|GetBase) 0 "/Game/Materials/Level/MAT_OpenCP.MAT_OpenCP")
  (Variables|Default|SetActivated true)
  (Components|Activation|Activate (Variables|Default|GetcollectCheckpointEffect) true)
  (CallFunction|PenguinFlag))

(fn Deactivate
  (Rendering|Material|SetMaterial (Variables|Default|GetBase) 0 "/Game/Materials/Level/MAT_ClosedCP.MAT_ClosedCP")
  (Variables|Default|SetActivated false)
  (CallFunction|PenguinUnflag))