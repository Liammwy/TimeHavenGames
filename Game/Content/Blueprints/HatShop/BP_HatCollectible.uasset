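; Collectible hat, built from a DT_Hats row, that bobs and spins, either open for pickup or locked in a chest.
; Entering its detection zone shows rune progress, and holding all the level's runes bursts the chest open.
; Pickup unlocks the hat in the game instance, increments the level's hat count and shows a collection widget.
; Already unlocked hats destroy themselves on BeginPlay; distance-based FMOD volume code is disconnected.
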(event OnComponentBeginOverlap(HatCollision)
  (params (OverlappedComponent :type Primitive%20Component%20Object%20Reference) (OtherActor :type Actor%20Object%20Reference) (OtherComp :type Primitive%20Component%20Object%20Reference) (OtherBodyIndex :type Integer) (bFromSweep :type Boolean) (SweepResult :type Hit%20Result%20Structure%20%28by%20ref%29))
  ;[1 0.01447 0 1 34] PICKUP HAT
  (if (== OtherComp (Variables|/Script/Engine.Character|GetCapsuleComponent (Variables|Default|GetTPC_Player)))
    (if (and (Variables|Default|GetOpenForPickup) (not (Variables|Default|GetHatCollected)))
      (Variables|Default|SetHatCollected true)
      ;;[1 0.01661 0] FUNCTION TO HANDLE HAT COLLECTION
      (CallFunction|GivePlayerHat (Variables|Default|GetTPC_Player))
      (Class|FMODBlueprintStatics|EventInstanceStop (Variables|Default|GetFMOD) false)
      (Class|FMODBlueprintStatics|PlayEventatLocation "/Game/FMOD/Events/HatGetJingle.HatGetJingle" (Transformation|GetActorTransform))
      (Development|PrintString "Player Picked Up Hat")
      (bind _asbp_global_game_instance (Utilities|Casting|CastToBP_Global_GameInstance (Game|GetGameInstance)))
      (for (_array_element _array_index) (Variables|/Game/Blueprints/BP_Global_GameInstance.BP_Global_GameInstance_C|GetlevelData _asbp_global_game_instance)
        (if (Utilities|Enum|Equal(Enum) (.level (Utilities|Struct|Breaks_levels _array_element)) (Variables|Default|GetlevelNames))
          (Utilities|Array|SetArrayElem (Variables|/Game/Blueprints/BP_Global_GameInstance.BP_Global_GameInstance_C|GetlevelData _asbp_global_game_instance) _array_index (Utilities|Struct|Makes_levels (.level (Utilities|Struct|Breaks_levels _array_element)) (.runecount (Utilities|Struct|Breaks_levels _array_element)) (+ (.hatCount (Utilities|Struct|Breaks_levels _array_element)) 1) (.isComplete (Utilities|Struct|Breaks_levels _array_element)) (.isCurrentLevel (Utilities|Struct|Breaks_levels _array_element)) (.isAccessible (Utilities|Struct|Breaks_levels _array_element)) (.cutsceneHasPlayed (Utilities|Struct|Breaks_levels _array_element)) (.maximumRuneCount (Utilities|Struct|Breaks_levels _array_element)) (.maximumHatCount (Utilities|Struct|Breaks_levels _array_element)) (.runeHighScore (Utilities|Struct|Breaks_levels _array_element))))))
      ;[1 0 0.06749] Comment
      (CallFunction|HatDisappear)
      (Utilities|FlowControl|Delay 0.2)
      (CallFunction|HatPickupUI))))

(event OnComponentEndOverlap(DetectionZone)
  (params (OverlappedComponent :type Primitive%20Component%20Object%20Reference) (OtherActor :type Actor%20Object%20Reference) (OtherComp :type Primitive%20Component%20Object%20Reference) (OtherBodyIndex :type Integer))
  (Utilities|Casting|CastToBP_ThirdPersonCharacter OtherActor)
  (Rendering|SetVisibility (Variables|Default|GetWidget) false false))

(event OnComponentBeginOverlap(DetectionZone)
  (params (OverlappedComponent :type Primitive%20Component%20Object%20Reference) (OtherActor :type Actor%20Object%20Reference) (OtherComp :type Primitive%20Component%20Object%20Reference) (OtherBodyIndex :type Integer) (bFromSweep :type Boolean) (SweepResult :type Hit%20Result%20Structure%20%28by%20ref%29))
  (bind _progressboxpivot (Variables|Default|GetProgressBoxPivot))
  (bind _relativescale3d (Variables|/Script/Engine.SceneComponent|GetRelativeScale3D _progressboxpivot))
  ;[1 0.1873 0.7945 1 34] DO HAT UNLOCK ANIMATION
  (Utilities|Casting|CastToBP_ThirdPersonCharacter OtherActor)
  (bind _aswbp_runes_left (Utilities|Casting|CastToWBP_RunesLeft (UserInterface|GetWidget (Variables|Default|GetWidget))))
  (Default|UpdateRunes _aswbp_runes_left (Variables|Default|GetTotalRunes) (Variables|/Game/Blueprints/Player/Components/BPC_Currency.BPC_Currency_C|Getcurrency (Variables|/Game/Blueprints/Player/BP_ThirdPersonCharacter.BP_ThirdPersonCharacter_C|GetBPC_Currency (Variables|Default|GetTPC_Player))))
  (Rendering|SetVisibility (Variables|Default|GetWidget) (not (Variables|Default|GetOpenForPickup)) false)
  (bind _percentage_z (CallFunction|GetRunePercentage))
  (if (== _percentage_z 1.0)
    (CallFunction|AllCollectiblesAnimation _percentage_z)
    (else
      (Variables|Default|SetProgressBoxScaleSave (.z (Variables|/Script/Engine.SceneComponent|GetRelativeScale3D (Variables|Default|GetProgressBoxPivot))))
      (bind _alpha (Timeline|Timeline PlayFromStart)
        (:Update
          (Transformation|SetRelativeScale3D _progressboxpivot (Math|Vector|MakeVector (.x _relativescale3d) (.y _relativescale3d) (+ (Variables|Default|GetProgressBoxScaleSave) (* _alpha (- _percentage_z (Variables|Default|GetProgressBoxScaleSave)))))))))))

(event OnComponentBeginOverlap(hatCollisionBox)
  (params (OverlappedComponent :type Primitive%20Component%20Object%20Reference) (OtherActor :type Actor%20Object%20Reference) (OtherComp :type Primitive%20Component%20Object%20Reference) (OtherBodyIndex :type Integer) (bFromSweep :type Boolean) (SweepResult :type Hit%20Result%20Structure%20%28by%20ref%29))
  (Variables|Default|SethearJingle true))

(event OnComponentEndOverlap(hatCollisionBox)
  (params (OverlappedComponent :type Primitive%20Component%20Object%20Reference) (OtherActor :type Actor%20Object%20Reference) (OtherComp :type Primitive%20Component%20Object%20Reference) (OtherBodyIndex :type Integer))
  (Variables|Default|SethearJingle false))

(event Custom|HatPickupUI
  ;[1 0.3711 0 1 50] HAT PICKUP UI HANDLING
  (bind _returnvalue (UserInterface|CreateWidget "/Game/Blueprints/UI/WBP_CollectedItem.WBP_CollectedItem_C" (Game|GetPlayerController 0)))
  (UserInterface|Viewport|AddtoViewport _returnvalue 0)
  (Default|HatCollectible _returnvalue (Variables|Default|Gethat))
  (UserInterface|Animation|PlayAnimation _returnvalue (Variables|/Game/Blueprints/UI/WBP_CollectedItem.WBP_CollectedItem_C|GetgotCollection _returnvalue) 0.0 1 "Forward" 1.0 false)
  (Utilities|FlowControl|Delay (Class|WidgetAnimation|GetEndTime (Variables|/Game/Blueprints/UI/WBP_CollectedItem.WBP_CollectedItem_C|GetgotCollection _returnvalue)))
  (Widget|RemovefromParent _returnvalue))

(event Custom|HatDisappear
  ;[1 1 1 1 39] HAT DISAPPEAR AND UI APPEAR
  (bind _hatscale (Timeline|HatReSizeAnimatio PlayFromStart)
    (:Update
      (Transformation|SetRelativeScale3D (Variables|Default|GetHatPivot) (Math|Conversions|ToVector(Float) _hatscale)))
    (:Finished
      (Actor|DestroyActor))))

(event Custom|allCollectiblesAnimation
  (params (percentageZ :type Float%20%28double-precision%29))
  (bind _chestbase (Variables|Default|GetChestBase))
  (bind _chestlid (Variables|Default|GetChestLid))
  ;[1 1 1] trigger chest exploding on all runes collected
  (if (not (Variables|Default|GetOpenForPickup))
    (if (not (Variables|Default|GetunlockAnimTriggered))
      (Variables|Default|SetunlockAnimTriggered true)
      (Collision|SetCollisionEnabled _chestbase "NoCollision")
      (Rendering|SetVisibility _chestbase false false)
      (Collision|SetCollisionEnabled _chestlid "NoCollision")
      (Rendering|SetVisibility _chestlid false false)
      (CallFunction|UnlockHat))))

(event Custom|hatExplosion
  ;[1 1 1 1 34] HAT EXPLOSION CODE
  (Class|FMODBlueprintStatics|PlayEventatLocation "/Game/FMOD/Events/FireLight.FireLight" (Transformation|GetActorTransform))
  (bind _size (Timeline|Timeline_0 Play)
    (:Update
      (Transformation|SetRelativeScale3D (Variables|Default|GetBoxPivot) (Math|Conversions|ToVector(Float) _size)))
    (:Finished
      (CallFunction|UnlockHat)
      (Rendering|SetVisibility (Variables|Default|GetWidget) false false))))

(event Custom|HatGrow
  ;[1 0.1489 0.06918 1 57] HAT GROW FOR ICE PICKUPS
  (bind _hatscale (Timeline|Timeline_1 PlayFromStart)
    (:Update
      (Transformation|SetRelativeScale3D (Variables|Default|GetHatPivot) (Math|Conversions|ToVector(Float) _hatscale)))))

(event Custom|getPlayerLocation)

(event EventBeginPlay
  ;[1 0.6896 0 1 34] GET TOTAL RUNES
  (bind _returnvalue (Class|FMODBlueprintStatics|PlayEventatLocation "/Game/FMOD/Events/HatAmbient.HatAmbient" (Math|Conversions|ToTransform(Vector) (Transformation|GetActorLocation))))
  (bind _output_get (Variables|Default|SetFMOD _returnvalue))
  (Class|FMODBlueprintStatics|EventInstanceSetVolume _output_get 5.0)
  (bind _asbp_third_person_character (Utilities|Casting|CastToBP_ThirdPersonCharacter (Game|GetPlayerCharacter 0)))
  (bind _output_get_2 (Variables|Default|SetTPC_Player _asbp_third_person_character))
  (bind _runetotal (Default|NumOfRunes _output_get_2))
  (Variables|Default|SetTotalRunes _runetotal)
  ;[0.9087 0.1834 1 1 50] ONLY ALLOW HAT PICKUP IF IT IS A NEW HAT
  (CallFunction|SetLevelVariable)
  (bind _asbp_global_game_instance (Utilities|Casting|CastToBP_Global_GameInstance (Game|GetGameInstance)))
  (if (.unlocked (Utilities|Struct|BreakS_Hats (Utilities|Array|Get(acopy) (Variables|/Game/Blueprints/BP_Global_GameInstance.BP_Global_GameInstance_C|GethatData _asbp_global_game_instance) (.indxNum (Utilities|Struct|BreakS_Hats (Variables|Default|Gethat))))))
    (Actor|DestroyActor)
    (Variables|Default|Setdestroyed true)))

(event EventTick
  (params (DeltaSeconds :type Float%20%28single-precision%29))
  ;[0 1 0.1796 1 34] HANDLE HAT MOVEMENT
  (bind _output_get (Variables|Default|SetElapsedTime (+ (Variables|Default|GetElapsedTime) (* DeltaSeconds (Variables|Default|GetMoveDirection)))))
  (if (Variables|Default|GetOpenForPickup)
    (CallFunction|MoveObject (Variables|Default|GetHatPivot) _output_get DeltaSeconds)
    (else
      (CallFunction|MoveObject (Variables|Default|GetBoxPivot) _output_get DeltaSeconds)))
  (if (or (< (Variables|Default|GetElapsedTime) 0.0) (> (Variables|Default|GetElapsedTime) (Variables|Default|GetBobSpeed)))
    (Variables|Default|SetMoveDirection (* (Variables|Default|GetMoveDirection) -1)))
  (if (Variables|Default|GethearJingle)
    (CallFunction|GetPlayerLocation)))

(fn ConstructionScript
  (bind _chestlid (Variables|Default|GetChestLid))
  (bind _chestbase (Variables|Default|GetChestBase))
  (bind _chestlid_2 (Variables|Default|GetChestLid))
  (bind _chestbase_2 (Variables|Default|GetChestBase))
  ;[1 1 1] Get hat structure from data table based on hat type
  (Components|Box|SetBoxExtent (Variables|Default|GethatCollisionBox) (Variables|Default|GethatJingleSize) true)
  (Variables|Default|SetmaxDistance (.X (Math|Vector|BreakVector (Variables|Default|GethatJingleSize))))
  (bind _returnvalue (Utilities|GetDataTableRow "/Game/Blueprints/HatShop/DT_Hats.DT_Hats" (Utilities|String|StringToName (Utilities|String|EnumtoString (Variables|Default|GethatType))))
    (:then
      ;[1 1 1 1 40] Set mesh to hat type, hide box / hat pivot if needed.
      (Variables|Default|Sethat _returnvalue)
      (Components|StaticMesh|SetStaticMesh (Variables|Default|GetHatMesh) (.hatModel (Utilities|Struct|BreakS_Hats _returnvalue)))
      (if (not (Variables|Default|GetOpenForPickup))
        (Development|SetHiddeninGame (Variables|Default|GetHatPivot) true true)
        (Collision|SetCollisionEnabled _chestbase_2 "QueryAndPhysics")
        (Rendering|SetVisibility _chestbase_2 true false)
        (Collision|SetCollisionEnabled _chestlid "QueryAndPhysics")
        (Rendering|SetVisibility _chestlid true false)
        (else
          (Development|SetHiddeninGame (Variables|Default|GetBoxPivot) true true)
          (Collision|SetCollisionEnabled _chestbase "NoCollision")
          (Rendering|SetVisibility _chestbase false false)
          (Collision|SetCollisionEnabled _chestlid_2 "NoCollision")
          (Rendering|SetVisibility _chestlid_2 false false))))))

(fn GivePlayerHat
  (params (Player :type BP%20Third%20Person%20Character%20Object%20Reference))
  ;[1 1 1 1 50] When giving a player a hat, cast to the global instance and set the unlocked value to true. This way the hat is unlocked universally
  (bind _returnvalue (Utilities|GetDataTableRow "/Game/Blueprints/HatShop/DT_Hats.DT_Hats" (Utilities|String|StringToName (Utilities|String|EnumtoString (Variables|Default|GethatType))))
    (:then
      (bind _asbp_global_game_instance (Utilities|Casting|CastToBP_Global_GameInstance (Game|GetGameInstance)))
      (Utilities|Array|SetArrayElem (Variables|/Game/Blueprints/BP_Global_GameInstance.BP_Global_GameInstance_C|GethatData _asbp_global_game_instance) (.indxNum (Utilities|Struct|BreakS_Hats _returnvalue)) (Utilities|Struct|MakeS_Hats (.hatType (Utilities|Struct|BreakS_Hats _returnvalue)) (.HatName (Utilities|Struct|BreakS_Hats _returnvalue)) (.indxNum (Utilities|Struct|BreakS_Hats _returnvalue)) (.hatModel (Utilities|Struct|BreakS_Hats _returnvalue)) true false (.hatDescription (Utilities|Struct|BreakS_Hats _returnvalue)))))))

(fn MoveObject
  (params (pivot :type Scene%20Component%20Object%20Reference) (elapsedTime :type Float%20%28double-precision%29) (deltaTime :type Float%20%28double-precision%29))
  (bind _relativelocation (Variables|/Script/Engine.SceneComponent|GetRelativeLocation pivot))
  (if (not (Variables|Default|Getdestroyed))
    (Transformation|SetRelativeLocation pivot (Math|Vector|MakeVector (.x _relativelocation) (.y _relativelocation) (Math|Interpolation|Ease "EaseInOut" elapsedTime 3e+01 5e+01 2.0)) false false)
    (Transformation|AddRelativeRotation pivot (Math|Rotator|MakeRotator 0.0 0.0 (* deltaTime (* (Variables|Default|GetRotationSpeed) 1e+01))) false false)
    (return)))

(fn GetRunePercentage
  (bind _tpc_player (Variables|Default|GetTPC_Player))
  ;[0.2444 1 0.1655] CALCULATE PERCENTAGE
  (Utilities|IsValid _tpc_player
    (:Is%20Valid
      (return (/ (Math|Conversions|ToFloat(Integer) (Variables|/Game/Blueprints/Player/Components/BPC_Currency.BPC_Currency_C|Getcurrency (Variables|/Game/Blueprints/Player/BP_ThirdPersonCharacter.BP_ThirdPersonCharacter_C|GetBPC_Currency _tpc_player))) (Math|Conversions|ToFloat(Integer) (Variables|Default|GetTotalRunes)))))))

(fn UnlockHat
  ;[0.1458 0.812 1] EXPLODE BOX - HAT UNLOCKED
  (Components|Activation|Activate (Variables|Default|GetNS_SnowballExplosion) false)
  ;[1 0.4063 0.03844] HAT IS VISIBLE
  (Development|SetHiddeninGame (Variables|Default|GetBoxPivot) true true)
  (Development|SetHiddeninGame (Variables|Default|GetHatPivot) false true)
  (Development|SetHiddeninGame (Variables|Default|GetHatCollision) true true)
  (Variables|Default|SetOpenForPickup true))

(fn SetLevelVariable
  (bind _returnvalue (Game|GetCurrentLevelName true))
  (switch string _returnvalue
    (:Tutorial
      (Variables|Default|SetlevelNames "NewEnumerator8"))
    (:FireBreathLevel
      (Variables|Default|SetlevelNames "NewEnumerator0"))
    (:SuperJumpLevel
      (Variables|Default|SetlevelNames "NewEnumerator1"))
    (:TimeSlowLevel
      (Variables|Default|SetlevelNames "NewEnumerator7"))))