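; Camera track actor that moves a camera along a spline to follow a character, with an Enter box that switches the player's locked camera on and off.
; The owner's nearest point on the Path spline, minus a lag distance, gives a spline time that places the camera on the separate CameraTrack spline.
; Tick interpolates the camera toward that location and a look-at rotation on the owner set by SetCamOwner.
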(event OnComponentBeginOverlap(Enter1)
  (params (OverlappedComponent :type Primitive%20Component%20Object%20Reference) (OtherActor :type Actor%20Object%20Reference) (OtherComp :type Primitive%20Component%20Object%20Reference) (OtherBodyIndex :type Integer) (bFromSweep :type Boolean) (SweepResult :type Hit%20Result%20Structure%20%28by%20ref%29))
  ;[1 0.0625 0.0625] Outdated methods using multiple collision boxes (probs should delete)
)

(event OnComponentBeginOverlap(Exit1)
  (params (OverlappedComponent :type Primitive%20Component%20Object%20Reference) (OtherActor :type Actor%20Object%20Reference) (OtherComp :type Primitive%20Component%20Object%20Reference) (OtherBodyIndex :type Integer) (bFromSweep :type Boolean) (SweepResult :type Hit%20Result%20Structure%20%28by%20ref%29))
  ;[1 0.0625 0.0625] Outdated methods using multiple collision boxes (probs should delete)
)

(event OnComponentBeginOverlap(Enter)
  (params (OverlappedComponent :type Primitive%20Component%20Object%20Reference) (OtherActor :type Actor%20Object%20Reference) (OtherComp :type Primitive%20Component%20Object%20Reference) (OtherBodyIndex :type Integer) (bFromSweep :type Boolean) (SweepResult :type Hit%20Result%20Structure%20%28by%20ref%29))
  (bind _playerref (Variables|Default|GetPlayerRef))
  ;[1 1 1] Activate fixed camera on overlapping 'Enter' box
  (if (== OtherComp (Variables|Default|GetCharacterColliderRef))
    (Variables|Default|SetIsMainTrack? true)
    (Default|UseMainCameraTrack _playerref)
    (Default|OnEnterLockedCamera _playerref)))

(event OnComponentBeginOverlap(Exit)
  (params (OverlappedComponent :type Primitive%20Component%20Object%20Reference) (OtherActor :type Actor%20Object%20Reference) (OtherComp :type Primitive%20Component%20Object%20Reference) (OtherBodyIndex :type Integer) (bFromSweep :type Boolean) (SweepResult :type Hit%20Result%20Structure%20%28by%20ref%29))
  ;[1 0.0625 0.0625] Outdated methods using multiple collision boxes (probs should delete)
)

(event OnComponentEndOverlap(Enter)
  (params (OverlappedComponent :type Primitive%20Component%20Object%20Reference) (OtherActor :type Actor%20Object%20Reference) (OtherComp :type Primitive%20Component%20Object%20Reference) (OtherBodyIndex :type Integer))
  (bind _playerref (Variables|Default|GetPlayerRef))
  ;[1 1 1] Deactivate fixed camera on leaving 'Enter' box
  (if (== OtherComp (Variables|Default|GetCharacterColliderRef))
    (Variables|Default|SetIsMainTrack? false)
    (Default|UseMainCameraTrack _playerref)
    (Default|OnExitLockedCamera _playerref)))

(event EventBeginPlay
  ;[1 1 1] Start New Cam System
  (bind _returnvalue (Actor|GetActorOfClass "/Game/Blueprints/Player/BP_ThirdPersonCharacter.BP_ThirdPersonCharacter_C"))
  (Variables|Default|SetCharacterColliderRef (Variables|/Script/Engine.Character|GetCapsuleComponent _returnvalue))
  (Variables|Default|SetPlayerRef _returnvalue))

(event EventTick
  (params (DeltaSeconds :type Float%20%28single-precision%29))
  (bind _camowner (Variables|Default|GetCamOwner)
    (:then
      (CallFunction|UpdateCamera "0, 0, 0" "0, 0, 0" (Transformation|GetActorLocation _camowner))
      (CallFunction|InterpLocation)
      (CallFunction|InterpRotation))
    (:else)))

(fn ConstructionScript)

(fn SetCamOwner
  (params (Character :type BP%20Third%20Person%20Character%20Object%20Reference))
  (bind _output_get (Variables|Default|SetCamOwner Character))
  (Utilities|IsValid _output_get
    (:Is%20Valid
      (Actor|Tick|SetActorTickEnabled true)
      (CallFunction|UpdateCamera "0, 0, 0" "0, 0, 0" (Transformation|GetActorLocation (Variables|Default|GetCamOwner))))
    (:Is%20Not%20Valid
      (Actor|Tick|SetActorTickEnabled false))))

(fn UpdateCamera
  (params (WorldLocationHuman :type Vector) (WorldLocationSnowman :type Vector) (WorldLocationCamOwner :type Vector))
  (Variables|Default|SetDesiredLocation (Spline|GetLocationatTime (Variables|Default|GetCameraTrack) (CallFunction|GetTimeAlongSplineatNearbyLocation WorldLocationCamOwner (Variables|Default|GetMovement%20Lag%20Offset)) "World" false))
  (Variables|Default|SetDesiredRotation (Math|Rotator|FindLookatRotation (Transformation|GetWorldLocation (Variables|Default|GetCamera)) (Transformation|GetActorLocation (Variables|Default|GetCamOwner)))))

(fn GetTimeAlongSplineatNearbyLocation
  (params (World%20Location :type Vector) (Distance%20Lag :type Float%20%28double-precision%29))
  (bind _path (Variables|Default|GetPath))
  (return (Class|SplineComponent|GetTimeatDistanceAlongSpline _path (- (Class|SplineComponent|GetDistanceAlongSplineatSplineInputKey _path (Class|SplineComponent|FindInputKeyClosesttoWorldLocation _path World%20Location)) Distance%20Lag))))

(fn InterpLocation
  (bind _camera (Variables|Default|GetCamera))
  (bind _returnvalue (Transformation|GetWorldLocation _camera))
  (if (not (Utilities|Operators|EqualEqual (Variables|Default|GetDesiredLocation) _returnvalue 1.0))
    (Transformation|SetWorldLocation (Variables|Default|GetCamera) (Math|Interpolation|VInterpTo _returnvalue (Variables|Default|GetDesiredLocation) (Utilities|Time|GetWorldDeltaSeconds) (Variables|Default|GetMovement%20Lag%20Speed)) false false)))

(fn InterpRotation
  (bind _camera (Variables|Default|GetCamera))
  (bind _returnvalue (Transformation|GetWorldRotation _camera))
  (if (not (Utilities|Operators|EqualEqual (Variables|Default|GetDesiredRotation) _returnvalue 0.01))
    (Transformation|SetWorldRotation (Variables|Default|GetCamera) (Math|Interpolation|RInterpTo _returnvalue (Variables|Default|GetDesiredRotation) (Utilities|Time|GetWorldDeltaSeconds) (Variables|Default|GetRotation%20Lag%20Speed)) false false)))

(fn GetPathLocationNear
  (params (NearWorldPosition :type Vector))
  (return (Spline|GetLocationatTime (Variables|Default|GetPath) (CallFunction|GetTimeAlongSplineatNearbyLocation NearWorldPosition (Variables|Default|GetMovement%20Lag%20Offset)) "World" false)))