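; BP_WalkingPenguin is a decorative level penguin whose mesh swings in yaw to mimic a waddling walk.
; A timeline, with configurable length and rate, alternates forward and reverse on each finish, lerping yaw between plus and minus the walk amount.
; The referenced MultiPatrolPath's PlayingBackwards flag flips the facing 180 degrees.
; BeginPlay also caches that path's spline and whether it exists; this graph contains no movement logic.
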(event Custom|PlayWalkRotationTimeline
  (bind _walkrotationamount (Variables|Default|GetwalkRotationAmount))
  (bind _walkrotationamount_2 (Variables|Default|GetwalkRotationAmount))
  (if (Variables|Default|GetwalkRotationTimelineReverse)
    (bind _newtrack_0 (Timeline|TL_WalkRotation PlayFromStart)
      (:Update
        ;[1 1 1] rotate model
        (if (Variables|/Game/Blueprints/Level/Spikes/BP_MultiPatrolPath.BP_MultiPatrolPath_C|GetPlayingBackwards (Variables|Default|GetmultiPatrolPathRef))
          ;;[1 0.8152 0.2044] +180 degrees when going backwards along path
          (Transformation|SetRelativeRotation (Variables|Default|GetPenguinMesh) (Math|Rotator|MakeRotator 0.0 0.0 (+ (Math|Float|Lerp (* _walkrotationamount_2 -1.0) _walkrotationamount_2 _newtrack_0) 2.7e+02)) false false)
          (else
            (Transformation|SetRelativeRotation (Variables|Default|GetPenguinMesh) (Math|Rotator|MakeRotator 0.0 0.0 (+ (Math|Float|Lerp (* _walkrotationamount -1.0) _walkrotationamount _newtrack_0) 9e+01)) false false))))
      (:Finished
        (Variables|Default|SetwalkRotationTimelineReverse (not (Variables|Default|GetwalkRotationTimelineReverse)))
        (CallFunction|PlayWalkRotationTimeline)))
    (else
      (Timeline|TL_WalkRotation ReverseFromEnd))))

(event EventBeginPlay
  (bind _tl_walkrotation (Variables|Default|GetTL_WalkRotation))
  (Components|Timeline|SetTimelineLength _tl_walkrotation (Variables|Default|GetwalkRotationTimelineLength))
  (Components|Timeline|SetPlayRate _tl_walkrotation (Variables|Default|GetwalkRotationTimelineRate))
  (CallFunction|PlayWalkRotationTimeline)
  (bind _output_get (Variables|Default|SetwalkSplineRef (Actor|GetComponentbyClass (Variables|Default|GetmultiPatrolPathRef) "/Script/Engine.SplineComponent")))
  (Variables|Default|SethasMultiPatrolPath (not (== _output_get 0))))

(fn ConstructionScript)