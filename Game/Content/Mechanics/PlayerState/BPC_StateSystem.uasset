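; BPC_StateSystem is a component that tracks the player's movement state as grounded, jumping or climbing.
; Jump, land and climb events each set CurrentState, print a debug message and update IsClimbing on the animation Blueprint, true only for climbing.
; A helper reaches that Blueprint by casting the owner to BP_ThirdPersonCharacter and its mesh's anim instance to PlayerAnim_BP.
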(event Custom|OnPlayerJump
  (Variables|Default|SetCurrentState "NewEnumerator2")
  (Development|PrintString "[HELLO] jumping")
  (bind _asplayer_anim_bp (Utilities|AccessAnimationClass))
  (Variables|/Game/DevelopmentLevels/Arun/Character_Model_and_Animation/PlayerAnim_BP.PlayerAnim_BP_C|SetIsClimbing _asplayer_anim_bp false))

(event Custom|OnPlayerLand
  (Variables|Default|SetCurrentState "NewEnumerator0")
  (Development|PrintString "[HELLO] grounded")
  (bind _asplayer_anim_bp (Utilities|AccessAnimationClass))
  (Variables|/Game/DevelopmentLevels/Arun/Character_Model_and_Animation/PlayerAnim_BP.PlayerAnim_BP_C|SetIsClimbing _asplayer_anim_bp false))

(event Custom|OnPlayerClimb
  (Variables|Default|SetCurrentState "NewEnumerator1")
  (Development|PrintString "[HELLO] climbing")
  (bind _asplayer_anim_bp (Utilities|AccessAnimationClass))
  (Variables|/Game/DevelopmentLevels/Arun/Character_Model_and_Animation/PlayerAnim_BP.PlayerAnim_BP_C|SetIsClimbing _asplayer_anim_bp true))