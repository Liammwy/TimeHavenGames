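; Cutscene manager actor that plays a Level Sequence and signals when it ends.
; The PlayCutscene function calls through to an event that validates the LevelSequenceActor, starts its SequencePlayer and then binds to OnFinished.
; When playback finishes, the bound handler calls CutsceneFinished to notify other code.
; Debug prints trace the trigger, player name and completion.
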(event Custom|PlayCutscene_Event
  (bind _levelsequenceactor (Variables|Default|GetLevelSequenceActor))
  (bind _sequenceplayer (Variables|/Script/LevelSequence.LevelSequenceActor|GetSequencePlayer _levelsequenceactor))
  (Development|PrintString "PlayCutscene_Event Triggered!" true true "(R=1.000000,G=0.034391,B=0.793774,A=1.000000)")
  (Utilities|IsValid _levelsequenceactor
    (:Is%20Valid
      (Development|PrintString (Utilities|GetDisplayName _sequenceplayer) true true "(R=1.000000,G=0.854225,B=0.022275,A=1.000000)")
      (Sequencer|Player|Play _sequenceplayer :!class /Script/MovieScene.MovieSceneSequencePlayer)
      (EventDispatchers|BindEventtoOnFinished _sequenceplayer (delegate Custom|OnCutsceneEnded)))))

(event Custom|OnCutsceneEnded
  (Development|PrintString "Hello")
  (Default|CallCutsceneFinished))

(event EventBeginPlay)

(event Collision|EventActorBeginOverlap
  (params (OtherActor :type Actor%20Object%20Reference)))

(event EventTick
  (params (DeltaSeconds :type Float%20%28single-precision%29)))

(fn ConstructionScript)

(fn PlayCutscene
  (CallFunction|PlayCutsceneEvent))