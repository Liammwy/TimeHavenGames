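; BP_SignArrow is an arrow sign whose Widget component is oriented by Left, Right, Up and Down flags.
; The construction script sets the widget's relative rotation through nested branches, with Left taking priority over Right and Up over Down, giving sideways and diagonal directions.
; With neither Left nor Right, rotation is untouched; the straight-down rotation sits behind a repeated Down check in the Right-only path, where Down is already false.
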(fn ConstructionScript
  (if (Variables|Default|Getleft)
    (if (Variables|Default|Getup)
      (Transformation|SetRelativeRotation (Variables|Default|GetWidget) "0.000000,-90.000000,45.000000" false false)
      (elif (Variables|Default|Getdown)
        (Transformation|SetRelativeRotation (Variables|Default|GetWidget) "0.000000,-90.000000,135.000000" false false)
        (else
          (Transformation|SetRelativeRotation (Variables|Default|GetWidget) "0.000000,-90.000000,90.000000" false false))))
    (elif (Variables|Default|Getright)
      (if (Variables|Default|Getup)
        (Transformation|SetRelativeRotation (Variables|Default|GetWidget) "0.000000,-90.000000,-45.000000" false false)
        (elif (Variables|Default|Getdown)
          (Transformation|SetRelativeRotation (Variables|Default|GetWidget) "0.000000,-90.000000,-135.000000" false false)
          (else
            (Transformation|SetRelativeRotation (Variables|Default|GetWidget) "0.000000,-90.000000,-90.000000" false false)
            (if (Variables|Default|Getdown)
              (Transformation|SetRelativeRotation (Variables|Default|GetWidget) "0.000000,-90.000000,180.000000" false false))))))))