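; BP_Refule is a collectible refuel pickup that resets the player's hover time and respawns.
; When the player pawn overlaps its box, it hides the mesh, disables overlap events, plays a 2D refuelling sound and calls ResetHoverTime on the character's BPC_Hover component.
; Instead of being destroyed, it waits RespawnTime, then restores visibility and overlap events for reuse.
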(event OnComponentBeginOverlap(Box)
  (params (OverlappedComponent :type Primitive%20Component%20Object%20Reference) (OtherActor :type Actor%20Object%20Reference) (OtherComp :type Primitive%20Component%20Object%20Reference) (OtherBodyIndex :type Integer) (bFromSweep :type Boolean) (SweepResult :type Hit%20Result%20Structure%20%28by%20ref%29))
  ;[1 1 1] Respawns box and resets the player hover time
  (if (== OtherActor (Game|Player|GetPlayerPawn 0))
    (Rendering|SetVisibility (Variables|Default|GetStaticMesh) false false)
    (Variables|/Script/Engine.PrimitiveComponent|SetbGenerateOverlapEvents (Variables|Default|GetBox) false)
    (bind _asbp_third_person_character (Utilities|Casting|CastToBP_ThirdPersonCharacter (Game|Player|GetPlayerPawn 0)))
    (Class|FMODBlueprintStatics|PlayEvent2D "/Game/FMOD/Events/Refuelling.Refuelling")
    (Default|ResetHoverTime (Actor|GetComponentbyClass _asbp_third_person_character "/Game/Blueprints/Player/Components/BPC_Hover.BPC_Hover_C"))
    (Utilities|FlowControl|Delay (Variables|Default|GetRespawn%20Time))
    (Rendering|SetVisibility (Variables|Default|GetStaticMesh) true false)
    (Variables|/Script/Engine.PrimitiveComponent|SetbGenerateOverlapEvents (Variables|Default|GetBox) true)))

(event EventBeginPlay)

(event Collision|EventActorBeginOverlap
  (params (OtherActor :type Actor%20Object%20Reference)))

(event EventTick
  (params (DeltaSeconds :type Float%20%28single-precision%29)))

(fn ConstructionScript)