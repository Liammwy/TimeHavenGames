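; Player character component that reacts to special floors the character stands on, currently bounce pads.
; On BeginPlay it caches the owning third-person character and its movement component.
; Each tick it compares the movement component's floor actor to a CurrentFloor variable, which is never updated here.
; When they differ, the floor's BPC_Floor_StandOnEvent type selects the response, passing the player to BP_BouncePad and triggering the bounce.
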(event EventBeginPlay
  (bind _asbp_third_person_character (Utilities|Casting|CastToBP_ThirdPersonCharacter (Components|GetOwner)))
  (Variables|Default|SetcharacterMovement (Variables|/Script/Engine.Character|GetCharacterMovement _asbp_third_person_character))
  (Variables|Default|SetplayerRef _asbp_third_person_character))

(event EventTick
  (params (DeltaSeconds :type Float%20%28single-precision%29))
  (bind _charactermovement (Variables|Default|GetcharacterMovement))
  (bind _currentfloor (Variables|/Script/Engine.CharacterMovementComponent|GetCurrentFloor _charactermovement))
  (bind _hitresult (Utilities|Struct|BreakFindFloorResult _currentfloor))
  (bind _hitactor (Collision|BreakHitResult _hitresult))
  (bind _returnvalue (Actor|GetComponentsByClass _hitactor "/Game/Blueprints/Level/Components/BPC_Floor_StandOnEvent.BPC_Floor_StandOnEvent_C"))
  (if (not (== (Variables|Default|GetcurrentFloor) _hitactor))
    (if (> (Utilities|Array|Length _returnvalue) 0)
      (switch Utilities|FlowControl|Switch|SwitchonEnum_Floor_StandOnEvent (Variables|/Game/Blueprints/Level/Components/BPC_Floor_StandOnEvent.BPC_Floor_StandOnEvent_C|GetEventType (Utilities|Array|Get(acopy) _returnvalue))
        (:NewEnumerator1
          (bind _asbp_bounce_pad (Utilities|Casting|CastToBP_BouncePad _hitactor))
          (Variables|/Game/Blueprints/Level/BP_BouncePad.BP_BouncePad_C|SetPlayerRef _asbp_bounce_pad (Variables|Default|GetplayerRef))
          (Default|BouncePlayer _asbp_bounce_pad))))))