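; Patrol path that moves an assigned actor along a spline in a repeating loop, snapping it to the first point in the construction script.
; A timeline, with play rate scaled by TimeLineLength, maps its alpha to spline distance up to the last point and restarts from the beginning when finished.
; When OnGround is set, it drives BP_MovingSpikeBall's Rolling using the alpha delta and a look-ahead spline direction for earlier turns.
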(event Custom|Play%20TimeLine
  (bind _spline (Variables|Default|GetSpline))
  (Variables|Default|SetPrevTimelineAlpha 0.0)
  (bind _newtrack_0 (Timeline|Timeline PlayFromStart)
    (:Update
      (Variables|Default|SetPrevActorPos (Transformation|GetActorLocation (Variables|Default|GetSpline%20Actor)))
      (Transformation|SetActorLocation (Variables|Default|GetSpline%20Actor) (Spline|GetLocationatDistanceAlongSpline (Variables|Default|GetSpline) (Math|Float|Lerp 0.0 (Spline|GetDistanceAlongSplineatSplinePoint _spline (- (Spline|GetNumberOfSplinePoints _spline) 1)) _newtrack_0) "World") false false)
      (if (Variables|Default|GetOnGround)
        ;[1 1 1] Rotation Handling Code
        (bind _asbp_moving_spike_ball (Utilities|Casting|CastToBP_MovingSpikeBall (Variables|Default|GetSpline%20Actor)))
        (Default|Rolling _asbp_moving_spike_ball (Class|SplineComponent|GetDirectionatTime (Variables|Default|GetSpline) (+ _newtrack_0 0.2) "World" false) (- _newtrack_0 (Variables|Default|GetPrevTimelineAlpha)))
        (Variables|Default|SetPrevTimelineAlpha _newtrack_0)))
    (:Finished
      (CallFunction|PlayTimeLine))))

(event EventBeginPlay
  (Components|Timeline|SetPlayRate (Variables|Default|GetTimeline) (/ 1.0 (Variables|Default|GetTimeLine%20Length)))
  (CallFunction|PlayTimeLine))

(fn ConstructionScript
  ;[1 1 1] Puts selected actor On spline
  (Transformation|SetActorLocation (Variables|Default|GetSpline%20Actor) (Spline|GetLocationatSplinePoint (Variables|Default|GetSpline) 0 "World") false false))