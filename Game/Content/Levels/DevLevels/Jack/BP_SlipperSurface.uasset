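; Slippery ice surface actor that makes the player slide while inside its box trigger.
; On overlap it lowers the character's ground friction and braking, sets the sliding flag on the Snowman or player anim blueprint, notifies the state system and starts an FMOD slip sound.
; Leaving restores fixed movement values and stops the sound; Tick pauses it while horizontal velocity is low.
; The construction script applies the chosen mesh and fits the box to its bounds.
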(event OnComponentBeginOverlap(Box)
  (params (OverlappedComponent :type Primitive%20Component%20Object%20Reference) (OtherActor :type Actor%20Object%20Reference) (OtherComp :type Primitive%20Component%20Object%20Reference) (OtherBodyIndex :type Integer) (bFromSweep :type Boolean) (SweepResult :type Hit%20Result%20Structure%20%28by%20ref%29))
  (bind _playerref (Variables|Default|GetPlayerRef))
  (bind _charactermovement (Variables|/Script/Engine.Character|GetCharacterMovement _playerref))
  (bind _bpc_statesystem (Variables|/Game/Blueprints/Player/BP_ThirdPersonCharacter.BP_ThirdPersonCharacter_C|GetBPC_StateSystem _playerref))
  (if (== OtherComp (Variables|Default|GetPlayerHitboxRef))
    (Variables|/Script/Engine.CharacterMovementComponent|SetGroundFriction _charactermovement 0.0)
    (Variables|/Script/Engine.CharacterMovementComponent|SetBrakingDecelerationWalking _charactermovement 3.5e+02)
    (Variables|Default|SetOnIceSurface true)
    (bind (_asnew_player_anim_bp _assnowman_anim_bp _snowman) (Default|AccessAnimClass _bpc_statesystem))
    (if _snowman
      (Variables|/Game/Blueprints/Player/Animation/Snowman_AnimBp.Snowman_AnimBp_C|SetIsSliding _assnowman_anim_bp true)
      (else
        (Variables|/Game/Blueprints/Player/Animation/NewPlayerAnim_BP.NewPlayerAnim_BP_C|SetIsSliding _asnew_player_anim_bp true)))
    (Default|OnPlayerSlipped _bpc_statesystem)
    (bind _returnvalue (Class|FMODBlueprintStatics|PlayEvent2D "/Game/FMOD/Events/IceSlipping.IceSlipping"))
    (Variables|Default|Setfmod _returnvalue)
    (Variables|Default|SetisPaused false)))

(event OnComponentEndOverlap(Box)
  (params (OverlappedComponent :type Primitive%20Component%20Object%20Reference) (OtherActor :type Actor%20Object%20Reference) (OtherComp :type Primitive%20Component%20Object%20Reference) (OtherBodyIndex :type Integer))
  (bind _playerref (Variables|Default|GetPlayerRef))
  (bind _charactermovement (Variables|/Script/Engine.Character|GetCharacterMovement _playerref))
  (bind _bpc_statesystem (Variables|/Game/Blueprints/Player/BP_ThirdPersonCharacter.BP_ThirdPersonCharacter_C|GetBPC_StateSystem _playerref))
  (if (== OtherComp (Variables|Default|GetPlayerHitboxRef))
    (Variables|/Script/Engine.CharacterMovementComponent|SetGroundFriction _charactermovement 8.0)
    (Variables|/Script/Engine.CharacterMovementComponent|SetBrakingDecelerationWalking _charactermovement 2e+03)
    (Variables|Default|SetOnIceSurface false)
    (bind (_asnew_player_anim_bp _assnowman_anim_bp _snowman) (Default|AccessAnimClass _bpc_statesystem))
    (if _snowman
      (Variables|/Game/Blueprints/Player/Animation/Snowman_AnimBp.Snowman_AnimBp_C|SetIsSliding _assnowman_anim_bp false)
      (else
        (Variables|/Game/Blueprints/Player/Animation/NewPlayerAnim_BP.NewPlayerAnim_BP_C|SetIsSliding _asnew_player_anim_bp false)))
    (Default|OnPlayerLand _bpc_statesystem)
    (Class|FMODBlueprintStatics|EventInstanceStop (stale OnComponentBeginOverlap(Box) _returnvalue) false)
    (Variables|Default|SetisPaused true)))

(event EventBeginPlay
  (bind _returnvalue (Actor|GetActorOfClass "/Game/Blueprints/Player/BP_ThirdPersonCharacter.BP_ThirdPersonCharacter_C"))
  (Utilities|IsValid _returnvalue
    (:Is%20Valid
      (Variables|Default|SetPlayerRef _returnvalue)
      (Variables|Default|SetPlayerHitboxRef (Variables|/Script/Engine.Character|GetCapsuleComponent _returnvalue)))))

(event EventTick
  (params (DeltaSeconds :type Float%20%28single-precision%29))
  (bind _playerref (Variables|Default|GetPlayerRef))
  (bind _returnvalue (Transformation|GetVelocity _playerref))
  (if (Variables|Default|GetOnIceSurface)
    (if (and (Math|Float|InRange(Float) (.x _returnvalue) -75.0 75.0) (Math|Float|InRange(Float) (.y _returnvalue) -75.0 75.0))
      (Class|FMODBlueprintStatics|EventInstanceSetPaused (Variables|Default|Getfmod) true)
      (Variables|Default|SetisPaused true)
      (elif (Variables|Default|GetisPaused)
        (Class|FMODBlueprintStatics|EventInstanceSetPaused (Variables|Default|Getfmod) false)
        (Variables|Default|SetisPaused false)))))

(fn ConstructionScript
  (Components|StaticMesh|SetStaticMesh (Variables|Default|GetSlipperSurfaceMesh) (Variables|Default|GetMesh))
  (Components|Box|SetBoxExtent (Variables|Default|GetBox) (.Max (Components|StaticMesh|GetLocalBounds (Variables|Default|GetSlipperSurfaceMesh))) true)
  (Transformation|SetRelativeLocation (Variables|Default|GetBox) (.location (Transformation|GetRelativeTransform (Variables|Default|GetSlipperSurfaceMesh))) false false))