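; BP_FallingPlat is a level platform that falls after the player touches it, then respawns.
; BeginPlay caches the BP_ThirdPersonCharacter capsule, and only that component overlapping TriggerMesh starts the fall.
; After a delay, FallingPlat starts simulating physics and is set visible.
; After a second delay, the actor destroys itself, then calls RespawnPlat to spawn a fresh copy at the actor's current transform.
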(event OnComponentBeginOverlap(TriggerMesh)
  (params (OverlappedComponent :type Primitive%20Component%20Object%20Reference) (OtherActor :type Actor%20Object%20Reference) (OtherComp :type Primitive%20Component%20Object%20Reference) (OtherBodyIndex :type Integer) (bFromSweep :type Boolean) (SweepResult :type Hit%20Result%20Structure%20%28by%20ref%29))
  (if (== OtherComp (Variables|Default|GetPlayerHitboxRef))
    (Utilities|FlowControl|Delay (Variables|Default|GetTime%20From%20landing%20to%20falling))
    (Physics|SetSimulatePhysics (Variables|Default|GetFalling%20Plat) true)
    (Rendering|SetVisibility (Variables|Default|GetFalling%20Plat) true false)
    (Utilities|FlowControl|Delay (Variables|Default|GetTime%20to%20respawn))
    (Actor|DestroyActor)
    (CallFunction|RespawnPlat)))

(event Custom|Respawn%20Plat
  (Game|SpawnActorfromClass "BP_FallingPlat_C" (Transformation|GetActorTransform) "Undefined" "MultiplyWithRoot" 0 0))

(event EventBeginPlay
  (bind _returnvalue (Actor|GetActorOfClass "/Game/Blueprints/Player/BP_ThirdPersonCharacter.BP_ThirdPersonCharacter_C"))
  (Variables|Default|SetPlayerRef _returnvalue)
  (Variables|Default|SetPlayerHitboxRef (Variables|/Script/Engine.Character|GetCapsuleComponent _returnvalue)))

(fn ConstructionScript)