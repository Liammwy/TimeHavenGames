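; Torch event listener Blueprint that reveals a hat pickup as the reward for lighting all torches.
; On BeginPlay it hides the referenced HatPickup's mesh and disables its collision.
; When the all-torches-ignited response fires, it plays a 2D torch jingle, shows the hat mesh and enables query-only collision, so the existing pickup is toggled rather than spawned.
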(event EventBeginPlay
  (bind _hatpickup (Variables|Default|GetHatPickup))
  ;[1 1 1] Hide hat on begin play
  (Collision|SetCollisionEnabled (Variables|/Game/Blueprints/HatShop/BP_HatCollectible.BP_HatCollectible_C|GetHatCollision _hatpickup) "NoCollision")
  (Rendering|SetVisibility (Variables|/Game/Blueprints/HatShop/BP_HatCollectible.BP_HatCollectible_C|GetHatMesh _hatpickup) false false))

(event EventRespondtoAllTorchesIgnited
  (bind _hatpickup (Variables|Default|GetHatPickup))
  ;[1 1 1] Show hat + activate collision when all torches lit
  (Class|FMODBlueprintStatics|PlayEvent2D "/Game/FMOD/Events/TorchJingle.TorchJingle")
  (Collision|SetCollisionEnabled (Variables|/Game/Blueprints/HatShop/BP_HatCollectible.BP_HatCollectible_C|GetHatCollision _hatpickup) "QueryOnly")
  (Rendering|SetVisibility (Variables|/Game/Blueprints/HatShop/BP_HatCollectible.BP_HatCollectible_C|GetHatMesh _hatpickup) true false))

(fn ConstructionScript
  (|CallParentFunction))