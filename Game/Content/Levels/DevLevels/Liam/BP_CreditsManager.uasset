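; Level manager for the credits screen that returns the player to the splash level when the credits end or are skipped.
; On BeginPlay it binds to the credits Level Sequence player's finished event.
; Sequence completion and the UI Back input both feed one DoOnce, which sets a manual black camera fade at zero amount, waits briefly, then opens the SlashScreen level.
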(event Custom|Return%20to%20Main%20Menu
  (Utilities|FlowControl|DoOnce false
    (:Completed
      (Class|PlayerCameraManager|SetManualCameraFade :self (Variables|/Script/Engine.PlayerController|GetPlayerCameraManager (Game|GetPlayerController 0)))
      (Utilities|FlowControl|Delay 1.0)
      (Game|OpenLevel(byName) "SlashScreen"))))

(event Input|EnhancedActionEvents|EnhancedInputActionIA_UI_Back
  (params (ActionValue :type Boolean) (ElapsedSeconds :type Float%20%28double-precision%29) (TriggeredSeconds :type Float%20%28double-precision%29) (InputAction :type Input%20Action%20Object%20Reference :default "/Game/Data/Input/UI_Actions/IA_UI_Back.IA_UI_Back"))
  (Utilities|FlowControl|DoOnce false
    (:Completed
      (Class|PlayerCameraManager|SetManualCameraFade :self (Variables|/Script/Engine.PlayerController|GetPlayerCameraManager (Game|GetPlayerController 0)))
      (Utilities|FlowControl|Delay 1.0)
      (Game|OpenLevel(byName) "SlashScreen"))))

(event EventBeginPlay
  (EventDispatchers|BindEventtoOnFinished (Variables|/Script/LevelSequence.LevelSequenceActor|GetSequencePlayer (Variables|Default|GetLevel%20Sequence)) (delegate Custom|Return%20to%20Main%20Menu)))

(fn ConstructionScript)