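; Breakable block power-up level actor that shatters when the player hits it mid super jump from inside its bottom trigger zone.
; Breaking hides the cube, plays a sound pitched for time dilation, spawns stored collectibles, zeroes the player's vertical velocity and notifies BPC_SuperJump.
; Ten fragment meshes then simulate physics, shrinking on Tick until hidden.
; The construction script freezes collectibles and line-traces down to place a ground decal.
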(event OnComponentHit(Cube)
  (params (HitComponent :type Primitive%20Component%20Object%20Reference) (OtherActor :type Actor%20Object%20Reference) (OtherComp :type Primitive%20Component%20Object%20Reference) (NormalImpulse :type Vector :default "0, 0, 0") (Hit :type Hit%20Result%20Structure%20%28by%20ref%29))
  (if (== OtherComp (Variables|Default|GetPlayerHitboxRef))
    (if (and (Variables|Default|GetplayerInBreakZone) (Variables|/Game/Blueprints/Player/Components/BPC_SuperJump.BPC_SuperJump_C|GetmidSuperJump (Variables|/Game/Blueprints/Player/BP_ThirdPersonCharacter.BP_ThirdPersonCharacter_C|GetBPC_SuperJump (Variables|Default|GetPlayerRef))))
      (CallFunction|BlockHitFunction true))))

(event OnComponentEndOverlap(BottomCollider)
  (params (OverlappedComponent :type Primitive%20Component%20Object%20Reference) (OtherActor :type Actor%20Object%20Reference) (OtherComp :type Primitive%20Component%20Object%20Reference) (OtherBodyIndex :type Integer))
  (if (== OtherComp (Variables|Default|GetPlayerHitboxRef))
    (Variables|Default|SetplayerInBreakZone false)
    (Development|PrintString "Hello")))

(event OnComponentBeginOverlap(BottomCollider)
  (params (OverlappedComponent :type Primitive%20Component%20Object%20Reference) (OtherActor :type Actor%20Object%20Reference) (OtherComp :type Primitive%20Component%20Object%20Reference) (OtherBodyIndex :type Integer) (bFromSweep :type Boolean) (SweepResult :type Hit%20Result%20Structure%20%28by%20ref%29))
  (if (== OtherComp (Variables|Default|GetPlayerHitboxRef))
    (Variables|Default|SetplayerInBreakZone true)))

(event EventBeginPlay
  (bind _returnvalue (Actor|GetActorOfClass "/Game/Blueprints/Player/BP_ThirdPersonCharacter.BP_ThirdPersonCharacter_C"))
  (Variables|Default|SetPlayerRef _returnvalue)
  (Variables|Default|SetPlayerHitboxRef (Variables|/Script/Engine.Character|GetCapsuleComponent _returnvalue))
  ;[1 1 1] Add all fragment meshes to array on BeginPlay
  (Utilities|Array|Add (Variables|Default|GetFragments) (Variables|Default|GetFragment_1))
  (Utilities|Array|Add (Variables|Default|GetFragments) (Variables|Default|GetFragment_2))
  (Utilities|Array|Add (Variables|Default|GetFragments) (Variables|Default|GetFragment_3))
  (Utilities|Array|Add (Variables|Default|GetFragments) (Variables|Default|GetFragment_4))
  (Utilities|Array|Add (Variables|Default|GetFragments) (Variables|Default|GetFragment_5))
  (Utilities|Array|Add (Variables|Default|GetFragments) (Variables|Default|GetFragment_6))
  (Utilities|Array|Add (Variables|Default|GetFragments) (Variables|Default|GetFragment_7))
  (Utilities|Array|Add (Variables|Default|GetFragments) (Variables|Default|GetFragment_8))
  (Utilities|Array|Add (Variables|Default|GetFragments) (Variables|Default|GetFragment_9))
  (Utilities|Array|Add (Variables|Default|GetFragments) (Variables|Default|GetFragment_10)))

(event EventTick
  (params (DeltaSeconds :type Float%20%28single-precision%29))
  (if (Variables|Default|GetisBroken)
    (if (not (Variables|Default|GetfragmentsDestroyed))
      (bind _output_get (Variables|Default|SettimeSinceBroken (+ (Variables|Default|GettimeSinceBroken) DeltaSeconds)))
      (if (>= _output_get (Variables|Default|GetbrokenFragmentLifetime))
        ;[1 1 1] Deactivate fragments when lifetime ended
        (for _array_element (Variables|Default|GetFragments)
          (Physics|SetSimulatePhysics _array_element false)
          (Rendering|SetVisibility _array_element false false)
          (Collision|SetCollisionEnabled _array_element "NoCollision")
          (Variables|Default|SetfragmentsDestroyed true))
        (else
          ;[1 1 1] Update shrinking mesh visuals
          (for _array_element_2 (Variables|Default|GetFragments)
            (Transformation|SetRelativeScale3D _array_element_2 (Math|Vector|MakeVector (- 1.0 (/ (Variables|Default|GettimeSinceBroken) (Variables|Default|GetbrokenFragmentLifetime))) (- 1.0 (/ (Variables|Default|GettimeSinceBroken) (Variables|Default|GetbrokenFragmentLifetime))) (- 1.0 (/ (Variables|Default|GettimeSinceBroken) (Variables|Default|GetbrokenFragmentLifetime)))))))))))

(fn ConstructionScript
  (bind _defaultsceneroot (Variables|Default|GetDefaultSceneRoot))
  (bind _returnvalue (Transformation|GetWorldLocation _defaultsceneroot))
  (Default|FreezeAllCollectibles (Variables|Default|GetBPC_CollectibleSpawner))
  (bind (_outhit _returnvalue_2) (Collision|LineTraceByChannel _returnvalue (- _returnvalue "0.000000,0.000000,1000.000000") "TraceTypeQuery1" false 0 "None"))
  (if _returnvalue_2
    (Transformation|SetWorldLocation (Variables|Default|GetDecal) (.Location (Collision|BreakHitResult _outhit)) false false)))

(fn BlockHitFunction
  (params (HitBottomColl :type Boolean))
  (bind _playerref (Variables|Default|GetPlayerRef))
  (bind _charactermovement (Variables|/Script/Engine.Character|GetCharacterMovement _playerref))
  (if (Variables|/Game/Blueprints/Player/Components/BPC_SuperJump.BPC_SuperJump_C|GetmidSuperJump (Variables|/Game/Blueprints/Player/BP_ThirdPersonCharacter.BP_ThirdPersonCharacter_C|GetBPC_SuperJump (Variables|Default|GetPlayerRef)))
    (bind _returnvalue (Class|FMODBlueprintStatics|PlayEventatLocation "/Game/FMOD/Events/BlockBreaking.BlockBreaking" (Transformation|GetActorTransform)))
    (if (== (Class|GameplayStatics|GetGlobalTimeDilation) 1.0)
      _
      (else
        (Class|FMODBlueprintStatics|EventInstanceSetPitch _returnvalue 0.5)))
    (Rendering|SetVisibility (Variables|Default|GetCube) false false)
    (Rendering|SetVisibility (Variables|Default|GetDecal) false false)
    (Collision|SetCollisionEnabled (Variables|Default|GetCube) "NoCollision")
    (Collision|SetCollisionEnabled (Variables|Default|GetBottomCollider) "NoCollision")
    ;[1 1 1] Spawn any collectibles inside block
    (Default|SpawnCollectibles (Variables|Default|GetBPC_CollectibleSpawner))
    (if HitBottomColl
      (Variables|/Script/Engine.MovementComponent|SetVelocity _charactermovement (Math|Vector|MakeVector (.x (Variables|/Script/Engine.MovementComponent|GetVelocity _charactermovement)) (.y (Variables|/Script/Engine.MovementComponent|GetVelocity _charactermovement)) 0.0))
      (Default|OnBlockHit (Actor|GetComponentbyClass _playerref "/Game/Blueprints/Player/Components/BPC_SuperJump.BPC_SuperJump_C"))
      ;[1 1 1] Trigger fragment physics
      (for _array_element (Variables|Default|GetFragments)
        (Physics|SetEnableGravity _array_element true)
        (Physics|SetSimulatePhysics _array_element true))
      (Variables|Default|SetisBroken true)
      (Variables|Default|SettimeSinceBroken 0.0))))