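; Torch event listener that reveals five rune pickups one after another once all torches are ignited.
; BeginPlay hides each rune's mesh and disables its collision box, and RespondtoAllTorchesIgnited starts a timer.
; Tick then shows the next rune at each ShowRuneInterval, choosing it by count through GetNextRuneToShow and enabling query collision.
; An older branch that shows all runes at once is left unconnected.
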(event EventBeginPlay
  (bind _rune_0 (Variables|Default|GetRune_0))
  (bind _rune_1 (Variables|Default|GetRune_1))
  (bind _rune_2 (Variables|Default|GetRune_2))
  (bind _rune_3 (Variables|Default|GetRune_3))
  (bind _rune_4 (Variables|Default|GetRune_4))
  ;[1 1 1] Hide all 5 runes on begin play
  (Rendering|SetVisibility (Variables|/Game/Blueprints/Collectibles/BP_Collectible.BP_Collectible_C|GetStaticMesh _rune_0) false false)
  (Collision|SetCollisionEnabled (Variables|/Game/Blueprints/Collectibles/BP_Collectible.BP_Collectible_C|GetBox _rune_0) "NoCollision")
  (Rendering|SetVisibility (Variables|/Game/Blueprints/Collectibles/BP_Collectible.BP_Collectible_C|GetStaticMesh _rune_1) false false)
  (Collision|SetCollisionEnabled (Variables|/Game/Blueprints/Collectibles/BP_Collectible.BP_Collectible_C|GetBox _rune_1) "NoCollision")
  (Rendering|SetVisibility (Variables|/Game/Blueprints/Collectibles/BP_Collectible.BP_Collectible_C|GetStaticMesh _rune_2) false false)
  (Collision|SetCollisionEnabled (Variables|/Game/Blueprints/Collectibles/BP_Collectible.BP_Collectible_C|GetBox _rune_2) "NoCollision")
  (Rendering|SetVisibility (Variables|/Game/Blueprints/Collectibles/BP_Collectible.BP_Collectible_C|GetStaticMesh _rune_3) false false)
  (Collision|SetCollisionEnabled (Variables|/Game/Blueprints/Collectibles/BP_Collectible.BP_Collectible_C|GetBox _rune_3) "NoCollision")
  (Rendering|SetVisibility (Variables|/Game/Blueprints/Collectibles/BP_Collectible.BP_Collectible_C|GetStaticMesh _rune_4) false false)
  (Collision|SetCollisionEnabled (Variables|/Game/Blueprints/Collectibles/BP_Collectible.BP_Collectible_C|GetBox _rune_4) "NoCollision"))

(event EventTick
  (params (DeltaSeconds :type Float%20%28single-precision%29))
  (if (Variables|Default|GetTorchEventTriggered)
    (if (not (Variables|Default|GetAllRunesShown))
      (bind _output_get (Variables|Default|SetTimeSinceTriggered (+ DeltaSeconds (Variables|Default|GetTimeSinceTriggered))))
      (if (>= _output_get (Variables|Default|GetNextShowRuneTime))
        (if true
          (bind _newparam (CallFunction|GetNextRunetoShow))
          (Rendering|SetVisibility (Variables|/Game/Blueprints/Collectibles/BP_Collectible.BP_Collectible_C|GetStaticMesh _newparam) true false)
          (Collision|SetCollisionEnabled (Variables|/Game/Blueprints/Collectibles/BP_Collectible.BP_Collectible_C|GetBox _newparam) "QueryOnly")
          (Variables|Default|SetNextShowRuneTime (+ (Variables|Default|GetShowRuneInterval) (Variables|Default|GetNextShowRuneTime)))
          (bind _output_get_2 (Variables|Default|SetNumRunesShown (+ (Variables|Default|GetNumRunesShown) 1)))
          (if (>= _output_get_2 5)
            (Variables|Default|SetAllRunesShown true)))))))

(event EventRespondtoAllTorchesIgnited
  (Variables|Default|SetTorchEventTriggered true)
  (Variables|Default|SetTimeSinceTriggered 0.0)
  (Variables|Default|SetNextShowRuneTime 0.0))

(fn ConstructionScript
  (|CallParentFunction))

(fn GetNextRunetoShow
  (if (== (Variables|Default|GetNumRunesShown) 0)
    (return (Variables|Default|GetRune_0))
    (elif (== (Variables|Default|GetNumRunesShown) 1)
      (return (Variables|Default|GetRune_1))
      (elif (== (Variables|Default|GetNumRunesShown) 2)
        (return (Variables|Default|GetRune_2))
        (elif (== (Variables|Default|GetNumRunesShown) 3)
          (return (Variables|Default|GetRune_3))
          (elif (== (Variables|Default|GetNumRunesShown) 4)
            (return (Variables|Default|GetRune_4))
            (else
              (return 0))))))))