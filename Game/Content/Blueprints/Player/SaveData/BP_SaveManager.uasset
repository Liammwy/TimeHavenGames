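; Save manager that persists the player's collected rune count in a BP_SaveGame slot and applies it to the character's currency component.
; BeginPlay loads or creates the save, but clears the character's BPCCurrency reference just before writing Currency to it.
; UpdateRuneCounter increments the cached count and LoadGame copies it to the character.
; SaveGame ignores RunesCollected and writes zero to the slot, while InitialiseSaveGame discards the object it creates.
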(event EventBeginPlay
  (bind _savename (Variables|Default|GetSaveName))
  (bind _returnvalue (SaveGame|DoesSaveGameExist _savename))
  (if _returnvalue
    (bind _returnvalue_2 (SaveGame|LoadGamefromSlot _savename))
    (bind _asbp_save_game (Utilities|Casting|CastToBP_SaveGame _returnvalue_2))
    (bind _output_get (Variables|Default|SetCurrentSaveGame _asbp_save_game))
    (bind _asbp_third_person_character (Utilities|Casting|CastToBP_ThirdPersonCharacter (Game|GetPlayerCharacter 0)))
    (bind _output_get_2 (Variables|/Game/Blueprints/Player/BP_ThirdPersonCharacter.BP_ThirdPersonCharacter_C|SetBPC_Currency _asbp_third_person_character 0))
    (Variables|/Game/Blueprints/Player/Components/BPC_Currency.BPC_Currency_C|Setcurrency _output_get_2 (Variables|/Game/Blueprints/Player/SaveData/BP_SaveGame.BP_SaveGame_C|GetPlayerRunesColleted _output_get))
    (Development|PrintString "Manager Started again")
    (else
      (bind _returnvalue_3 (SaveGame|CreateSaveGameObject "/Game/Blueprints/Player/SaveData/BP_SaveGame.BP_SaveGame_C"))
      (Variables|/Game/Blueprints/Player/SaveData/BP_SaveGame.BP_SaveGame_C|SetPlayerRunesColleted _returnvalue_3 0)
      (SaveGame|SaveGametoSlot _returnvalue_3 (Variables|Default|GetSaveName))
      (Variables|Default|SetCurrentSaveGame _returnvalue_3))))

(fn SaveGame
  (params (RunesCollected :type Integer))
  (bind _currentsavegame (Variables|Default|GetCurrentSaveGame))
  (bind _returnvalue (SaveGame|DoesSaveGameExist (Variables|Default|GetSaveName)))
  (if _returnvalue
    (Variables|/Game/Blueprints/Player/SaveData/BP_SaveGame.BP_SaveGame_C|SetPlayerRunesColleted _currentsavegame 0)
    (SaveGame|SaveGametoSlot _currentsavegame (Variables|Default|GetSaveName))
    (Development|PrintString "Currency/Runes Saved")))

(fn LoadGame
  (bind _returnvalue (SaveGame|DoesSaveGameExist (Variables|Default|GetSaveName)))
  (if _returnvalue
    (bind _asbp_third_person_character (Utilities|Casting|CastToBP_ThirdPersonCharacter (Game|GetPlayerCharacter 0)))
    (Variables|/Game/Blueprints/Player/Components/BPC_Currency.BPC_Currency_C|Setcurrency (Variables|/Game/Blueprints/Player/BP_ThirdPersonCharacter.BP_ThirdPersonCharacter_C|GetBPC_Currency _asbp_third_person_character) (Variables|/Game/Blueprints/Player/SaveData/BP_SaveGame.BP_SaveGame_C|GetPlayerRunesColleted (Variables|Default|GetCurrentSaveGame)))))

(fn InitialiseSaveGame
  (SaveGame|CreateSaveGameObject "/Game/Blueprints/Player/SaveData/BP_SaveGame.BP_SaveGame_C"))

(fn UpdateRuneCounter
  (params (RunesToAdd :type Integer))
  (bind _currentsavegame (Variables|Default|GetCurrentSaveGame))
  (Variables|/Game/Blueprints/Player/SaveData/BP_SaveGame.BP_SaveGame_C|SetPlayerRunesColleted _currentsavegame (+ (Variables|/Game/Blueprints/Player/SaveData/BP_SaveGame.BP_SaveGame_C|GetPlayerRunesColleted _currentsavegame) RunesToAdd)))