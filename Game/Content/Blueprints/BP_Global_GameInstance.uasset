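; Global GameInstance that holds persistent game state: a game timer, hat and level data, the snowman model choice and master volume.
; Init starts a looping one-second timer, and save, load and overwrite events move time, hat and level data through named BP_SaveGame slots.
; Level open and close events play cached ice or fade transition widgets, guarded by a shared transitioning flag.
; UpdateMasterVolume applies volume via sound mix and audio bus.
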(event Custom|CloseLevelUIFade
  ;[0.194 0.1502 0.7931 1 42] LEVEL TRANSITION: DEFAULT CLOSE
  (if (not (Variables|Default|GetTransitioningScene))
    (Variables|Default|SetTransitioningScene true)
    (Utilities|IsValid (Variables|Default|GetFadeTransition)
      (:Is%20Valid
        (Widget|SetVisibility (Variables|Default|GetFadeTransition) "Visible"))
      (:Is%20Not%20Valid
        (bind _returnvalue (UserInterface|CreateWidget "/Game/UI/Transitions/WB_FadeTransition.WB_FadeTransition_C" (Game|GetPlayerController 0)))
        (Variables|Default|SetFadeTransition _returnvalue)))
    (UserInterface|Viewport|AddtoViewport (Variables|Default|GetFadeTransition) 11)
    (Default|InTransition (Variables|Default|GetFadeTransition))
    (Utilities|FlowControl|Delay (Class|WidgetAnimation|GetEndTime (Variables|/Game/UI/Transitions/WB_FadeTransition.WB_FadeTransition_C|GetFadeIn (Variables|Default|GetFadeTransition))))
    (Variables|Default|SetTransitioningScene false)))

(event Custom|SaveGame
  (params (SaveGameName :type String))
  ;[1 1 1] Save Function Call
  (Variables|Default|SetsaveName SaveGameName)
  (bind _returnvalue (SaveGame|DoesSaveGameExist SaveGameName))
  (if _returnvalue
    (Utilities|Casting|CastToBP_ThirdPersonCharacter (Game|GetPlayerCharacter 0))
    (else
      (bind _returnvalue_2 (SaveGame|CreateSaveGameObject "/Game/Blueprints/Player/SaveData/BP_SaveGame.BP_SaveGame_C"))
      (Variables|Default|SetAs%20BP%20Save%20Game _returnvalue_2)))
  (Variables|/Game/Blueprints/Player/SaveData/BP_SaveGame.BP_SaveGame_C|SetSaveSlotDisplayName (Variables|Default|GetAs%20BP%20Save%20Game) (Variables|Default|GetUserSaveNameID))
  (Variables|/Game/Blueprints/Player/SaveData/BP_SaveGame.BP_SaveGame_C|SetSGS_GameTime (Variables|Default|GetAs%20BP%20Save%20Game) (Variables|Default|GetGame%20Time))
  (Variables|/Game/Blueprints/Player/SaveData/BP_SaveGame.BP_SaveGame_C|SethatsData (Variables|Default|GetAs%20BP%20Save%20Game) (Variables|Default|GethatData))
  (Variables|/Game/Blueprints/Player/SaveData/BP_SaveGame.BP_SaveGame_C|SetlevelData (Variables|Default|GetAs%20BP%20Save%20Game) (Variables|Default|GetlevelData))
  (SaveGame|SaveGametoSlot (Variables|Default|GetAs%20BP%20Save%20Game) SaveGameName))

(event Custom|LoadGame
  (params (SaveGameName :type String))
  ;[1 1 1] Load Function Call
  (Variables|Default|SetsaveName SaveGameName)
  (bind _returnvalue (SaveGame|DoesSaveGameExist SaveGameName))
  (if _returnvalue
    (bind _returnvalue_2 (SaveGame|LoadGamefromSlot SaveGameName))
    (bind _asbp_save_game (Utilities|Casting|CastToBP_SaveGame _returnvalue_2))
    (Variables|Default|SetAs%20BP%20Save%20Game _asbp_save_game)
    (Variables|Default|SetGame%20Time (Variables|/Game/Blueprints/Player/SaveData/BP_SaveGame.BP_SaveGame_C|GetSGS_GameTime _asbp_save_game))
    (Variables|Default|SethatData (Variables|/Game/Blueprints/Player/SaveData/BP_SaveGame.BP_SaveGame_C|GethatsData _asbp_save_game))
    (Variables|Default|SetlevelData (Variables|/Game/Blueprints/Player/SaveData/BP_SaveGame.BP_SaveGame_C|GetlevelData _asbp_save_game))))

(event Custom|AddGameTime
  ;[1 1 1] Game Timer
  (Math|Integer|IncrementInt (Variables|Default|GetGame%20Time)))

(event Custom|SavePlayerModel
  (params (IsSnowman :type Boolean) (Hat :type Static%20Mesh%20Object%20Reference))
  ;[1 0.252 0.2288] Snowman Hat Continuity - Still in use??
  (Variables|Default|SetIsSnowman IsSnowman)
  (Variables|Default|SetHat Hat))

(event Custom|OpenLevelUIFade
  ;[0.4851 0.1898 1 1 42] LEVEL TRANSITION: DEFAULT OPEN
  (if (not (Variables|Default|GetTransitioningScene))
    (Variables|Default|SetTransitioningScene true)
    (Utilities|IsValid (Variables|Default|GetFadeTransition)
      (:Is%20Valid
        _)
      (:Is%20Not%20Valid
        (bind _returnvalue (UserInterface|CreateWidget "/Game/UI/Transitions/WB_FadeTransition.WB_FadeTransition_C" (Game|GetPlayerController 0)))
        (Variables|Default|SetFadeTransition _returnvalue)))
    (UserInterface|Viewport|AddtoViewport (Variables|Default|GetFadeTransition) 11)
    (Default|OutTransition (Variables|Default|GetFadeTransition))
    (Utilities|FlowControl|Delay (Class|WidgetAnimation|GetEndTime (Variables|/Game/UI/Transitions/WB_FadeTransition.WB_FadeTransition_C|GetFadeIn (Variables|Default|GetFadeTransition))))
    (Widget|SetVisibility (Variables|Default|GetFadeTransition) "Hidden")
    (Variables|Default|SetTransitioningScene false)))

(event Custom|CloseLevelUI
  ;[0.2738 1 0 1 42] LEVEL TRANSITION: ICE CLOSE
  (if (not (Variables|Default|GetTransitioningScene))
    (Variables|Default|SetTransitioningScene true)
    (Utilities|IsValid (Variables|Default|GetDefaultTransition)
      (:Is%20Valid
        (Widget|SetVisibility (Variables|Default|GetDefaultTransition) "Visible"))
      (:Is%20Not%20Valid
        (bind _returnvalue (UserInterface|CreateWidget "/Game/UI/Transitions/WB_IceTransition.WB_IceTransition_C" (Game|GetPlayerController 0)))
        (Variables|Default|SetDefaultTransition _returnvalue)))
    (UserInterface|Viewport|AddtoViewport (Variables|Default|GetDefaultTransition) 11)
    (Default|InTransition (Variables|Default|GetDefaultTransition))
    (Utilities|FlowControl|Delay (Class|WidgetAnimation|GetEndTime (Variables|/Game/UI/Transitions/WB_IceTransition.WB_IceTransition_C|GetSlideIn (Variables|Default|GetDefaultTransition))))
    (Variables|Default|SetTransitioningScene false)))

(event Custom|OpenLevelUI
  ;[0.1455 1 0.003805 1 42] LEVEL TRANSITION: ICE OPEN
  (if (not (Variables|Default|GetTransitioningScene))
    (Variables|Default|SetTransitioningScene true)
    (Utilities|IsValid (Variables|Default|GetDefaultTransition)
      (:Is%20Valid
        _)
      (:Is%20Not%20Valid
        (bind _returnvalue (UserInterface|CreateWidget "/Game/UI/Transitions/WB_IceTransition.WB_IceTransition_C" (Game|GetPlayerController 0)))
        (Variables|Default|SetDefaultTransition _returnvalue)))
    (UserInterface|Viewport|AddtoViewport (Variables|Default|GetDefaultTransition) 11)
    (Utilities|FlowControl|Delay 0.3)
    (Default|OutTransition (Variables|Default|GetDefaultTransition))
    (Utilities|FlowControl|Delay (Class|WidgetAnimation|GetEndTime (Variables|/Game/UI/Transitions/WB_IceTransition.WB_IceTransition_C|GetSlideIn (Variables|Default|GetDefaultTransition))))
    (Widget|SetVisibility (Variables|Default|GetDefaultTransition) "Hidden")
    (Variables|Default|SetTransitioningScene false)))

(event Custom|overwriteSave
  (params (Save%20Game%20Name :type String))
  (Variables|Default|SetsaveName Save%20Game%20Name)
  (SaveGame|DeleteGameinSlot Save%20Game%20Name)
  (bind _returnvalue (SaveGame|CreateSaveGameObject "/Game/Blueprints/Player/SaveData/BP_SaveGame.BP_SaveGame_C"))
  (bind _output_get (Variables|Default|SetAs%20BP%20Save%20Game _returnvalue))
  (Variables|/Game/Blueprints/Player/SaveData/BP_SaveGame.BP_SaveGame_C|SetSaveSlotDisplayName _output_get (Variables|Default|GetUserSaveNameID))
  (SaveGame|SaveGametoSlot _output_get Save%20Game%20Name))

(event Custom|Start%20Game%20Timer
  ;[1 1 1] Game Timer
  (Utilities|Time|SetTimerbyEvent (delegate Custom|AddGameTime) 1.0 true))

(event EventInit
  ;[0 1 0.3523] Game Instance Init
  (CallFunction|StartGameTimer))

(fn GetPlayerMesh
  (return 0 0 (Variables|Default|GetIsSnowman)))

(fn UpdateMasterVolume
  (params (NewVolume :type Float%20%28double-precision%29))
  ;[1 1 1] Master Volume Adjustment System (Was in Slider UI)
  (bind _output_get (Variables|Default|SetSavedMasterVolume NewVolume))
  (Audio|SetSoundMixClassOverride "/Game/MasterVolume.MasterVolume" "/Engine/EngineSounds/Master.Master" _output_get 1.0 1.0 true)
  (Class|FMODBlueprintStatics|BusSetVolume "/Game/FMOD/Buses/Master.Master" _output_get)
  (Audio|PushSoundMixModifier "/Game/MasterVolume.MasterVolume"))