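; Patrol path actor that moves a list of actors along a spline, spaced by a fixed offset, looping or ping-ponging.
; The construction script pre-positions the actors, and BeginPlay scales the timeline rate to the path duration, with Tick counting down any start delay.
; Timeline updates set each actor's spline distance, wrapping past the end, with optional rotation control.
; On finish it replays, pausing and reversing when ping-pong is enabled.
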(event Custom|PlayTimeline
  (params (PlayBackwards :type Boolean))
  (bind _spline (Variables|Default|GetSpline))
  (bind _spline_2 (Variables|Default|GetSpline))
  (bind _returnvalue (Spline|GetSplineLength _spline))
  (Variables|Default|SetPlayingBackwards PlayBackwards)
  ;[1 1 1] If 'Ping Pong' true, play backwards if wanted - otherwise just forwards
  (if (Variables|Default|GetPingPong)
    (if PlayBackwards
      (bind _alpha (Timeline|Timeline ReverseFromEnd)
        (:Update
          (for (_array_element _array_index) (Variables|Default|GetActors)
            (bind _output_get (Variables|Default|SetDistance%20along%20spline (+ (Math|Float|Lerp 0.0 (Spline|GetSplineLength (Variables|Default|GetSpline)) _alpha) (* _array_index (Variables|Default|GetOffset%20Between%20actors)))))
            (if (> _output_get _returnvalue)
              (Variables|Default|SetDistance%20along%20spline (- (Variables|Default|GetDistance%20along%20spline) _returnvalue)))
            (if (Variables|Default|GetControl%20Actor%20Rotation)
              (Transformation|SetActorLocationAndRotation _array_element (Spline|GetLocationatDistanceAlongSpline _spline_2 (Variables|Default|GetDistance%20along%20spline) "World") (Spline|GetRotationatDistanceAlongSpline _spline_2 (Variables|Default|GetDistance%20along%20spline) "World"))
              (else
                (Transformation|SetActorLocation _array_element (Spline|GetLocationatDistanceAlongSpline _spline_2 (Variables|Default|GetDistance%20along%20spline) "World") false false)))))
        (:Finished
          ;[1 1 1] If 'Ping Pong' true, wait for Ping Pong delay before playing again - otherwise straight away
          (if (Variables|Default|GetPingPong)
            (Utilities|FlowControl|Delay (Variables|Default|GetPingPongDelay)))
          (CallFunction|PlayTimeline (not PlayBackwards))))
      (else
        (Timeline|Timeline PlayFromStart)))
    (else
      (Timeline|Timeline PlayFromStart))))

(event EventBeginPlay
  (Components|Timeline|SetPlayRate (Variables|Default|GetTimeline) (/ 1.0 (Variables|Default|GetTimelineLength)))
  (if (> (Variables|Default|GetTimelineDelay) 0.0)
    (Variables|Default|SetPreventTimeline true)
    (Variables|Default|SetTimeToPrevent (Variables|Default|GetTimelineDelay))
    (else
      (CallFunction|PlayTimeline false))))

(event EventTick
  (params (DeltaSeconds :type Float%20%28single-precision%29))
  (if (Variables|Default|GetPreventTimeline)
    (if (> (Variables|Default|GetTimeToPrevent) 0.0)
      (bind _output_get (Variables|Default|SetTimeToPrevent (- (Variables|Default|GetTimeToPrevent) DeltaSeconds)))
      (if (<= _output_get 0.0)
        (Variables|Default|SetPreventTimeline (<= _output_get 0.0))
        (CallFunction|PlayTimeline false)))))

(fn ConstructionScript
  (bind _spline (Variables|Default|GetSpline))
  (for (_array_element _array_index) (Variables|Default|GetActors)
    (if (Variables|Default|GetControl%20Actor%20Rotation)
      (Transformation|SetActorLocationAndRotation _array_element (Spline|GetLocationatDistanceAlongSpline _spline (* (Variables|Default|GetOffset%20Between%20actors) _array_index) "World") (Spline|GetRotationatDistanceAlongSpline _spline (* (Variables|Default|GetOffset%20Between%20actors) _array_index) "World"))
      (else
        (Transformation|SetActorLocation _array_element (Spline|GetLocationatDistanceAlongSpline _spline (* (Variables|Default|GetOffset%20Between%20actors) _array_index) "World") false false)))))