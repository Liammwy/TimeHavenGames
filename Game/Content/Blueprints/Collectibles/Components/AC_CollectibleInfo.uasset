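; Collectible component that picks a mesh and runs pickup logic by CollectibleType: currency, broken key, time machine or jetpack refill.
; SetMesh reads data tables, choosing a random rune for currency.
; GetCorrectCollection dispatches: currency adds money, updates the popup and increments the GameInstance rune count for the name-matched level, while refill resets hover time.
; Non-refill pickups play a rising-pitch sound; key and time machine handlers are empty.
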(event EventBeginPlay
  (bind _returnvalue (Game|GetCurrentLevelName true))
  (switch string _returnvalue
    (:Tutorial
      (Variables|Default|SetlevelNames "NewEnumerator8"))
    (:FireBreathLevel
      (Variables|Default|SetlevelNames "NewEnumerator0"))
    (:SuperJumpLevel
      (Variables|Default|SetlevelNames "NewEnumerator1"))
    (:TimeSlowLevel
      (Variables|Default|SetlevelNames "NewEnumerator7"))))

(fn SetMesh
  (params (staticMesh :type Static%20Mesh%20Component%20Object%20Reference))
  (bind _collectibletype (Variables|Default|GetcollectibleType))
  (bind _returnvalue (Utilities|String|EnumtoString _collectibletype))
  (bind _returnvalue_2 (Utilities|String|StringToName _returnvalue))
  (if (== _returnvalue_2 "currency")
    (bind _outrownames (DataTable|GetDataTableRowNames "/Game/Data/Collectibles/DT_Runes.DT_Runes"))
    (bind _returnvalue_3 (Utilities|GetDataTableRow "/Game/Data/Collectibles/DT_Runes.DT_Runes" (.OutItem (Utilities|Array|Random _outrownames)))
      (:then
        (Components|StaticMesh|SetStaticMesh staticMesh (.runematerial _returnvalue_3))
        (Variables|Default|SetindxVal (.runeidx _returnvalue_3))))
    (else
      (bind _returnvalue_4 (Utilities|GetDataTableRow "/Game/Data/Collectibles/DT_CollectibleType.DT_CollectibleType" _returnvalue_2)
        (:then
          (Components|StaticMesh|SetStaticMesh staticMesh (.collectiblemesh _returnvalue_4)))))))

(fn CurrencyCollection
  (params (hitActor :type Object%20Object%20Reference))
  ;[1 1 1 1 30] Adding money to player when collecting the currency collectible
  (bind _asbp_third_person_character (Utilities|Casting|CastToBP_ThirdPersonCharacter hitActor))
  (Default|AddMoney (Actor|GetComponentbyClass _asbp_third_person_character "/Game/Blueprints/Player/Components/BPC_Currency.BPC_Currency_C"))
  (Variables|/Game/Blueprints/UI/WBP_Runes.WBP_Runes_C|SetnumOfCollectiblesInQueue (Variables|/Game/Blueprints/Player/BP_ThirdPersonCharacter.BP_ThirdPersonCharacter_C|GetpopupUI _asbp_third_person_character) (+ (Variables|/Game/Blueprints/UI/WBP_Runes.WBP_Runes_C|GetnumOfCollectiblesInQueue (Variables|/Game/Blueprints/Player/BP_ThirdPersonCharacter.BP_ThirdPersonCharacter_C|GetpopupUI _asbp_third_person_character)) 1))
  (Variables|/Game/Blueprints/UI/WBP_Runes.WBP_Runes_C|SetindxNum (Variables|/Game/Blueprints/Player/BP_ThirdPersonCharacter.BP_ThirdPersonCharacter_C|GetpopupUI _asbp_third_person_character) (Variables|Default|GetindxVal))
  (Game|GetCurrentLevelName true)
  (bind _asbp_global_game_instance (Utilities|Casting|CastToBP_Global_GameInstance (Game|GetGameInstance)))
  (for (_array_element _array_index) (Variables|/Game/Blueprints/BP_Global_GameInstance.BP_Global_GameInstance_C|GetlevelData _asbp_global_game_instance)
    (if (Utilities|Enum|Equal(Enum) (Variables|Default|GetlevelNames) (.level (Utilities|Struct|Breaks_levels _array_element)))
      (Utilities|Array|SetArrayElem (Variables|/Game/Blueprints/BP_Global_GameInstance.BP_Global_GameInstance_C|GetlevelData _asbp_global_game_instance) _array_index (Utilities|Struct|Makes_levels (.level (Utilities|Struct|Breaks_levels _array_element)) (+ (.runecount (Utilities|Struct|Breaks_levels _array_element)) 1) (.hatCount (Utilities|Struct|Breaks_levels _array_element)) (.isComplete (Utilities|Struct|Breaks_levels _array_element)) (.isCurrentLevel (Utilities|Struct|Breaks_levels _array_element)) (.isAccessible (Utilities|Struct|Breaks_levels _array_element)) (.cutsceneHasPlayed (Utilities|Struct|Breaks_levels _array_element)) (.maximumRuneCount (Utilities|Struct|Breaks_levels _array_element)) (.maximumHatCount (Utilities|Struct|Breaks_levels _array_element)) (.runeHighScore (Utilities|Struct|Breaks_levels _array_element)))))))

(fn BrokenKeyCollection
  (params (hitActor :type Object%20Object%20Reference)))

(fn TimeMachineCollection
  (params (hitActor :type Object%20Object%20Reference)))

(fn GetCorrectCollection
  (params (hitActor :type Object%20Object%20Reference))
  ;[1 1 1 1 30] Getting the collection type of the collectible, meaning different functions can run depending on what collectible they've hit
  (bind _output_get (Variables|Default|SetCollectible hitActor))
  (LocalVariables|SetactorHit _output_get)
  (switch Utilities|FlowControl|Switch|SwitchonENUM_CollectibleTypes (Variables|Default|GetcollectibleType)
    (:NewEnumerator0
      (CallFunction|CurrencyCollection (LocalVariables|GetactorHit))
      (bind _returnvalue (Class|FMODBlueprintStatics|PlayEvent2D "/Game/FMOD/Events/ItemPickup.ItemPickup" :!label _label))
      (bind _asbp_third_person_character (Utilities|Casting|CastToBP_ThirdPersonCharacter (Game|GetPlayerCharacter 0)))
      (Class|FMODBlueprintStatics|EventInstanceSetPitch _returnvalue (Variables|/Game/Blueprints/Player/BP_ThirdPersonCharacter.BP_ThirdPersonCharacter_C|GetCollectPitchModify _asbp_third_person_character))
      (Default|IncreasePitchModify _asbp_third_person_character)
      (Default|PitchUpTimer _asbp_third_person_character))
    (:NewEnumerator1
      (CallFunction|BrokenKeyCollection (LocalVariables|GetactorHit))
      (goto _label))
    (:NewEnumerator2
      (CallFunction|TimeMachineCollection (LocalVariables|GetactorHit))
      (goto _label))
    (:NewEnumerator3
      (CallFunction|RefillJetpackCollection (LocalVariables|GetactorHit))))
  (return true))

(fn RefillJetpackCollection
  (params (HitActor :type Object%20Object%20Reference))
  (Utilities|Casting|CastToBP_Refule HitActor)
  (bind _asbp_third_person_character (Utilities|Casting|CastToBP_ThirdPersonCharacter (Game|GetPlayerCharacter 0)))
  (Default|ResetHoverTime (Actor|GetComponentbyClass _asbp_third_person_character "/Game/Blueprints/Player/Components/BPC_Hover.BPC_Hover_C"))
  (Development|PrintString "Refilled "))