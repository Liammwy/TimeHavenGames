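; Decorative red mushroom actor for level dressing, built from Cap and Stem components with no active runtime logic.
; Its construction script can randomise actor scale independently per axis, then vary cap and stem width while keeping their relative Z scale.
; A separate toggle gives cap and stem independent random yaw.
; The random values are unseeded, so they re-roll whenever the construction script reruns.
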(event EventBeginPlay)

(event Collision|EventActorBeginOverlap
  (params (OtherActor :type Actor%20Object%20Reference)))

(event EventTick
  (params (DeltaSeconds :type Float%20%28single-precision%29)))

(fn ConstructionScript
  (bind _returnvalue (Math|Random|RandomFloatinRange 0.0 3.6e+02))
  (bind _minrandomsize_stem (Variables|Default|GetMinRandomSize_Stem))
  (bind _maxrandomsize_stem (Variables|Default|GetMaxRandomSize_Stem))
  (bind _minrandomsize (Variables|Default|GetMinRandomSize))
  (bind _maxrandomsize (Variables|Default|GetMaxRandomSize))
  (bind _cap (Variables|Default|GetCap))
  (bind _stem (Variables|Default|GetStem))
  (bind _minrandomsize_cap (Variables|Default|GetMinRandomSize_Cap))
  (bind _maxrandomsize_cap (Variables|Default|GetMaxRandomSize_Cap))
  (bind _returnvalue_2 (Math|Random|RandomFloatinRange _minrandomsize_cap _maxrandomsize_cap))
  (bind _returnvalue_3 (Math|Random|RandomFloatinRange _minrandomsize_stem _maxrandomsize_stem))
  (bind _returnvalue_4 (Math|Random|RandomFloatinRange _minrandomsize _maxrandomsize))
  ;[1 1 1] Randomise mushroom scale if  Randomise Scale is true
  (if (Variables|Default|GetRandomiseScale)
    ;;[1 0.2446 0.06435] overall actor scale
    (Transformation|SetActorScale3D (Math|Vector|MakeVector _returnvalue_4 _returnvalue_4 _returnvalue_4))
    ;;[1 0.1579 0.06819] cap size
    (Transformation|SetRelativeScale3D _cap (Math|Vector|MakeVector _returnvalue_2 _returnvalue_2 (.z (Variables|/Script/Engine.SceneComponent|GetRelativeScale3D _cap))))
    ;;[1 0.8122 0.2487] stem size
    (Transformation|SetRelativeScale3D _stem (Math|Vector|MakeVector _returnvalue_3 _returnvalue_3 (.z (Variables|/Script/Engine.SceneComponent|GetRelativeScale3D _stem)))))
  ;[1 1 1] Set random rotation if Randomise Rotation true
  (if (Variables|Default|GetRandomise%20Rotation)
    (Transformation|SetRelativeRotation (Variables|Default|GetCap) (Math|Rotator|MakeRotator 0.0 0.0 _returnvalue) false false)
    (Transformation|SetRelativeRotation (Variables|Default|GetStem) (Math|Rotator|MakeRotator 0.0 0.0 _returnvalue) false false)))