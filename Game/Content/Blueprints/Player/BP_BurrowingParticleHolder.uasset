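; BP_BurrowingParticleHolder is an actor that follows the player character, apparently to show an effect while burrowing.
; Every Tick it looks up BP_ThirdPersonCharacter with GetActorOfClass and moves itself to that location without sweeping.
; Its Sphere component starts hidden in the construction script, and ToggleEmitting flips the Emitting flag and the Sphere's visibility together.
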(event EventTick
  (params (DeltaSeconds :type Float%20%28single-precision%29))
  (bind _returnvalue (Actor|GetActorOfClass "/Game/Blueprints/Player/BP_ThirdPersonCharacter.BP_ThirdPersonCharacter_C"))
  (Transformation|SetActorLocation (Transformation|GetActorLocation _returnvalue) false false))

(fn ConstructionScript
  (Rendering|SetVisibility (Variables|Default|GetSphere) false false))

(fn ToggleEmitting
  (bind _sphere (Variables|Default|GetSphere))
  (if (Variables|Default|GetEmitting)
    (Variables|Default|SetEmitting false)
    (Rendering|SetVisibility _sphere false false)
    (else
      (Variables|Default|SetEmitting true)
      (Rendering|SetVisibility _sphere true false))))