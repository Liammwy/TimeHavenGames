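; Player component that shows a drop shadow decal beneath player character 0 while it is off the ground.
; BeginPlay spawns the decal at the hit point of a downward trace from the character.
; Tick repeats the trace, moving the decal to the impact point and shrinking its Y and Z scale as distance grows.
; At short trace distances, it hides the decal by moving it to a fixed world position below the origin.
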(event EventBeginPlay
  (bind _returnvalue (Game|GetPlayerCharacter 0))
  (bind _returnvalue_2 (Transformation|GetActorLocation _returnvalue))
  (bind _outhit (Collision|LineTraceByChannel _returnvalue_2 (- _returnvalue_2 "0.000000,0.000000,1000.000000") "TraceTypeQuery1" false 0 "ForOneFrame"))
  (bind _returnvalue_3 (Rendering|Decal|SpawnDecalatLocation "/Game/Materials/Player/M_DropShadow.M_DropShadow" "20.000000,25.000000,25.000000" (.impactpoint _outhit) "-90.000000,0.000000,0.000000" 0.0))
  (Variables|Default|SetShadow _returnvalue_3))

(event EventTick
  (params (DeltaSeconds :type Float%20%28single-precision%29))
  (bind _returnvalue (Game|GetPlayerCharacter 0))
  (bind _returnvalue_2 (Transformation|GetActorLocation _returnvalue))
  (bind _outhit (Collision|LineTraceByChannel _returnvalue_2 (- _returnvalue_2 "0.000000,0.000000,1000.000000") "TraceTypeQuery1" false 0 "None"))
  (if (< (.distance _outhit) 75.0)
    (Transformation|SetWorldLocation (Variables|Default|GetShadow) "0.000000,0.000000,-100.000000" false false)
    (else
      (Transformation|SetWorldLocation (Variables|Default|GetShadow) (.impactpoint _outhit) false false)
      (bind _newscale (CallFunction|NewRelativeScale (.distance _outhit)))
      (Transformation|SetWorldScale3D (Variables|Default|GetShadow) _newscale))))

(fn NewRelativeScale
  (params (distanceFromGround :type Float%20%28double-precision%29))
  (bind _returnvalue (/ distanceFromGround 1e+03))
  (bind _defaultscale (LocalVariables|GetdefaultScale))
  (bind _returnvalue_2 (- 1.4 _returnvalue))
  (bind _returnvalue_3 (* _defaultscale _returnvalue_2))
  (return (Math|Vector|MakeVector 1.0 (.y _returnvalue_3) (.z _returnvalue_3))))