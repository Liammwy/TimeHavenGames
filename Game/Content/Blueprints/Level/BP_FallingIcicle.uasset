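; Falling icicle hazard that drops when the player enters its detection field, or after a countdown in constant-fall mode.
; Tick moves it down until it hits a non-ignored actor, force-respawning the player if struck.
; Impact hides it and releases eight physics fragments that shrink away, then a delay restores it at its cached pre-fall location.
; A separate overlap volume toggles particles around the player character's presence.
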(event OnComponentBeginOverlap(DetectionField)
  (params (OverlappedComponent :type Primitive%20Component%20Object%20Reference) (OtherActor :type Actor%20Object%20Reference) (OtherComp :type Primitive%20Component%20Object%20Reference) (OtherBodyIndex :type Integer) (bFromSweep :type Boolean) (SweepResult :type Hit%20Result%20Structure%20%28by%20ref%29))
  ;[1 1 1] If player enters detection field under icicle, trigger fall
  (if (not (Variables|Default|GetisFalling))
    (if (== OtherActor (Variables|Default|GetPlayerRef))
      (if (not (Variables|Default|GetconstantFall))
        (CallFunction|TriggerFall)))))

(event OnComponentBeginOverlap(IcicleImpactField)
  (params (OverlappedComponent :type Primitive%20Component%20Object%20Reference) (OtherActor :type Actor%20Object%20Reference) (OtherComp :type Primitive%20Component%20Object%20Reference) (OtherBodyIndex :type Integer) (bFromSweep :type Boolean) (SweepResult :type Hit%20Result%20Structure%20%28by%20ref%29))
  ;[1 1 1] If object hits icicle underside, destroy icicle. Kill player if they were hit.
  (if (not (Utilities|Array|ContainsItem (Variables|Default|GetIgnoreClasses) (Utilities|GetClass OtherActor)))
    (if (Variables|Default|GetisActive)
      (if (Variables|Default|GetisFalling)
        (if (== (Variables|Default|GetPlayerRef) OtherActor)
          (Default|ForceRespawn (Variables|Default|GetPlayerRef)))
        (CallFunction|DestroyIcicleEvent) ; MUST BE AT END because event has delay for respawn
      ))))

(event OnComponentBeginOverlap(particleCollision)
  (params (OverlappedComponent :type Primitive%20Component%20Object%20Reference) (OtherActor :type Actor%20Object%20Reference) (OtherComp :type Primitive%20Component%20Object%20Reference) (OtherBodyIndex :type Integer) (bFromSweep :type Boolean) (SweepResult :type Hit%20Result%20Structure%20%28by%20ref%29))
  (Utilities|Casting|CastToBP_ThirdPersonCharacter OtherActor)
  (Components|Activation|SetActive (Variables|Default|GetParticleSystem) true false))

(event OnComponentEndOverlap(particleCollision)
  (params (OverlappedComponent :type Primitive%20Component%20Object%20Reference) (OtherActor :type Actor%20Object%20Reference) (OtherComp :type Primitive%20Component%20Object%20Reference) (OtherBodyIndex :type Integer))
  (Components|Activation|SetActive (Variables|Default|GetParticleSystem) false true))

(event Custom|DestroyIcicleEvent
  ;[1 1 1] Turn off visuals/colliders, delay and trigger respawn
  (Class|FMODBlueprintStatics|PlayEventatLocation "/Game/FMOD/Events/Icicle_Land.Icicle_Land" (Math|Conversions|ToTransform(Vector) (Transformation|GetActorLocation)))
  (Variables|Default|SetisActive false)
  (Rendering|SetVisibility (Variables|Default|GetIcicleRoot) false false)
  (Collision|SetCollisionEnabled (Variables|Default|GetIcicleRoot) "NoCollision")
  (Collision|SetCollisionEnabled (Variables|Default|GetIcicleImpactField) "NoCollision")
  (Collision|SetCollisionEnabled (Variables|Default|GetPlatform) "NoCollision")
  (Rendering|SetVisibility (Variables|Default|GetVisuals) false false)
  (for _array_element (Variables|Components|GetFragments)
    (Physics|SetEnableGravity _array_element true)
    (Physics|SetSimulatePhysics _array_element true)
    (Variables|Default|SetisBroken true)
    (Variables|Default|SettimeSinceBroken 0.0)
    (Utilities|FlowControl|Delay (Variables|Default|GettimeUntilRespawn))
    (CallFunction|RespawnIcicle)))

(event EventBeginPlay
  ;[1 1 1] Assign player reference on play
  (bind _outactors (Actor|GetAllActorsOfClass "/Game/Blueprints/Player/BP_ThirdPersonCharacter.BP_ThirdPersonCharacter_C"))
  (Variables|Default|SetPlayerRef (Utilities|Array|Get(acopy) _outactors))
  (Variables|Default|SetcurrentFallDelay (Variables|Default|GetconstantFallDelay))
  (Utilities|Array|Add (Variables|Components|GetFragments) (Variables|Default|GetFragment_1))
  (Utilities|Array|Add (Variables|Components|GetFragments) (Variables|Default|GetFragment_2))
  (Utilities|Array|Add (Variables|Components|GetFragments) (Variables|Default|GetFragment_3))
  (Utilities|Array|Add (Variables|Components|GetFragments) (Variables|Default|GetFragment_4))
  (Utilities|Array|Add (Variables|Components|GetFragments) (Variables|Default|GetFragment_5))
  (Utilities|Array|Add (Variables|Components|GetFragments) (Variables|Default|GetFragment_6))
  (Utilities|Array|Add (Variables|Components|GetFragments) (Variables|Default|GetFragment_7))
  (Utilities|Array|Add (Variables|Components|GetFragments) (Variables|Default|GetFragment_8))
  (for _array_element (Variables|Components|GetFragments)
    (Utilities|Array|Add (Variables|Default|GetFragmentStartPositions) (Transformation|GetRelativeTransform _array_element))))

(event EventTick
  (params (DeltaSeconds :type Float%20%28single-precision%29))
  (CallFunction|UpdateBrokenFragments DeltaSeconds)
  ;[1 1 1] Update falling movement if active and falling
  (if (Variables|Default|GetisActive)
    (if (Variables|Default|GetisFalling)
      (CallFunction|UpdateFalling DeltaSeconds)
      (elif (Variables|Default|GetconstantFall)
        (bind _output_get (Variables|Default|SetcurrentFallDelay (- (Variables|Default|GetcurrentFallDelay) DeltaSeconds)))
        (if (<= _output_get 0.0)
          (CallFunction|TriggerFall))))))

(fn ConstructionScript
  (Variables|Default|SetisActive true))

(fn UpdateFalling
  (params (deltaTime :type Float%20%28double-precision%29))
  (bind _icicleroot (Variables|Default|GetIcicleRoot))
  (bind _returnvalue (Transformation|GetWorldLocation _icicleroot))
  (if (Variables|Default|GetisFalling)
    (Transformation|SetWorldLocation (Variables|Default|GetIcicleRoot) (Math|Vector|MakeVector (.x _returnvalue) (.y _returnvalue) (- (.z _returnvalue) (* deltaTime (Variables|Default|GetfallSpeed)))) false false)))

(fn TriggerFall
  (Variables|Default|SetisFalling true)
  ;[1 1 1] Get cache of location at start of fall - will respawn here
  (bind _output_get (Variables|Default|SetworldLocationCache (Transformation|GetWorldLocation (Variables|Default|GetIcicleRoot))))
  (Class|FMODBlueprintStatics|PlayEventatLocation "/Game/FMOD/Events/Icicle_Break.Icicle_Break" (Math|Conversions|ToTransform(Vector) _output_get)))

(fn RespawnIcicle
  (Variables|Default|SetisFalling false)
  (Variables|Default|SetisActive true)
  (Rendering|SetVisibility (Variables|Default|GetIcicleRoot) true true)
  (Collision|SetCollisionEnabled (Variables|Default|GetIcicleImpactField) "QueryAndPhysics")
  (Collision|SetCollisionEnabled (Variables|Default|GetPlatform) "QueryAndPhysics")
  (Rendering|SetVisibility (Variables|Default|GetVisuals) true false)
  ;[1 1 1] Set location to cached value at time of fall trigger
  (Transformation|SetWorldLocation (Variables|Default|GetIcicleRoot) (Variables|Default|GetworldLocationCache) false true)
  (Variables|Default|SetisBroken false)
  (Variables|Default|SetfragmentsDestroyed false)
  (for (_array_element _array_index) (Variables|Components|GetFragments)
    (Rendering|SetVisibility _array_element true false)
    (Transformation|SetRelativeLocationAndRotation _array_element (.location (Utilities|Array|Get(acopy) (Variables|Default|GetFragmentStartPositions) _array_index)) (.rotation (Utilities|Array|Get(acopy) (Variables|Default|GetFragmentStartPositions) _array_index)) false false)
    (Physics|SetSimulatePhysics _array_element false)))

(fn UpdateBrokenFragments
  (params (deltaTime :type Float%20%28double-precision%29))
  (if (Variables|Default|GetisBroken)
    (if (not (Variables|Default|GetfragmentsDestroyed))
      (bind _output_get (Variables|Default|SettimeSinceBroken (+ (Variables|Default|GettimeSinceBroken) deltaTime)))
      (if (>= _output_get (Variables|Default|GetbrokenFragmentLifetime))
        ;[1 1 1] Deactivate fragments when lifetime ended
        (for _array_element (Variables|Components|GetFragments)
          (Physics|SetSimulatePhysics _array_element false)
          (Rendering|SetVisibility _array_element false false)
          (Collision|SetCollisionEnabled _array_element "NoCollision")
          (Variables|Default|SetfragmentsDestroyed true))
        (else
          ;[1 1 1] Update shrinking mesh visuals
          (for _array_element_2 (Variables|Components|GetFragments)
            (Transformation|SetRelativeScale3D _array_element_2 (Math|Vector|MakeVector (- 1.0 (/ (Variables|Default|GettimeSinceBroken) (Variables|Default|GetbrokenFragmentLifetime))) (- 1.0 (/ (Variables|Default|GettimeSinceBroken) (Variables|Default|GetbrokenFragmentLifetime))) (- 1.0 (/ (Variables|Default|GettimeSinceBroken) (Variables|Default|GetbrokenFragmentLifetime)))))))))))