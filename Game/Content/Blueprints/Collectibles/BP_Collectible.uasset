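; Collectible pickup actor that either bobs and spins in the world or lies buried, collectable only while the player is burrowing.
; ACCollectibleInfo supplies the mesh and handles collection on overlap with the player capsule, hiding mesh and decal on success.
; The construction script traces downward to place the decal on the ground, and GrowIn scales the actor up by timeline.
; Non-buried items re-fetch player references every bobbing-timeline update.
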(event OnComponentBeginOverlap(Box)
  (params (OverlappedComponent :type Primitive%20Component%20Object%20Reference) (OtherActor :type Actor%20Object%20Reference) (OtherComp :type Primitive%20Component%20Object%20Reference) (OtherBodyIndex :type Integer) (bFromSweep :type Boolean) (SweepResult :type Hit%20Result%20Structure%20%28by%20ref%29))
  (if (== OtherComp (Variables|Default|GetplayerCollisionRef))
    (if (Variables|Default|GetBuried)
      (bind _climbing (Default|IsBurrowing? (Variables|Default|GetplayerRef)))
      (if _climbing
        (bind _success (Default|GetCorrectCollection (Variables|Default|GetAC_CollectibleInfo) OtherActor :!label _label))
        (if _success
          (Collision|SetCollisionEnabled (Variables|Default|GetBox) "NoCollision")
          (Rendering|SetVisibility (Variables|Default|GetStaticMesh) false false)))
      (else
        (goto _label)))))

(event Custom|GrowIn
  ;[1 0.09697 0.01729 1 50] GROW COLLECTIBLE FROM NOTHING TO NORMAL SIZE
  (bind _hatscale (Timeline|Timeline PlayFromStart)
    (:Update
      (Transformation|SetRelativeScale3D (Variables|Default|GetDefaultSceneRoot) (Math|Conversions|ToVector(Float) _hatscale)))))

(event EventBeginPlay
  (bind _returnvalue (Transformation|GetActorLocation))
  (bind _returnvalue_2 (Transformation|GetActorRotation))
  (Default|SetMesh (Variables|Default|GetAC_CollectibleInfo) (Variables|Default|GetStaticMesh))
  (if (Variables|Default|GetBuried)
    _
    (else
      (bind (_direction _itembobbing _itemrotating) (Timeline|itemBobbing Play)
        (:Update
          (if (Variables|Default|GetUpdateWithTimelines)
            (Transformation|SetActorLocation (Math|Vector|MakeVector (.x _returnvalue) (.y _returnvalue) (+ (.z _returnvalue) _itembobbing)) false false)
            (Transformation|SetActorRotation (Math|Rotator|MakeRotator (.roll _returnvalue_2) (.pitch _returnvalue_2) (+ (.yaw _returnvalue_2) _itemrotating))))))))
  (bind _returnvalue_3 (Actor|GetActorOfClass "/Game/Blueprints/Player/BP_ThirdPersonCharacter.BP_ThirdPersonCharacter_C"))
  (Variables|Default|SetplayerRef _returnvalue_3)
  (Variables|Default|SetplayerCollisionRef (Variables|/Script/Engine.Character|GetCapsuleComponent _returnvalue_3)))

(fn ConstructionScript
  (bind _defaultsceneroot (Variables|Default|GetDefaultSceneRoot))
  (bind _returnvalue (Transformation|GetWorldLocation _defaultsceneroot))
  (Default|SetMesh (Variables|Default|GetAC_CollectibleInfo) (Variables|Default|GetStaticMesh))
  (bind (_outhit _returnvalue_2) (Collision|LineTraceByChannel _returnvalue (- _returnvalue "0.000000,0.000000,1000.000000") "TraceTypeQuery1" false 0 "None"))
  (if _returnvalue_2
    (Transformation|SetWorldLocation (Variables|Default|GetDecal) (.Location (Collision|BreakHitResult _outhit)) false false)))