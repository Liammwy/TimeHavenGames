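; BPC_GravityFlip is a player component for the Gravity Flip scarf power, currently only a stub.
; On BeginPlay it binds to the owning third-person character's scarf power manager and tracks whether the changed scarf type matches its own.
; While active, the scarf ability input only prints a debug message, with no gravity logic yet.
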(event Custom|UpdateActivity
  (params (NewScarfType :type Enum_ScarfPowerType%20Enum :default "NewEnumerator0"))
  ;[1 1 1 1 45] Handle's power activity
  (if (Utilities|Enum|Equal(Enum) NewScarfType "NewEnumerator5")
    (Variables|Default|SetisCurrentPower true)
    (else
      (Variables|Default|SetisCurrentPower false))))

(event Input|EnhancedActionEvents|EnhancedInputActionIA_ScarfAbility
  (params (ActionValue :type Boolean) (ElapsedSeconds :type Float%20%28double-precision%29) (TriggeredSeconds :type Float%20%28double-precision%29) (InputAction :type Input%20Action%20Object%20Reference :default "/Game/Data/Input/Actions/IA_ScarfAbility.IA_ScarfAbility"))
  ;[1 1 1 1 29] Power used
  (:Started
    (if (Variables|Default|GetisCurrentPower)
      (Development|PrintString "Actually using Gravity Flip"))))

(event EventBeginPlay
  ;[1 1 1 1 45] Handle's power activity
  (bind _asbp_third_person_character (Utilities|Casting|CastToBP_ThirdPersonCharacter (Components|GetOwner)))
  (EventDispatchers|BindEventtoOnScarfPowerChanged (Variables|/Game/Blueprints/Player/BP_ThirdPersonCharacter.BP_ThirdPersonCharacter_C|GetBPC_ScarfPowerManager _asbp_third_person_character) (delegate Custom|UpdateActivity)))