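; Player component for the Burrow scarf power, letting the character hide and climb on burrowable walls.
; It tracks the scarf manager's active power; F or left shoulder toggles climbing when a short forward trace hits a BP_BurrowableWall.
; Climbing toggles player visibility and spawned burrow particles, switches movement to Flying, and re-aligns yaw to the wall normal each Tick.
; A missed trace drops the player into Falling; the scarf ability input only prints.
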(event Custom|StopClimbing
  (bind _player (Variables|Default|GetPlayer))
  (bind _charactermovement (Variables|/Script/Engine.Character|GetCharacterMovement _player))
  ;[1 1 1] Stop Climbing
  (Default|ToggleVisibility _player)
  (Variables|Default|SetIsClimbing false)
  (Pawn|Components|CharacterMovement|SetMovementMode _charactermovement "MOVE_Falling" 0)
  (Variables|/Script/Engine.CharacterMovementComponent|SetbOrientRotationToMovement _charactermovement true)
  (Default|ToggleEmitting (Variables|Default|GetBurrowingEffects)))

(event Custom|UpdateActivity
  (params (NewScarfType :type Enum_ScarfPowerType%20Enum :default "NewEnumerator0"))
  ;[1 1 1 1 45] Handle's power activity
  (if (Utilities|Enum|Equal(Enum) NewScarfType "NewEnumerator4")
    (Variables|Default|SetisCurrentPower true)
    (else
      (Variables|Default|SetisCurrentPower false))))

(event Input|EnhancedActionEvents|EnhancedInputActionIA_ScarfAbility
  (params (ActionValue :type Boolean) (ElapsedSeconds :type Float%20%28double-precision%29) (TriggeredSeconds :type Float%20%28double-precision%29) (InputAction :type Input%20Action%20Object%20Reference :default "/Game/Data/Input/Actions/IA_ScarfAbility.IA_ScarfAbility"))
  ;[1 1 1 1 29] Power used
  (:Started
    (if (Variables|Default|GetisCurrentPower)
      (Development|PrintString "Actually using Burrow"))))

(event EventTick
  (params (DeltaSeconds :type Float%20%28single-precision%29))
  (bind _player (Variables|Default|GetPlayer))
  (bind _returnvalue (Transformation|GetActorRotation _player))
  ;[1 1 1] Keeps player looking at the wall
  (if (Variables|Default|GetIsClimbing)
    (bind (_outhit _returnvalue_2) (CallFunction|ClimbingLineTrace))
    (if _returnvalue_2
      (if (== (Utilities|GetClass (.HitActor (Collision|BreakHitResult _outhit))) "/Game/Blueprints/Level/LandChunks/BP_BurrowableWall.BP_BurrowableWall_C")
        (Variables|Default|SetHitPoint (.ImpactPoint (Collision|BreakHitResult _outhit)))
        (bind _output_get (Variables|Default|SetNormalRotation (Math|Rotator|MakeRotator (.roll _returnvalue) (.pitch _returnvalue) (+ (.yaw (Math|Rotator|MakeRotfromX (.Normal (Collision|BreakHitResult _outhit)))) 1.8e+02))))
        (Transformation|SetActorRotation (Variables|Default|GetPlayer) _output_get))
      (else
        (CallFunction|StopClimbing)))))

(event EventBeginPlay
  (bind _asbp_third_person_character (Utilities|Casting|CastToBP_ThirdPersonCharacter (Components|GetOwner)))
  (Variables|Default|SetPlayer _asbp_third_person_character)
  (bind _returnvalue (Game|SpawnActorfromClass "/Game/Blueprints/Player/BP_BurrowingParticleHolder.BP_BurrowingParticleHolder_C" (Transformation|GetActorTransform (Components|GetOwner)) "Undefined" "MultiplyWithRoot" 0 0))
  ;[1 1 1 1 45] Handle's power activity
  (Variables|Default|SetBurrowingEffects _returnvalue)
  (bind _asbp_third_person_character_2 (Utilities|Casting|CastToBP_ThirdPersonCharacter (Components|GetOwner)))
  (EventDispatchers|BindEventtoOnScarfPowerChanged (Variables|/Game/Blueprints/Player/BP_ThirdPersonCharacter.BP_ThirdPersonCharacter_C|GetBPC_ScarfPowerManager _asbp_third_person_character_2) (delegate Custom|UpdateActivity)))

(event Input|KeyboardEvents|F
  (params (Key :type Key%20Structure :default "None"))
  (bind _returnvalue (Components|GetOwner))
  (bind _player (Variables|Default|GetPlayer))
  (bind _returnvalue_2 (Transformation|GetActorRotation _returnvalue))
  (bind _charactermovement (Variables|/Script/Engine.Character|GetCharacterMovement _player))
  ;[1 1 1] Starts the climing mechanics
  (:Pressed
    (if (Variables|Default|GetIsCurrentPower)
      (if (not (Variables|Default|GetIsClimbing))
        (bind (_outhit _returnvalue_3) (CallFunction|ClimbingLineTrace))
        (if _returnvalue_3
          (if (== (Utilities|GetClass (.HitActor (Collision|BreakHitResult _outhit))) "/Game/Blueprints/Level/LandChunks/BP_BurrowableWall.BP_BurrowableWall_C")
            (Variables|Default|SetIsClimbing true)
            (Default|ToggleEmitting (Variables|Default|GetBurrowingEffects))
            (Variables|Default|SetNormalRotation (Math|Rotator|MakeRotator (.roll _returnvalue_2) (.pitch _returnvalue_2) (+ (.yaw (Math|Rotator|MakeRotfromX (.Normal (Collision|BreakHitResult _outhit)))) 1.8e+02)))
            (Variables|Default|SetHitPoint (.ImpactPoint (Collision|BreakHitResult _outhit)))
            (Default|ToggleVisibility (Variables|Default|GetPlayer))
            (Pawn|Components|CharacterMovement|SetMovementMode _charactermovement "MOVE_Flying" 0)
            (Variables|/Script/Engine.CharacterMovementComponent|SetbOrientRotationToMovement _charactermovement false)
            (Transformation|SetActorRotation (Variables|Default|GetPlayer) (Variables|Default|GetNormalRotation))))
        (else
          (CallFunction|StopClimbing)
          (Default|ToggleVisibility (Variables|Default|GetPlayer)))))))

(event Input|GamepadEvents|GamepadLeftShoulder
  (params (Key :type Key%20Structure :default "None"))
  (bind _returnvalue (Components|GetOwner))
  (bind _player (Variables|Default|GetPlayer))
  (bind _returnvalue_2 (Transformation|GetActorRotation _returnvalue))
  (bind _charactermovement (Variables|/Script/Engine.Character|GetCharacterMovement _player))
  ;[1 1 1] Starts the climing mechanics
  (:Pressed
    (if (Variables|Default|GetIsCurrentPower)
      (if (not (Variables|Default|GetIsClimbing))
        (bind (_outhit _returnvalue_3) (CallFunction|ClimbingLineTrace))
        (if _returnvalue_3
          (if (== (Utilities|GetClass (.HitActor (Collision|BreakHitResult _outhit))) "/Game/Blueprints/Level/LandChunks/BP_BurrowableWall.BP_BurrowableWall_C")
            (Variables|Default|SetIsClimbing true)
            (Default|ToggleEmitting (Variables|Default|GetBurrowingEffects))
            (Variables|Default|SetNormalRotation (Math|Rotator|MakeRotator (.roll _returnvalue_2) (.pitch _returnvalue_2) (+ (.yaw (Math|Rotator|MakeRotfromX (.Normal (Collision|BreakHitResult _outhit)))) 1.8e+02)))
            (Variables|Default|SetHitPoint (.ImpactPoint (Collision|BreakHitResult _outhit)))
            (Default|ToggleVisibility (Variables|Default|GetPlayer))
            (Pawn|Components|CharacterMovement|SetMovementMode _charactermovement "MOVE_Flying" 0)
            (Variables|/Script/Engine.CharacterMovementComponent|SetbOrientRotationToMovement _charactermovement false)
            (Transformation|SetActorRotation (Variables|Default|GetPlayer) (Variables|Default|GetNormalRotation))))
        (else
          (CallFunction|StopClimbing)
          (Default|ToggleVisibility (Variables|Default|GetPlayer)))))))

(fn ClimbingLineTrace
  (bind _self self)
  (bind _returnvalue (Components|GetOwner _self))
  (bind _returnvalue_2 (Transformation|GetActorLocation _returnvalue))
  (bind (_outhit _returnvalue_3) (Collision|LineTraceByChannel _returnvalue_2 (+ _returnvalue_2 (* (Transformation|GetActorForwardVector _returnvalue) 50)) "TraceTypeQuery1" false 0 "Persistent"))
  (return _outhit _returnvalue_3))