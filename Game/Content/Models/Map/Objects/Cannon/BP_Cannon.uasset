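; BP_Cannon is a map cannon that automatically fires exploding ball projectiles at a fixed interval.
; Tick accumulates time and, every CannonFireDelay, spawns a TESTJOSEPH_ExplodingBall at the Arrow component's transform.
; It passes speed, lifetime and the actor's forward vector to the ball, then calls its launch function.
; A PawnSensing handler detects the third-person character but only runs a delay, so firing is independent of detection.
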(event OnSeePawn(PawnSensing)
  (params (Pawn :type Pawn%20Object%20Reference))
  (Utilities|Casting|CastToBP_ThirdPersonCharacter Pawn)
  (Utilities|FlowControl|Delay (Variables|Default|GetCannon%20Fire%20Delay)))

(event EventTick
  (params (DeltaSeconds :type Float%20%28single-precision%29))
  (bind _output_get (Variables|Default|SetTimeSinceLastFire (+ DeltaSeconds (Variables|Default|GetTimeSinceLastFire))))
  (if (>= _output_get (Variables|Default|GetCannon%20Fire%20Delay))
    (Variables|Default|SetTimeSinceLastFire 0.0)
    (bind _returnvalue (Game|SpawnActorfromClass "/Game/Blueprints/Level/Testing/TESTJOSEPH_ExplodingBall.TESTJOSEPH_ExplodingBall_C" (Transformation|GetWorldTransform (Variables|Default|GetArrow)) "Undefined" "MultiplyWithRoot" 0 0))
    (Variables|/Game/Blueprints/Level/Testing/TESTJOSEPH_ExplodingBall.TESTJOSEPH_ExplodingBall_C|SetProjectileSpeed _returnvalue (Variables|Default|GetProjectile%20speed))
    (Variables|/Game/Blueprints/Level/Testing/TESTJOSEPH_ExplodingBall.TESTJOSEPH_ExplodingBall_C|SetProjectileDirection _returnvalue (Transformation|GetActorForwardVector))
    (Variables|/Game/Blueprints/Level/Testing/TESTJOSEPH_ExplodingBall.TESTJOSEPH_ExplodingBall_C|SetMaxLifetime _returnvalue (Variables|Default|GetProjectileLifetime))
    (Default|OnProjectileLaunch _returnvalue)))

(fn ConstructionScript)