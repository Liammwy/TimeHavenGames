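; BP_MovingSpikeBall is a level hazard that forces the player to respawn on contact.
; On BeginPlay it caches the third-person character and its capsule, and a DeathHitbox overlap with that capsule calls ForceRespawn.
; A Rolling event adds two relative rotations to Visuals derived from its component velocity, apparently to fake rolling.
; The graph contains no movement logic and no call to Rolling.
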(event OnComponentBeginOverlap(DeathHitbox)
  (params (OverlappedComponent :type Primitive%20Component%20Object%20Reference) (OtherActor :type Actor%20Object%20Reference) (OtherComp :type Primitive%20Component%20Object%20Reference) (OtherBodyIndex :type Integer) (bFromSweep :type Boolean) (SweepResult :type Hit%20Result%20Structure%20%28by%20ref%29))
  (if (== OtherComp (Variables|Default|GetPlayerHitboxRef))
    (Default|ForceRespawn (Variables|Default|GetPlayerRef))))

(event Custom|Rolling
  (bind _visuals (Variables|Default|GetVisuals))
  (bind _returnvalue (Transformation|GetComponentVelocity _visuals))
  (Transformation|AddRelativeRotation (Variables|Default|GetVisuals) (Math|Conversions|RotationFromXVector _returnvalue) false false)
  (Transformation|AddRelativeRotation (Variables|Default|GetVisuals) (Math|Rotator|MakeRotfromXZ (Transformation|GetComponentVelocity (Variables|Default|GetVisuals)) _returnvalue) false false))

(event EventBeginPlay
  (bind _returnvalue (Actor|GetActorOfClass "/Game/Blueprints/Player/BP_ThirdPersonCharacter.BP_ThirdPersonCharacter_C"))
  (Variables|Default|SetPlayerRef _returnvalue)
  (Variables|Default|SetPlayerHitboxRef (Variables|/Script/Engine.Character|GetCapsuleComponent _returnvalue)))

(fn ConstructionScript)