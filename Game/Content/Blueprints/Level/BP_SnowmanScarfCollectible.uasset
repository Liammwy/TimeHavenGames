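; Snowman scarf collectible placed in a level that gives the player a new scarf look on overlap.
; BeginPlay caches the player character's capsule, and the collection radius overlap only responds to that component.
; On collection it applies the scarf mesh's first material to the character, passes the player to the ACSnowmanScarf component's GetScarfType, and sets the IsSnowman flag on the global game instance.
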(event OnComponentBeginOverlap(snowmancollectionradius)
  (params (OverlappedComponent :type Primitive%20Component%20Object%20Reference) (OtherActor :type Actor%20Object%20Reference) (OtherComp :type Primitive%20Component%20Object%20Reference) (OtherBodyIndex :type Integer) (bFromSweep :type Boolean) (SweepResult :type Hit%20Result%20Structure%20%28by%20ref%29))
  (if (== OtherComp (Variables|Default|GetplayerCollisionRef))
    (bind _asbp_third_person_character (Utilities|Casting|CastToBP_ThirdPersonCharacter OtherActor))
    (bind _output_get (Variables|Default|SetCollectedMaterial (Rendering|Material|GetMaterial (Variables|Default|GetStaticMesh3) 0)))
    (Default|ApplyScarfMaterial _asbp_third_person_character _output_get)
    (Default|GetScarfType (Variables|Default|GetAC_SnowmanScarf) OtherActor)
    (bind _asbp_global_game_instance (Utilities|Casting|CastToBP_Global_GameInstance (Game|GetGameInstance)))
    (Variables|/Game/Blueprints/BP_Global_GameInstance.BP_Global_GameInstance_C|SetIsSnowman _asbp_global_game_instance true)))

(event Collision|EventActorBeginOverlap
  (params (OtherActor :type Actor%20Object%20Reference)))

(event EventTick
  (params (DeltaSeconds :type Float%20%28single-precision%29)))

(event EventBeginPlay
  (bind _returnvalue (Actor|GetActorOfClass "/Game/Blueprints/Player/BP_ThirdPersonCharacter.BP_ThirdPersonCharacter_C"))
  (Variables|Default|SetplayerCollisionRef (Variables|/Script/Engine.Character|GetCapsuleComponent _returnvalue)))

(fn ConstructionScript)