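; Level puzzle manager that detects when three referenced torches are all ignited at once.
; On BeginPlay it binds to each torch's ignition-change event and rechecks all three on every change.
; When all are lit, it waits five seconds without rechecking, then notifies its EventListener, calls its all-ignited event and sets the torches to stay permanently ignited.
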(event Custom|OnTorchIgnitionStateChanged
  (if (Math|Boolean|ANDBoolean (Variables|/Game/Blueprints/Level/PowerUps/BP_FireBreathTorch.BP_FireBreathTorch_C|GetIsIgnited (Variables|Default|GetTorchRef_0)) (Variables|/Game/Blueprints/Level/PowerUps/BP_FireBreathTorch.BP_FireBreathTorch_C|GetIsIgnited (Variables|Default|GetTorchRef_1)) (Variables|/Game/Blueprints/Level/PowerUps/BP_FireBreathTorch.BP_FireBreathTorch_C|GetIsIgnited (Variables|Default|GetTorchRef_2)))
    (Utilities|FlowControl|Delay 5.0)
    (Default|RespondtoAllTorchesIgnited (Variables|Default|GetEventListener))
    (Default|CallOnAllTorchesIgnited)
    (Variables|/Game/Blueprints/Level/PowerUps/BP_FireBreathTorch.BP_FireBreathTorch_C|SetStayPermanentlyIgnited (Variables|Default|GetTorchRef_0) true)
    (Variables|/Game/Blueprints/Level/PowerUps/BP_FireBreathTorch.BP_FireBreathTorch_C|SetStayPermanentlyIgnited (Variables|Default|GetTorchRef_1) true)
    (Variables|/Game/Blueprints/Level/PowerUps/BP_FireBreathTorch.BP_FireBreathTorch_C|SetStayPermanentlyIgnited (Variables|Default|GetTorchRef_2) true)))

(event EventBeginPlay
  (EventDispatchers|BindEventtoOnIgnitionStateChanged (Variables|Default|GetTorchRef_0) (delegate Custom|OnTorchIgnitionStateChanged))
  (EventDispatchers|BindEventtoOnIgnitionStateChanged (Variables|Default|GetTorchRef_1) (delegate Custom|OnTorchIgnitionStateChanged))
  (EventDispatchers|BindEventtoOnIgnitionStateChanged (Variables|Default|GetTorchRef_2) (delegate Custom|OnTorchIgnitionStateChanged)))

(fn ConstructionScript)