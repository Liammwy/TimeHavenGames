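; Trigger volume actor that switches the player's view to a fixed camera actor (CamPos) while inside its box, for locked-camera level sections.
; Overlap begin and end blend the view target to CamPos or back to the player, notifying the character via OnEnterLockedCamera/OnExitLockedCamera.
; Snow effects swap between CamPos's particles and the player's SnowfallArea.
; ActiveOnLevelStart optionally applies the locked view at BeginPlay, without the snow swap.
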(event OnComponentBeginOverlap(Box)
  (params (OverlappedComponent :type Primitive%20Component%20Object%20Reference) (OtherActor :type Actor%20Object%20Reference) (OtherComp :type Primitive%20Component%20Object%20Reference) (OtherBodyIndex :type Integer) (bFromSweep :type Boolean) (SweepResult :type Hit%20Result%20Structure%20%28by%20ref%29))
  (bind _playerref (Variables|Default|GetPlayerRef))
  ;[1 1 1] Ensure overlap actor is the player
  (if (== OtherActor _playerref)
    (bind _asplayer_controller (Utilities|Casting|CastToPlayerController (Pawn|GetController _playerref)))
    ;[1 1 1] Set Blend Time for transition time
    (Game|Player|SetViewTargetwithBlend _asplayer_controller (Variables|Default|GetCamPos) (Variables|Default|GetSpeedTransition) "VTBlend_Linear" 0.0 false)
    ;[1 1 1] Signal fixed camera section to player controller to update relative movemnt input
    (Default|OnEnterLockedCamera (Variables|Default|GetPlayerRef))
    (Components|Activation|SetActive (Variables|/Game/Levels/DevLevels/Jack/BP_CamPos.BP_CamPos_C|GetsnowParticles (Variables|Default|GetCamPos)) true true)
    (bind _asbp_third_person_character (Utilities|Casting|CastToBP_ThirdPersonCharacter (Game|GetPlayerCharacter 0)))
    (Components|Activation|SetActive (Variables|/Game/Blueprints/Player/BP_ThirdPersonCharacter.BP_ThirdPersonCharacter_C|GetsnowfallArea _asbp_third_person_character) false false)
    (Rendering|SetVisibility (Variables|/Game/Blueprints/Player/BP_ThirdPersonCharacter.BP_ThirdPersonCharacter_C|GetsnowfallArea _asbp_third_person_character) false false)))

(event OnComponentEndOverlap(Box)
  (params (OverlappedComponent :type Primitive%20Component%20Object%20Reference) (OtherActor :type Actor%20Object%20Reference) (OtherComp :type Primitive%20Component%20Object%20Reference) (OtherBodyIndex :type Integer))
  (bind _playerref (Variables|Default|GetPlayerRef))
  ;[1 1 1] Ensure end overlap actor is player
  (if (== OtherActor _playerref)
    (bind _asplayer_controller (Utilities|Casting|CastToPlayerController (Pawn|GetController _playerref)))
    ;[1 1 1] Set Blend Time for transition time
    (Game|Player|SetViewTargetwithBlend _asplayer_controller (Variables|Default|GetPlayerRef) (Variables|Default|GetSpeedTransition) "VTBlend_Linear" 0.0 false)
    ;[1 1 1] Signal fixed camera section to player controller to update relative movemnt input
    (Default|OnExitLockedCamera (Variables|Default|GetPlayerRef))
    (Components|Activation|SetActive (Variables|/Game/Levels/DevLevels/Jack/BP_CamPos.BP_CamPos_C|GetsnowParticles (Variables|Default|GetCamPos)) false false)
    (bind _asbp_third_person_character (Utilities|Casting|CastToBP_ThirdPersonCharacter (Game|GetPlayerCharacter 0)))
    (Components|Activation|SetActive (Variables|/Game/Blueprints/Player/BP_ThirdPersonCharacter.BP_ThirdPersonCharacter_C|GetsnowfallArea _asbp_third_person_character) true true)
    (Rendering|SetVisibility (Variables|/Game/Blueprints/Player/BP_ThirdPersonCharacter.BP_ThirdPersonCharacter_C|GetsnowfallArea _asbp_third_person_character) true false)))

(event EventBeginPlay
  ;[1 1 1] Grab player ref on BeginPlay
  (bind _returnvalue (Actor|GetActorOfClass "/Game/Blueprints/Player/BP_ThirdPersonCharacter.BP_ThirdPersonCharacter_C"))
  (Variables|Default|SetPlayerRef _returnvalue)
  (if (Variables|Default|GetActiveOnLevelStart)
    (bind _asplayer_controller (Utilities|Casting|CastToPlayerController (Pawn|GetController _returnvalue)))
    (Game|Player|SetViewTargetwithBlend _asplayer_controller (Variables|Default|GetCamPos) (Variables|Default|GetSpeedTransition) "VTBlend_Linear" 0.0 false)
    (Default|OnEnterLockedCamera (Variables|Default|GetPlayerRef))))

(fn ConstructionScript)