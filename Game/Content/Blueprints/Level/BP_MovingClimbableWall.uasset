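; BP_MovingClimbableWall is a level actor for a moving wall that characters with a climbing component can latch onto.
; The construction script gives InterpToMovement a path from the start to the relative Movtopos, using Speed as the duration.
; BeginPlay enables player input and applies Scale to the cube's X and Y.
; On Hit, it calls HitWall on the other actor's BPC_Climbing, if present.
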(event EventBeginPlay
  (bind _cube (Variables|Default|GetCube))
  (bind _scale (Variables|Default|GetScale))
  (Input|EnableInput (Game|GetPlayerController 0))
  ;[1 1 1] Takes inspector parameter 'Scale' and changes the size of the moving platform
  (Transformation|SetRelativeScale3D _cube (Math|Vector|MakeVector _scale _scale (.z (Variables|/Script/Engine.SceneComponent|GetRelativeScale3D _cube)))))

(event Collision|EventHit
  (params (MyComp :type Primitive%20Component%20Object%20Reference) (Other :type Actor%20Object%20Reference) (OtherComp :type Primitive%20Component%20Object%20Reference) (bSelfMoved :type Boolean) (HitLocation :type Vector :default "0, 0, 0") (HitNormal :type Vector :default "0, 0, 0") (NormalImpulse :type Vector :default "0, 0, 0") (Hit :type Hit%20Result%20Structure%20%28by%20ref%29))
  (bind _returnvalue (Actor|GetComponentbyClass Other "/Game/Blueprints/Player/Components/BPC_Climbing.BPC_Climbing_C"))
  ;[1 1 1] When Player hits the wall, activate player connection if needed
  (Utilities|IsValid _returnvalue
    (:Is%20Valid
      (Default|HitWall _returnvalue false))))

(fn ConstructionScript
  (bind _interptomovement (Variables|Default|GetInterpToMovement))
  (Class|InterptoMovementComponent|AddControlPointPosition _interptomovement "0, 0, 0" true)
  (Class|InterptoMovementComponent|AddControlPointPosition (Variables|Default|GetInterpToMovement) (Variables|Default|Getmovtopos) true)
  (Variables|/Script/Engine.InterpToMovementComponent|SetDuration _interptomovement (Variables|Default|GetSpeed)))