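; Moving platform actor that travels between its start point and a configurable relative offset, with a player-triggered slow-down.
; The construction script builds the InterpToMovement path from Movtopos and uses Speed as its duration.
; BeginPlay enables input from the first player controller and applies Scale to the cube's X and Y.
; IA_SlowDown toggles the actor's own CustomTimeDilation between half and normal speed through a FlipFlop.
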(event Input|EnhancedActionEvents|EnhancedInputActionIA_SlowDown
  (params (ActionValue :type Boolean) (ElapsedSeconds :type Float%20%28double-precision%29) (TriggeredSeconds :type Float%20%28double-precision%29) (InputAction :type Input%20Action%20Object%20Reference :default "/Game/Data/Input/Actions/IA_SlowDown.IA_SlowDown"))
  ;[1 1 1] Slow Down
  (:Started
    (Utilities|FlowControl|FlipFlop
      (:A
        (Variables|Default|SetCustomTimeDilation 0.5))
      (:B
        (Variables|Default|SetCustomTimeDilation 1.0)))))

(event EventBeginPlay
  (bind _cube (Variables|Default|GetCube))
  (bind _scale (Variables|Default|GetScale))
  (Input|EnableInput (Game|GetPlayerController 0))
  ;[1 1 1] Takes inspector parameter 'Scale' and changes the size of the moving platform
  (Transformation|SetRelativeScale3D _cube (Math|Vector|MakeVector _scale _scale (.z (Variables|/Script/Engine.SceneComponent|GetRelativeScale3D _cube)))))

(event Collision|EventActorBeginOverlap
  (params (OtherActor :type Actor%20Object%20Reference)))

(event EventTick
  (params (DeltaSeconds :type Float%20%28single-precision%29)))

(fn ConstructionScript
  (bind _interptomovement (Variables|Default|GetInterpToMovement))
  (Class|InterptoMovementComponent|AddControlPointPosition _interptomovement "0, 0, 0" true)
  (Class|InterptoMovementComponent|AddControlPointPosition (Variables|Default|GetInterpToMovement) (Variables|Default|Getmovtopos) true)
  (Variables|/Script/Engine.InterpToMovementComponent|SetDuration _interptomovement (Variables|Default|GetSpeed)))