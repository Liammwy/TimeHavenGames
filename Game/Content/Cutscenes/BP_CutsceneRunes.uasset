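; Cutscene rune actor that endlessly cycles one static mesh through randomly chosen rune shapes.
; From BeginPlay it resets the mesh's relative location, randomly picks one of four rune meshes and plays a timeline.
; The timeline drives the mesh's relative Z to move the rune downward, then calls DoItAgain on finish to repeat the cycle.
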(event Custom|DoItAgain
  (bind _staticmesh (Variables|Default|GetStaticMesh))
  (bind _staticmesh_2 (Variables|Default|GetStaticMesh))
  (bind _relativelocation (Variables|/Script/Engine.SceneComponent|GetRelativeLocation _staticmesh_2))
  ;[0 1 0.8283] Randomises Rune
  (Transformation|SetRelativeLocation (Variables|Default|GetStaticMesh) (Math|Vector|MakeVector 0.0 0.0 0.0) false false)
  (Variables|Default|Setint (Math|Random|RandomIntegerinRange 1 4))
  (if (== (Variables|Default|Getint) 1)
    (Components|StaticMesh|SetStaticMesh _staticmesh "/Game/Models/Map/Collectables/Runes/Rune1.Rune1")
    ;[0.2397 1 0] Will make runes go down
    (bind _newtrack_0 (Timeline|Timeline PlayFromStart)
      (:Update
        (Transformation|SetRelativeLocation _staticmesh_2 (Math|Vector|MakeVector (.x _relativelocation) (.y _relativelocation) (* _newtrack_0 25.0)) false false))
      (:Finished
        (CallFunction|DoItAgain)))
    (elif (== (Variables|Default|Getint) 2)
      (Components|StaticMesh|SetStaticMesh _staticmesh "/Game/Models/Map/Collectables/Runes/Rune2.Rune2")
      (Timeline|Timeline PlayFromStart)
      (elif (== (Variables|Default|Getint) 3)
        (Components|StaticMesh|SetStaticMesh _staticmesh "/Game/Models/Map/Collectables/Runes/Rune3.Rune3")
        (Timeline|Timeline PlayFromStart)
        (else
          (Components|StaticMesh|SetStaticMesh _staticmesh "/Game/Models/Map/Collectables/Runes/Rune4.Rune4")
          (Timeline|Timeline PlayFromStart))))))

(event EventBeginPlay
  (bind _staticmesh (Variables|Default|GetStaticMesh))
  (bind _staticmesh_2 (Variables|Default|GetStaticMesh))
  (bind _relativelocation (Variables|/Script/Engine.SceneComponent|GetRelativeLocation _staticmesh_2))
  ;[0 1 0.8283] Randomises Rune
  (Transformation|SetRelativeLocation (Variables|Default|GetStaticMesh) (Math|Vector|MakeVector 0.0 0.0 0.0) false false)
  (Variables|Default|Setint (Math|Random|RandomIntegerinRange 1 4))
  (if (== (Variables|Default|Getint) 1)
    (Components|StaticMesh|SetStaticMesh _staticmesh "/Game/Models/Map/Collectables/Runes/Rune1.Rune1")
    ;[0.2397 1 0] Will make runes go down
    (bind _newtrack_0 (Timeline|Timeline PlayFromStart)
      (:Update
        (Transformation|SetRelativeLocation _staticmesh_2 (Math|Vector|MakeVector (.x _relativelocation) (.y _relativelocation) (* _newtrack_0 25.0)) false false))
      (:Finished
        (CallFunction|DoItAgain)))
    (elif (== (Variables|Default|Getint) 2)
      (Components|StaticMesh|SetStaticMesh _staticmesh "/Game/Models/Map/Collectables/Runes/Rune2.Rune2")
      (Timeline|Timeline PlayFromStart)
      (elif (== (Variables|Default|Getint) 3)
        (Components|StaticMesh|SetStaticMesh _staticmesh "/Game/Models/Map/Collectables/Runes/Rune3.Rune3")
        (Timeline|Timeline PlayFromStart)
        (else
          (Components|StaticMesh|SetStaticMesh _staticmesh "/Game/Models/Map/Collectables/Runes/Rune4.Rune4")
          (Timeline|Timeline PlayFromStart))))))

(fn ConstructionScript)