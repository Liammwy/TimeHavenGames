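; BP_HatShop is the igloo hat shop entrance, showing the selected hat and an unlocked/total hat count.
; Tick rescans the game instance's HatData every frame to update the display mesh and both text layers.
; A proximity trigger lights the door for the player's capsule.
; Entering the collision volume saves the current level name to the game instance and has the game mode transition to HatShopUILevel.
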(event OnComponentBeginOverlap(Collision)
  (params (OverlappedComponent :type Primitive%20Component%20Object%20Reference) (OtherActor :type Actor%20Object%20Reference) (OtherComp :type Primitive%20Component%20Object%20Reference) (OtherBodyIndex :type Integer) (bFromSweep :type Boolean) (SweepResult :type Hit%20Result%20Structure%20%28by%20ref%29))
  ;[1 0 0.8073 1 66] SAVE DATA AND SEND PLAYER TO HAT LEVEL
  (Utilities|Casting|CastToBP_ThirdPersonCharacter OtherActor)
  (bind _asbp_global_game_instance (Utilities|Casting|CastToBP_Global_GameInstance (Game|GetGameInstance)))
  (bind _returnvalue (Game|GetCurrentLevelName true))
  (Variables|/Game/Blueprints/BP_Global_GameInstance.BP_Global_GameInstance_C|SetpreviousLevel _asbp_global_game_instance (Utilities|String|StringToName _returnvalue))
  (bind _asbp_third_person_game_mode (Utilities|Casting|CastToBP_ThirdPersonGameMode (Game|GetGameMode)))
  (Default|TransitiontoLevel _asbp_third_person_game_mode "HatShopUILevel" false))

(event OnComponentBeginOverlap(changeDoorColour)
  (params (OverlappedComponent :type Primitive%20Component%20Object%20Reference) (OtherActor :type Actor%20Object%20Reference) (OtherComp :type Primitive%20Component%20Object%20Reference) (OtherBodyIndex :type Integer) (bFromSweep :type Boolean) (SweepResult :type Hit%20Result%20Structure%20%28by%20ref%29))
  (if (== OtherComp (Variables|Default|GetplayerCollisionRef))
    (Rendering|Material|SetMaterial (Variables|Default|GetiglooDoor) 0 "/Game/Models/Map/Objects/Portals/Materials/M_YellowPortal.M_YellowPortal")
    (Rendering|SetVisibility (Variables|Default|GetPointLight) true false)))

(event OnComponentEndOverlap(changeDoorColour)
  (params (OverlappedComponent :type Primitive%20Component%20Object%20Reference) (OtherActor :type Actor%20Object%20Reference) (OtherComp :type Primitive%20Component%20Object%20Reference) (OtherBodyIndex :type Integer))
  (if (== OtherComp (Variables|Default|GetplayerCollisionRef))
    (Rendering|Material|SetMaterial (Variables|Default|GetiglooDoor) 0 "/Game/Models/Cutscene/Cave/M_Black.M_Black")
    (Rendering|SetVisibility (Variables|Default|GetPointLight) false false)))

(event Custom|updateTxt
  (bind _hatnumunlocked (Variables|Default|GethatNumUnlocked))
  (bind _outofhatsnum (Variables|Default|GetoutOfHatsNum))
  (bind _returnvalue (Utilities|String|ToString(Integer) _hatnumunlocked))
  (bind _returnvalue_2 (Utilities|String|ToString(Integer) _outofhatsnum))
  (bind _returnvalue_3 (Utilities|String|Append _returnvalue "/" _returnvalue_2))
  (bind _returnvalue_4 (Utilities|Text|ToText(String) _returnvalue_3))
  (Rendering|Components|TextRender|SetText (Variables|Default|GethatsOutOfTXT) _returnvalue_4)
  (Rendering|Components|TextRender|SetText (Variables|Default|GethatsOutOfTXTSHDW) _returnvalue_4))

(event EventBeginPlay
  (bind _returnvalue (Actor|GetActorOfClass "/Game/Blueprints/Player/BP_ThirdPersonCharacter.BP_ThirdPersonCharacter_C"))
  (Variables|Default|SetplayerCollisionRef (Variables|/Script/Engine.Character|GetCapsuleComponent _returnvalue)))

(event EventTick
  (params (DeltaSeconds :type Float%20%28single-precision%29))
  (Variables|Default|SethatNumUnlocked 0)
  (Variables|Default|SetoutOfHatsNum 0)
  (bind _asbp_global_game_instance (Utilities|Casting|CastToBP_Global_GameInstance (Game|GetGameInstance)))
  (for _array_element (Variables|/Game/Blueprints/BP_Global_GameInstance.BP_Global_GameInstance_C|GethatData _asbp_global_game_instance)
    (Math|Integer|IncrementInt (Variables|Default|GetoutOfHatsNum)
      (:%20%20
        (if (.unlocked (Utilities|Struct|BreakS_Hats _array_element))
          (Math|Integer|IncrementInt (Variables|Default|GethatNumUnlocked)
            (:%20%20
              (if (.selected (Utilities|Struct|BreakS_Hats _array_element))
                (Components|StaticMesh|SetStaticMesh (Variables|Default|Gethats) (.hatModel (Utilities|Struct|BreakS_Hats _array_element))))))))))
  (CallFunction|UpdateTxt))

(fn ConstructionScript)