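; A trigger actor in a dev level that changes the player camera's field of view while the third-person character is inside its ZoomOut volume.
; On BeginPlay it caches the BP_ThirdPersonCharacter and its capsule, which filters the overlap events.
; Overlap begin plays a timeline that drives FollowCamera's field of view, and overlap end reverses it.
; IsZoomed is set true on each timeline update and is reset only at BeginPlay.
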(event OnComponentBeginOverlap(ZoomOut)
  (params (OverlappedComponent :type Primitive%20Component%20Object%20Reference) (OtherActor :type Actor%20Object%20Reference) (OtherComp :type Primitive%20Component%20Object%20Reference) (OtherBodyIndex :type Integer) (bFromSweep :type Boolean) (SweepResult :type Hit%20Result%20Structure%20%28by%20ref%29))
  (if (== OtherComp (Variables|Default|GetPlayerHitbox))
    (bind _zoom_out (Timeline|Timeline Play)
      (:Update
        (Camera|SetFieldOfView (Variables|/Game/Blueprints/Player/BP_ThirdPersonCharacter.BP_ThirdPersonCharacter_C|GetFollowCamera (Variables|Default|GetPlayerRef)) _zoom_out)
        (Variables|Default|SetIs%20Zoomed? true)))))

(event OnComponentEndOverlap(ZoomOut)
  (params (OverlappedComponent :type Primitive%20Component%20Object%20Reference) (OtherActor :type Actor%20Object%20Reference) (OtherComp :type Primitive%20Component%20Object%20Reference) (OtherBodyIndex :type Integer))
  (if (== OtherComp (Variables|Default|GetPlayerHitbox))
    (bind _zoom_out (Timeline|Timeline Reverse)
      (:Update
        (Camera|SetFieldOfView (Variables|/Game/Blueprints/Player/BP_ThirdPersonCharacter.BP_ThirdPersonCharacter_C|GetFollowCamera (Variables|Default|GetPlayerRef)) _zoom_out)
        (Variables|Default|SetIs%20Zoomed? true)))))

(event EventBeginPlay
  (Variables|Default|SetIs%20Zoomed? false)
  (bind _returnvalue (Actor|GetActorOfClass "/Game/Blueprints/Player/BP_ThirdPersonCharacter.BP_ThirdPersonCharacter_C"))
  (Variables|Default|SetPlayerRef _returnvalue)
  (Variables|Default|SetPlayerHitbox (Variables|/Script/Engine.Character|GetCapsuleComponent _returnvalue)))

(event Collision|EventActorBeginOverlap
  (params (OtherActor :type Actor%20Object%20Reference)))

(event EventTick
  (params (DeltaSeconds :type Float%20%28single-precision%29)))

(fn ConstructionScript)