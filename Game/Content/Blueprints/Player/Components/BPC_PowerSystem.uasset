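; Player component that manages the power meter behind the time-slow ability, along with its HUD bar and screen tint widgets.
; Tick runs a countdown that periodically drains power while DrainPower is set, showing the tint, or otherwise regains it until full, hiding the tint.
; Draining clears the flag at empty, and each regain step restores normal global time dilation.
; The slowdown itself is not applied here.
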(event EventTick
  (params (DeltaSeconds :type Float%20%28single-precision%29))
  (bind _output_get (Variables|Default|SetcurrentDelay (- (Variables|Default|GetcurrentDelay) DeltaSeconds)))
  (if (<= _output_get 0.0)
    (Variables|Default|SetcurrentDelay 0.2)
    (if (Variables|Default|GetdrainPower)
      (CallFunction|DrainingPower)
      (Variables|/Script/UMG.Widget|SetVisibility (Variables|Default|GettimeSlowTint) "Visible")
      (elif (not (== (Variables|Default|GetcurrentPower) (Variables|Default|GetmaxPower)))
        (CallFunction|RegainingPower)
        (Variables|/Script/UMG.Widget|SetVisibility (Variables|Default|GettimeSlowTint) "Hidden")))))

(event EventBeginPlay
  (Variables|Default|SetcurrentPower (Variables|Default|GetmaxPower))
  (bind _returnvalue (UserInterface|CreateWidget "/Game/Blueprints/UI/WBP_TimeSlow.WBP_TimeSlow_C" (Game|GetPlayerController 0)))
  (bind _output_get (Variables|Default|SettimeSlowWidget _returnvalue))
  (UserInterface|Viewport|AddtoViewport _output_get 0)
  (bind _returnvalue_2 (UserInterface|CreateWidget "/Game/Blueprints/UI/WBP_TimeSlowTint.WBP_TimeSlowTint_C" (Game|GetPlayerController 0)))
  (bind _output_get_2 (Variables|Default|SettimeSlowTint _returnvalue_2))
  (UserInterface|Viewport|AddtoViewport _output_get_2 0))

(fn DrainingPower
  ;[1 1 1 1 30] Logic for draining power
  (if (<= (Variables|Default|GetcurrentPower) 0.0)
    (Variables|Default|SetdrainPower false)
    (else
      (Variables|Default|SetcurrentPower (Math|Float|Clamp(Float) (- (Variables|Default|GetcurrentPower) 1.0) 0.0 (Variables|Default|GetmaxPower)))
      (Default|SetPercent (Variables|Default|GettimeSlowWidget) (Variables|Default|GetcurrentPower) (Variables|Default|GetmaxPower)))))

(fn RegainingPower
  (Variables|Default|SetcurrentPower (Math|Float|Clamp(Float) (+ (Variables|Default|GetcurrentPower) 1.0) 0.0 (Variables|Default|GetmaxPower)))
  (Default|SetPercent (Variables|Default|GettimeSlowWidget) (Variables|Default|GetcurrentPower) (Variables|Default|GetmaxPower))
  (Utilities|Time|SetGlobalTimeDilation 1.0))